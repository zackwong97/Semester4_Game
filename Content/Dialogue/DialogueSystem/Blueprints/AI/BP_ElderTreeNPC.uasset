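; Elder Tree quest NPC that sends the player to gather elixir ingredients, then reveals Nakary as the curse's source and grants Fleeting Power.
; NarrationNum picks introduction, ingredient check or final reminder, with PingNPC branching on the controller's ingredient flags.
; OnDialogueEnd chains lines by index, triggering speech-bubble emotes, an area camera blend and scene continuation, with names chosen by CharacterID.
; Tick fades ElderTreeGlow in a material parameter collection following StartGlow.
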(event `self.Ping NPC`
  (params (Num :type Integer) (FeaturePlayerCharacter :type Integer))
  (switch `int` Num
    (:`0`
      (`self.DoneChecking`))))

(event `DoneChecking`
  (bind _playercontrollerref (`self.PlayerControllerRef`))
  (`KismetSystemLibrary.Delay` 0.2)
  (if (and (`/Game/Blueprint/GamePlay-PC.hasWhiteBlossom` _playercontrollerref) (`/Game/Blueprint/GamePlay-PC.hasVenusBranch` _playercontrollerref))
    (`self.AddCustomImportantDialogue` 11 (make `/Game/Dialogue/DialogueSystem/Blueprints/Structures/s_DialogueInfo` null (`KismetTextLibrary.Conv_StringToText` (`KismetStringLibrary.Concat_StrStr` "You did well " (select `int` (`/Game/Blueprint/GamePlay-PC.CharacterID` (`self.PlayerControllerRef`)) :`0` "Opiyo, " :`1` "Opiyo, " :`2` "Otoyo, ") "the evil energies seem to be weakened.")) "Elder Tree"))
    (else
      (`self.AddCustomImportantDialogue` 8 (make `/Game/Dialogue/DialogueSystem/Blueprints/Structures/s_DialogueInfo` null (`KismetTextLibrary.Conv_StringToText` (`KismetStringLibrary.Concat_StrStr` "You are back young " (select `int` (`/Game/Blueprint/GamePlay-PC.CharacterID` (`self.PlayerControllerRef`)) :`0` "Opiyo, " :`1` "Opiyo, " :`2` "Otoyo, " :`3` "") "If you really desire Nakary’s whereabouts I will have you seek a few rare ingredients in return first.")) "Elder Tree")))))

(event `self.AfterConversationSetup`
  (switch `int` (`self.narrationNum`)
    (:`0`
      (set `self.narrationNum` 1)
      (`self.AddCustomImportantDialogue` 0 (make `/Game/Dialogue/DialogueSystem/Blueprints/Structures/s_DialogueInfo` null (`KismetTextLibrary.Conv_StringToText` (`KismetStringLibrary.Concat_StrStr` "So you have come, " (select `int` (`/Game/Blueprint/GamePlay-PC.CharacterID` (`self.PlayerControllerRef`)) :`0` "Opiyo." :`1` "Opiyo." :`2` "Otoyo."))) "Elder Tree")))
    (:`1`
      (`/Game/Blueprint/GamePlay-PC.Check Ingredients` (`self.PlayerControllerRef`)))
    (:`2`
      (`self.AddCustomImportantDialogue` 10 (make `/Game/Dialogue/DialogueSystem/Blueprints/Structures/s_DialogueInfo` null "Brew those ingredients into a potion and head south child." "Elder Tree")))))

(event `self.ReceiveTick`
  (params (DeltaSeconds :type "Float (single-precision)"))
  (bind _parametervalue (`self.ParameterValue`))
  (bind _returnvalue (/ (`GameplayStatics.GetWorldDeltaSeconds`) (`self.SecondsToHitGlow`)))
  (if (`self.StartGlow`)
    (if (not (== _parametervalue 1.0))
      (bind _output_get (set `self.ParameterValue` (+ _parametervalue _returnvalue)))
      (if (> _output_get 1.0)
        (set `self.ParameterValue` 1.0))
      (`KismetMaterialLibrary.SetScalarParameterValue` "/Game/Environment/Props/Materials/Collections/MPC1.MPC1" "ElderTreeGlow" _output_get))
    (elif (not (== _parametervalue 0.0))
      (bind _output_get_2 (set `self.ParameterValue` (- _parametervalue _returnvalue)))
      (if (< _output_get_2 0.0)
        (set `self.ParameterValue` 0.0)
        (else
          (`KismetMaterialLibrary.SetScalarParameterValue` "/Game/Environment/Props/Materials/Collections/MPC1.MPC1" "ElderTreeGlow" _output_get_2))))))

(event `self.OnDialogueEnd`
  (params (Index :type Integer))
  (bind _returnvalue (select `int` (`/Game/Blueprint/GamePlay-PC.CharacterID` (`self.PlayerControllerRef`)) :`0` "Opiyo" :`1` "Opiyo" :`2` "Otoyo"))
  (bind _speechbubbleref (`/Game/Characters/Player/TestCharacter2/BP_Character_Base.SpeechBubbleRef` (`/Game/Blueprint/GamePlay-PC.CharacterRef` (`self.PlayerControllerRef`))))
  (bind _speechbubbleref_2 (`/Game/Characters/Player/TestCharacter2/BP_Character_Base.SpeechBubbleRef` (`/Game/Blueprint/GamePlay-PC.CharacterRef` (`self.PlayerControllerRef`))))
  (switch `int` Index
    (:`0`
      (`self.AddCustomImportantDialogue` 1 (make `/Game/Dialogue/DialogueSystem/Blueprints/Structures/s_DialogueInfo` null "I am the heart of this forest and I have watched this forest since birth." "Elder Tree")))
    (:`1`
      (`self.AddCustomImportantDialogue` 2 (make `/Game/Dialogue/DialogueSystem/Blueprints/Structures/s_DialogueInfo` null "The eyes of every living being in this forest are my own eyes as well." "Elder Tree")))
    (:`2`
      (`self.AddCustomImportantDialogue` 3 (make `/Game/Dialogue/DialogueSystem/Blueprints/Structures/s_DialogueInfo` null (`KismetTextLibrary.Conv_StringToText` (`KismetStringLibrary.Concat_StrStr` "Young " (select `int` (`/Game/Blueprint/GamePlay-PC.CharacterID` (`self.PlayerControllerRef`)) :`0` "Opiyo," :`1` "Opiyo," :`2` "Otoyo,") " I have heard your prayer loud and clear and I know what you seek. ")) "Elder Tree")))
    (:`3`
      (`self.AddCustomImportantDialogue` 4 (make `/Game/Dialogue/DialogueSystem/Blueprints/Structures/s_DialogueInfo` null "I shall help you find your mother, Nakary the Witch. But you must complete my request first if you wish to find her." "Elder Tree"))
      (`KismetSystemLibrary.Delay` 2.0)
      (`/Game/UI/Blueprints/SpeechBubbleWidget.Play DotDotDot` _speechbubbleref))
    (:`4`
      (`self.AddCustomImportantDialogue` 5 (make `/Game/Dialogue/DialogueSystem/Blueprints/Structures/s_DialogueInfo` null "A strong curse has tainted the forest." "Elder Tree"))
      (`KismetSystemLibrary.Delay` 2.0)
      (`/Game/UI/Blueprints/SpeechBubbleWidget.Play Exclamation` _speechbubbleref))
    (:`5`
      (`self.AddCustomImportantDialogue` 6 (make `/Game/Dialogue/DialogueSystem/Blueprints/Structures/s_DialogueInfo` null "Dark beasts have arisen and are destroying the forest" "Elder Tree")))
    (:`6`
      (`self.AddCustomImportantDialogue` 7 (make `/Game/Dialogue/DialogueSystem/Blueprints/Structures/s_DialogueInfo` null "Defeat them in order to weaken the curse." "Elder Tree")))
    (:`7`
      (`self.AddCustomImportantDialogue` 8 (make `/Game/Dialogue/DialogueSystem/Blueprints/Structures/s_DialogueInfo` null "You will need to collect ingredients for an elixir to cleanse this curse." "Elder Tree")))
    (:`8`
      (`self.AddCustomImportantDialogue` 9 (make `/Game/Dialogue/DialogueSystem/Blueprints/Structures/s_DialogueInfo` null "White Blossom and Venus Branch deep in the Ruined Tropics" "Elder Tree"))
      (`PlayerController.SetViewTargetWithBlend` (`self.PlayerControllerRef`) (`self.Area3Camera`) 2.0 "VTBlend_Cubic" 1.0 false))
    (:`9`
      (`self.AddCustomImportantDialogue` 10 (make `/Game/Dialogue/DialogueSystem/Blueprints/Structures/s_DialogueInfo` null "Return with those ingredients only then I shall tell you..." "Elder Tree")))
    (:`10`
      (`self.EndConversation` :!label _label))
    (:`11`
      (`self.AddCustomImportantDialogue` 12 (make `/Game/Dialogue/DialogueSystem/Blueprints/Structures/s_DialogueInfo` null (`KismetTextLibrary.Conv_StringToText` (`KismetStringLibrary.Concat_StrStr` "I sense that you have gathered the potion ingredients as well. Your mother would be proud of you, " (select `int` (`/Game/Blueprint/GamePlay-PC.CharacterID` (`self.PlayerControllerRef`)) :`0` "Opiyo." :`1` "Opiyo." :`2` "Otoyo."))) "Elder Tree")))
    (:`12`
      (`self.AddCustomImportantDialogue` 13 (make `/Game/Dialogue/DialogueSystem/Blueprints/Structures/s_DialogueInfo` null "Now, I must confess to you an unsettling truth. Forgive me for hiding this from you until now." "Elder Tree"))
      (`KismetSystemLibrary.Delay` 2.0)
      (`/Game/UI/Blueprints/SpeechBubbleWidget.Play Question Mark` _speechbubbleref_2))
    (:`13`
      (`KismetSystemLibrary.Delay` 1.0)
      (`self.AddCustomImportantDialogue` 14 (make `/Game/Dialogue/DialogueSystem/Blueprints/Structures/s_DialogueInfo` null "The source of the curse is... Nakary the Witch herself!" "Elder Tree"))
      (`KismetSystemLibrary.Delay` 2.0)
      (`/Game/UI/Blueprints/SpeechBubbleWidget.Play Exclamation` _speechbubbleref_2))
    (:`14`
      (`self.AddCustomImportantDialogue` 15 (make `/Game/Dialogue/DialogueSystem/Blueprints/Structures/s_DialogueInfo` null "She had meddled with dark magic in her potions. This has unleashed a dark curse which now defiles the forest." "Elder Tree")))
    (:`15`
      (`self.AddCustomImportantDialogue` 16 (make `/Game/Dialogue/DialogueSystem/Blueprints/Structures/s_DialogueInfo` null "She now pays for her misdeeds." "Elder Tree")))
    (:`16`
      (`self.AddCustomImportantDialogue` 17 (make `/Game/Dialogue/DialogueSystem/Blueprints/Structures/s_DialogueInfo` null "what?... no... mama..." (`KismetTextLibrary.Conv_StringToText` _returnvalue))))
    (:`17`
      (`self.AddCustomImportantDialogue` 18 (make `/Game/Dialogue/DialogueSystem/Blueprints/Structures/s_DialogueInfo` null (`KismetTextLibrary.Conv_StringToText` (`KismetStringLibrary.Concat_StrStr` "Calm yourself, " _returnvalue ".")) "Elder Tree")))
    (:`18`
      (`self.AddCustomImportantDialogue` 19 (make `/Game/Dialogue/DialogueSystem/Blueprints/Structures/s_DialogueInfo` null "I will tell you what you need to do to save both the forest and Nakary." "Elder Tree"))
      (`KismetSystemLibrary.Delay` 2.0)
      (`/Game/UI/Blueprints/SpeechBubbleWidget.Play DotDotDot` (`/Game/Characters/Player/TestCharacter2/BP_Character_Base.SpeechBubbleRef` (`/Game/Blueprint/GamePlay-PC.CharacterRef` (`self.PlayerControllerRef`)))))
    (:`19`
      (`self.AddCustomImportantDialogue` 20 (make `/Game/Dialogue/DialogueSystem/Blueprints/Structures/s_DialogueInfo` null "These ingredients you have gathered must be brewed into a potion. A potion that can release Nakary from the curse." "Elder Tree"))
      (`KismetSystemLibrary.Delay` 4.0)
      (`/Game/UI/Blueprints/SpeechBubbleWidget.Play Exclamation` (`/Game/Characters/Player/TestCharacter2/BP_Character_Base.SpeechBubbleRef` (`/Game/Blueprint/GamePlay-PC.CharacterRef` (`self.PlayerControllerRef`)))))
    (:`20`
      (`self.AddCustomImportantDialogue` 21 (make `/Game/Dialogue/DialogueSystem/Blueprints/Structures/s_DialogueInfo` null (`KismetTextLibrary.Conv_StringToText` (`KismetStringLibrary.Concat_StrStr` (select `int` (`/Game/Blueprint/GamePlay-PC.CharacterID` (`self.PlayerControllerRef`)) :`0` "Opiyo" :`1` "Opiyo" :`2` "Otoyo") ", I must ask of you to end this curse. The forest will die if this curse continues to spread.")) "Elder Tree")))
    (:`21`
      (`self.AddCustomImportantDialogue` 22 (make `/Game/Dialogue/DialogueSystem/Blueprints/Structures/s_DialogueInfo` null "Head south, the path to Nakary is now unsealed." "Elder Tree")))
    (:`22`
      (`self.AddCustomImportantDialogue` 23 (make `/Game/Dialogue/DialogueSystem/Blueprints/Structures/s_DialogueInfo` null "The forest will show you the way, but you must prepare for a harsh battle." "Elder Tree")))
    (:`23`
      ;[1 1 1] power
      (`self.AddCustomImportantDialogue` 24 (make `/Game/Dialogue/DialogueSystem/Blueprints/Structures/s_DialogueInfo` null "I will bestow upon you this power." "Elder Tree")))
    (:`24`
      (`/Game/Blueprint/GamePlay-PC.Gain Fleeting Power` (`self.PlayerControllerRef`))
      (`KismetSystemLibrary.Delay` 3.0)
      (`self.AddCustomImportantDialogue` 25 (make `/Game/Dialogue/DialogueSystem/Blueprints/Structures/s_DialogueInfo` null "I know this is a difficult task to ask of you to fight someone dear to you..." "Elder Tree")))
    (:`25`
      (`self.AddCustomImportantDialogue` 26 (make `/Game/Dialogue/DialogueSystem/Blueprints/Structures/s_DialogueInfo` null (`KismetTextLibrary.Conv_StringToText` (`KismetStringLibrary.Concat_StrStr` "Stand strong " (select `int` (`/Game/Blueprint/GamePlay-PC.CharacterID` (`self.PlayerControllerRef`)) :`0` "Opiyo" :`1` "Opiyo" :`2` "Otoyo") ".")) "Elder Tree"))
      (`/Game/Blueprint/GamePlay-PC.ContinueScene` (`self.PlayerControllerRef`) 10))
    (:`26`
      (set `self.narrationNum` 2)
      (goto _label))))

(fn `UserConstructionScript`
  (`parent.UserConstructionScript`))