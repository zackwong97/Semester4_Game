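; Dialogue NPC for an ending scene, voicing Nakary's scripted lines as she pleads with her child.
; After conversation setup on the first narration, she calls out Opiyo's or Otoyo's name based on flags set through SetCharactersName.
; Dialogue-end indices chain to her warning or tell the player controller to continue the scene.
; External PingNPC calls trigger her final plea or end the conversation.
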(event `self.Ping NPC`
  (params (Num :type Integer) (FeaturePlayerCharacter :type Integer))
  (switch `int` Num
    (:`1`
      (`self.AddCustomImportantDialogue` 3 (make `/Game/Dialogue/DialogueSystem/Blueprints/Structures/s_DialogueInfo` null "My Child! This is a mistake! PLEASE!!!" "Nakary")))
    (:`2`
      (`self.EndConversation`))))

(event `self.AfterConversationSetup`
  (switch `int` (`self.narrationNum`)
    (:`1`
      (`self.AddCustomImportantDialogue` 1 (make `/Game/Dialogue/DialogueSystem/Blueprints/Structures/s_DialogueInfo` null (`KismetTextLibrary.Conv_StringToText` (`KismetStringLibrary.Concat_StrStr` (select `bool` (`self.OpiyoInGame?`) :`true` "Opiyo? ") (select `bool` (`self.OtoyoInGame?`) :`true` "Otoyo?"))) "Nakary")))))

(event `Set Characters Name`
  (params (`OpiyoInGame?` :type "Boolean (by ref)") (`OtoyoInGame?` :type "Boolean (by ref)"))
  (set `self.OpiyoInGame?` `OpiyoInGame?`)
  (set `self.OtoyoInGame?` `OtoyoInGame?`))

(event `self.OnDialogueEnd`
  (params (Index :type Integer))
  (bind _playercontrollerref (`self.PlayerControllerRef`))
  (switch `int` Index
    (:`1`
      (`self.AddCustomImportantDialogue` 2 (make `/Game/Dialogue/DialogueSystem/Blueprints/Structures/s_DialogueInfo` null "No... Leave!!! I don't you to get hurt!" "Nakary")))
    (:`2`
      (`/Game/Blueprint/GamePlay-PC.ContinueScene` _playercontrollerref 6))
    (:`3`
      (`/Game/Blueprint/GamePlay-PC.ContinueScene` _playercontrollerref 7))))

(fn `UserConstructionScript`
  (`parent.UserConstructionScript`))