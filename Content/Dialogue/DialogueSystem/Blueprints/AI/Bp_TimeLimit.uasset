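; Dialogue showcase Blueprint that demonstrates time-limited decisions in the dialogue system and closes out the demo.
; After conversation setup it queues voiced lines, with each dialogue-end event triggering the next step by index.
; The second line leads into a two-option decision with a time limit, described in dialogue as auto-confirming the selected option on expiry.
; Either choice plays the same closing line, after which the conversation ends.
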(event `self.AfterConversationSetup`
  ;[1 1 1] Adds the first dialogue
  (`self.AddCustomImportantDialogue` 0 (make `/Game/Dialogue/DialogueSystem/Blueprints/Structures/s_DialogueInfo` "/Game/Dialogue/DialogueSystem/AudioFiles/Showcase/Showcase18.Showcase18" "Some decision that heavily influence the story can also have a custom time limit." (`self.Name`))))

(event `self.OnDialogueEnd`
  (params (Index :type Integer))
  ;[1 1 1] On Dialogue End
  (switch `int` Index
    (:`0`
      (`self.AddCustomImportantDialogue` 1 (make `/Game/Dialogue/DialogueSystem/Blueprints/Structures/s_DialogueInfo` "/Game/Dialogue/DialogueSystem/AudioFiles/Showcase/Showcase19.Showcase19" "After the time has expired, the currently selected option will be confirmed." (`self.Name`))))
    (:`1`
      (`self.AddDecision` 0 (make `/Game/Dialogue/DialogueSystem/Blueprints/Structures/s_DecisionInfo` (make `/Game/Dialogue/DialogueSystem/Blueprints/Structures/s_DialogueInfo` "/Game/Dialogue/DialogueSystem/AudioFiles/Showcase/Showcase20.Showcase20" "Here is an example: What do you want to do?" (`self.Name`)) (`|MakeArray` (make `/Game/Dialogue/DialogueSystem/Blueprints/Structures/s_OptionInfo` "Attack the enemy" null "NewEnumerator2") (make `/Game/Dialogue/DialogueSystem/Blueprints/Structures/s_OptionInfo` "Stay calm" null "NewEnumerator2") :!type "/Game/Dialogue/DialogueSystem/Blueprints/Structures/s_OptionInfo Structure") true)))
    (:`2`
      (`self.EndConversation`))))

(event `self.OnDecisionMade`
  (params (DecisionIndex :type Integer) (ChosenOptionIndex :type Integer))
  ;[1 1 1] On Decision Made
  (`self.AddCustomImportantDialogue` 2 (make `/Game/Dialogue/DialogueSystem/Blueprints/Structures/s_DialogueInfo` "/Game/Dialogue/DialogueSystem/AudioFiles/Showcase/Showcase21.Showcase21" "That was the showcase video for my dialogue system. I hope you liked it." (`self.Name`))))

(fn `UserConstructionScript`
  (`parent.UserConstructionScript`))