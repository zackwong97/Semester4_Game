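; Kachujin NPC Blueprint that scripts a short scene 1 conversation through parent dialogue hooks.
; An opening "BOOM!" line plays after setup, and its end has the player controller move the NPC to a P1 or P2 target, chosen by server or client.
; On arrival it queues "mama?" with a speaker name picked by CharacterID, then ends the conversation and updates scene state.
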(event `self.AfterConversationSetup`
  (`self.AddCustomImportantDialogue` 0 (make `/Game/Dialogue/DialogueSystem/Blueprints/Structures/s_DialogueInfo` null "BOOM!")))

(event `self.OnDialogueEnd`
  (params (Index :type Integer))
  (bind _gameplay_managerref (`self.Gameplay_ManagerRef`))
  (switch `int` Index
    (:`0`
      (`/Game/Blueprint/GamePlay-PC.MoveToLocationNPC` (`self.PlayerControllerRef`) (`self.K2_GetActorLocation` (select `bool` (`KismetSystemLibrary.IsServer`) :`false` (`/Game/Blueprint/Gameplay_Manager.P2-Scene1-MoveToLocation` _gameplay_managerref) :`true` (`/Game/Blueprint/Gameplay_Manager.P1-Scene1-MoveToLocation` _gameplay_managerref))) self Index))
    (:`1`
      (`self.EndConversation`)
      (`/Game/Blueprint/GamePlay-PC.Update Scene State` (`self.PlayerControllerRef`) 1))))

(event `self.Reach NPC`
  (params (Location :type "Vector Structure (by ref)") (DialogueNum :type "Integer (by ref)"))
  (switch `int` DialogueNum
    (:`0`
      (`self.AddCustomImportantDialogue` 1 (make `/Game/Dialogue/DialogueSystem/Blueprints/Structures/s_DialogueInfo` null "mama?" (select `int` (`/Game/Blueprint/GamePlay-PC.CharacterID` (`self.PlayerControllerRef`)) :`0` "Opiyo" :`1` "Opiyo" :`2` "Otoyo"))))))

(fn `UserConstructionScript`
  (`parent.UserConstructionScript`))