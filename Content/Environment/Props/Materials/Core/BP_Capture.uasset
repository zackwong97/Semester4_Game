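; BP_Capture is a scene capture actor that renders tagged grass affectors into the RT_GrassAffector render target, likely for interactive grass.
; On begin play it writes the ortho width to a Material Parameter Collection, clears the target and adds "GrassAffector"-tagged components of tagged actors to the show-only list.
; Each tick it follows the collection's character position in XY and publishes its location back for materials.
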(event `self.ReceiveBeginPlay`
  (`self.SetCaptureSize`)
  (`KismetRenderingLibrary.ClearRenderTarget2D` "/Game/Environment/Props/Materials/Core/RT_GrassAffector.RT_GrassAffector")
  (bind _outactors (`GameplayStatics.GetAllActorsWithTag` "GrassAffector"))
  (for _array_element _outactors
    (for _array_element_2 (`self.GetComponentsByTag` _array_element "/Script/Engine.PrimitiveComponent" "GrassAffector")
      (`SceneCaptureComponent.ShowOnlyComponent` (`self.SceneCapture`) _array_element_2))))

(event `self.ReceiveTick`
  (params (DeltaSeconds :type "Float (single-precision)"))
  (`self.MoveCapture`))

(fn `MoveCapture`
  (bind (_returnvalue_x _returnvalue_y _returnvalue_z) (`KismetMathLibrary.BreakVector` (`self.K2_GetActorLocation`)))
  (bind _returnvalue (`KismetMaterialLibrary.GetVectorParameterValue` "/Game/Environment/Props/Materials/MPC1.MPC1" "Character Position"))
  (bind (_r _g) (`KismetMathLibrary.BreakColor` _returnvalue))
  (`self.K2_SetActorLocation` (`KismetMathLibrary.MakeVector` _r _g _returnvalue_z))
  (`KismetMaterialLibrary.SetVectorParameterValue` "/Game/Environment/Props/Materials/MPC1.MPC1" "CaptureLocation" (`KismetMathLibrary.Conv_VectorToLinearColor` (`self.K2_GetActorLocation`))))

(fn `SetCaptureSize`
  (`KismetMaterialLibrary.SetScalarParameterValue` "/Game/Environment/Props/Materials/MPC1.MPC1" "CaptureSize" (`SceneCaptureComponent2D.OrthoWidth` (`self.SceneCapture`))))

(fn `UserConstructionScript`)