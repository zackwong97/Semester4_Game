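; Shrine prop actor that detects player characters nearby and exposes a toggleable world widget.
; Sphere overlap begin calls EnterShrine on any BP_Character_Base, passing itself, and overlap end calls LeaveShrine.
; EnableWidget and DisableWidget events show or hide the Widget component, leaving the decision of when to display it to outside callers.
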(event `self.Sphere.OnComponentBeginOverlap`
  (params (OverlappedComponent :type "PrimitiveComponent Object Reference") (OtherActor :type "Actor Object Reference") (OtherComp :type "PrimitiveComponent Object Reference") (OtherBodyIndex :type Integer) (bFromSweep :type Boolean) (SweepResult :type "HitResult Structure (by ref)"))
  (bind _asbp_character_base (cast `/Game/Characters/Player/TestCharacter2/BP_Character_Base` OtherActor))
  (`/Game/Characters/Player/TestCharacter2/BP_Character_Base.Enter Shrine` _asbp_character_base self))

(event `self.Sphere.OnComponentEndOverlap`
  (params (OverlappedComponent :type "PrimitiveComponent Object Reference") (OtherActor :type "Actor Object Reference") (OtherComp :type "PrimitiveComponent Object Reference") (OtherBodyIndex :type Integer))
  (bind _asbp_character_base (cast `/Game/Characters/Player/TestCharacter2/BP_Character_Base` OtherActor))
  (`/Game/Characters/Player/TestCharacter2/BP_Character_Base.Leave Shrine` _asbp_character_base))

(event `Enable Widget`
  (`SceneComponent.SetVisibility` (`self.Widget`) true false))

(event `Disable Widget`
  (`SceneComponent.SetVisibility` (`self.Widget`) false false))

(fn `UserConstructionScript`)