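; Scene capture actor that follows the player character and renders tagged grass affectors, apparently to drive grass trail effects.
; On BeginPlay it clears RT_GrassAffector and limits the capture to GrassAffector-tagged components on likewise tagged actors.
; Each tick it moves above the character and captures manually.
; It publishes capture ortho width and location to material parameter collection MPC1, letting materials map world position into the capture.
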(event `self.ReceiveBeginPlay`
  (`self.SetCaptureSize`)
  (`KismetRenderingLibrary.ClearRenderTarget2D` "/Game/Environment/Props/Textures/RT_GrassAffector.RT_GrassAffector")
  (bind _outactors (`GameplayStatics.GetAllActorsWithTag` "GrassAffector"))
  (for _array_element _outactors
    (for _array_element_2 (`self.GetComponentsByTag` _array_element "/Script/Engine.PrimitiveComponent" "GrassAffector")
      (`SceneCaptureComponent.ShowOnlyComponent` (`self.SceneCapture`) _array_element_2))))

(event `self.ReceiveTick`
  (params (DeltaSeconds :type "Float (single-precision)"))
  (`self.MoveCapture`)
  (`SceneCaptureComponent2D.CaptureScene` (`self.SceneCapture`)))

(fn `MoveCapture`
  (bind _asgame_play__pc (cast `/Game/Blueprint/GamePlay-PC` (`GameplayStatics.GetPlayerController` 0)))
  (bind (_returnvalue_x _returnvalue_y _returnvalue_z) (`KismetMathLibrary.BreakVector` (`self.K2_GetActorLocation` (`/Game/Blueprint/GamePlay-PC.CharacterRef` _asgame_play__pc))))
  (`self.K2_SetActorLocation` (`KismetMathLibrary.MakeVector` _returnvalue_x _returnvalue_y (+ _returnvalue_z 1000.0)))
  (`KismetMaterialLibrary.SetVectorParameterValue` "/Game/Environment/Props/Materials/Collections/MPC1.MPC1" "CaptureLocation" (`KismetMathLibrary.Conv_VectorToLinearColor` (`self.K2_GetActorLocation`))))

(fn `SetCaptureSize`
  (`KismetMaterialLibrary.SetScalarParameterValue` "/Game/Environment/Props/Materials/Collections/MPC1.MPC1" "CaptureSize" (`SceneCaptureComponent2D.OrthoWidth` (`self.SceneCapture`))))

(fn `UserConstructionScript`)