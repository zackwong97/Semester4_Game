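; Cauldron prop actor that serves as the world access point for the brewing UI.
; It creates one brewing widget on BeginPlay, then adds or removes it from the viewport through OpenWidget and CloseWidget, passing in the inventory widget if none is set.
; Actor Tick drives the widget's update manually, even while it is hidden.
; Cursor hover toggles custom depth rendering on the mesh.
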(event `self.ReceiveBeginPlay`
  (bind _returnvalue (`|CreateWidget` "/Game/UI/Blueprints/BrewingWidget.BrewingWidget_C"))
  (set `self.BrewingWidget` _returnvalue))

(event `Open Widget`
  (params (`inventory widget ref` :type "/Game/UI/Blueprints/Inventory Object Reference (by ref)"))
  (bind _brewingwidget (`self.BrewingWidget`))
  (bind _brewingwidget_2 (`self.BrewingWidget`))
  (`/Game/UI/Blueprints/BrewingWidget.InventoryRef` _brewingwidget_2
    (:`then`
      _)
    (:`else`
      (set `/Game/UI/Blueprints/BrewingWidget.InventoryRef` `inventory widget ref` _brewingwidget_2)))
  (if (not (`Widget.IsInViewport` _brewingwidget))
    (`UserWidget.AddToViewport` _brewingwidget 0)))

(event `Close Widget`
  (`Widget.RemoveFromParent` (`self.BrewingWidget`)))

(event `self.ReceiveTick`
  (params (DeltaSeconds :type "Float (single-precision)"))
  (bind _brewingwidget (`self.BrewingWidget`)
    (:`then`
      (`/Game/UI/Blueprints/BrewingWidget.Tick Widget` _brewingwidget))
    (:`else`)))

(event `self.StaticMesh.OnBeginCursorOver`
  (params (TouchedComponent :type "PrimitiveComponent Object Reference"))
  (`PrimitiveComponent.SetRenderCustomDepth` (`self.StaticMesh`) true))

(event `self.StaticMesh.OnEndCursorOver`
  (params (TouchedComponent :type "PrimitiveComponent Object Reference"))
  (`PrimitiveComponent.SetRenderCustomDepth` (`self.StaticMesh`) false))

(fn `UserConstructionScript`)