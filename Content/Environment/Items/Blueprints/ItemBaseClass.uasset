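; ItemBaseClass is the base Blueprint for world items that can be picked up.
; On BeginPlay, if its quantity exceeds one, it passes itself to the QuantityText widget on its widget component.
; Outline events toggle the mesh's custom depth stencil between two values for highlighting, and a pickup event destroys the actor.
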(event `self.ReceiveBeginPlay`
  (if (> (`self.QuantityOfItem`) 1)
    (bind _asquantity_text (cast `/Game/UI/Blueprints/QuantityText` (`WidgetComponent.GetUserWidgetObject` (`self.Widget`))))
    (set `/Game/UI/Blueprints/QuantityText.ItemBaseClassRef` self _asquantity_text)))

(event `Destroy when pickup`
  (`self.K2_DestroyActor`))

(event `EnableOutline`
  (bind _staticmesh (`self.StaticMesh`))
  (if (== (`PrimitiveComponent.CustomDepthStencilValue` _staticmesh) 5)
    (`PrimitiveComponent.SetCustomDepthStencilValue` _staticmesh 15)))

(event `DisableOutline`
  (`PrimitiveComponent.SetCustomDepthStencilValue` (`self.StaticMesh`) 5))

(fn `UserConstructionScript`)