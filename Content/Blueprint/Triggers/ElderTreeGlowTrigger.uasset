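; Trigger volume that makes the Elder Tree NPC glow and switches player cameras while non-AI characters are inside it.
; Overlap begin increments a player count, starts the glow and passes the trigger's Camera to that player's controller.
; Overlap end decrements the count and clears that camera, stopping the glow when the count reaches zero.
; The glow only stops if the leaving player's controller reference is valid.
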(event `self.CollisionComponent.OnComponentBeginOverlap`
  (params (OverlappedComponent :type "PrimitiveComponent Object Reference") (OtherActor :type "Actor Object Reference") (OtherComp :type "PrimitiveComponent Object Reference") (OtherBodyIndex :type Integer) (bFromSweep :type Boolean) (SweepResult :type "HitResult Structure (by ref)"))
  (bind _asbp_character_base (cast `/Game/Characters/Player/TestCharacter2/BP_Character_Base` OtherActor))
  (if (not (`/Game/Characters/Player/TestCharacter2/BP_Character_Base.isAI?` _asbp_character_base))
    (`/Engine/EditorBlueprintResources/StandardMacros.IncrementInt` (`self.NumPlayersIn`)
      (:`  `
        (set `/Game/Dialogue/DialogueSystem/Blueprints/AI/BP_ElderTreeNPC.StartGlow` true (`self.ElderTreeNPC`))
        (bind _playercontrollerref (`/Game/Characters/Player/TestCharacter2/BP_Character_Base.PlayerControllerRef` _asbp_character_base)
          (:`then`
            (`/Game/Blueprint/GamePlay-PC.Set View Camera` _playercontrollerref (`self.Camera`)))
          (:`else`))))))

(event `self.CollisionComponent.OnComponentEndOverlap`
  (params (OverlappedComponent :type "PrimitiveComponent Object Reference") (OtherActor :type "Actor Object Reference") (OtherComp :type "PrimitiveComponent Object Reference") (OtherBodyIndex :type Integer))
  (bind _asbp_character_base (cast `/Game/Characters/Player/TestCharacter2/BP_Character_Base` OtherActor))
  (if (not (`/Game/Characters/Player/TestCharacter2/BP_Character_Base.isAI?` _asbp_character_base))
    (bind _result (`/Engine/EditorBlueprintResources/StandardMacros.DecrementInt` (`self.NumPlayersIn`))
      (:`  `
        (bind _playercontrollerref (`/Game/Characters/Player/TestCharacter2/BP_Character_Base.PlayerControllerRef` _asbp_character_base)
          (:`then`
            (`/Game/Blueprint/GamePlay-PC.Set View Camera` _playercontrollerref null)
            (if (== _result 0)
              (set `/Game/Dialogue/DialogueSystem/Blueprints/AI/BP_ElderTreeNPC.StartGlow` false (`self.ElderTreeNPC`))))
          (:`else`))))))

(fn `UserConstructionScript`)