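; BossAreaTrigger is a trigger actor that tracks players entering and leaving a boss area.
; On the authority, its collision component's overlap events filter for non-AI BP_Character_Base actors and call PlayerEnterBossArea or PlayerExitBossArea on the Gameplay_Manager.
; The manager reference is looked up via GetAllActorsOfClass on begin overlap if not yet valid, while end overlap uses it without a check.
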(event `self.CollisionComponent.OnComponentBeginOverlap`
  (params (OverlappedComponent :type "PrimitiveComponent Object Reference") (OtherActor :type "Actor Object Reference") (OtherComp :type "PrimitiveComponent Object Reference") (OtherBodyIndex :type Integer) (bFromSweep :type Boolean) (SweepResult :type "HitResult Structure (by ref)"))
  (`/Engine/EditorBlueprintResources/ActorMacros.Switch Has Authority`
    (:`Authority`
      (bind _gameplay_manager (`self.gameplay_manager`)
        (:`then`
          _)
        (:`else`
          (bind _outactors (`GameplayStatics.GetAllActorsOfClass` "/Game/Blueprint/Gameplay_Manager.Gameplay_Manager_C"))
          (set `self.gameplay_manager` (`|GetArrayItem` _outactors))))
      (bind _asbp_character_base (cast `/Game/Characters/Player/TestCharacter2/BP_Character_Base` OtherActor))
      (if (not (`/Game/Characters/Player/TestCharacter2/BP_Character_Base.isAI?` _asbp_character_base))
        (`/Game/Blueprint/Gameplay_Manager.Player Enter Boss Area` _gameplay_manager)))))

(event `self.CollisionComponent.OnComponentEndOverlap`
  (params (OverlappedComponent :type "PrimitiveComponent Object Reference") (OtherActor :type "Actor Object Reference") (OtherComp :type "PrimitiveComponent Object Reference") (OtherBodyIndex :type Integer))
  (`/Engine/EditorBlueprintResources/ActorMacros.Switch Has Authority`
    (:`Authority`
      (bind _asbp_character_base (cast `/Game/Characters/Player/TestCharacter2/BP_Character_Base` OtherActor))
      (if (not (`/Game/Characters/Player/TestCharacter2/BP_Character_Base.isAI?` _asbp_character_base))
        (`/Game/Blueprint/Gameplay_Manager.Player Exit Boss Area` (`self.gameplay_manager`))))))

(fn `UserConstructionScript`)