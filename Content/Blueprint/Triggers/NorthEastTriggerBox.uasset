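; Server-authoritative trigger box that activates an AI spawner and rewards two quest items once its enemies are gone.
; A non-AI character overlapping the box clears the spawner's DontAutoStart flag.
; Tick polls the spawner until it has hit its limit with no spawns remaining, then fires once after a short delay.
; Downward traces from two marker actors place the item drops, with spawn particles sent through every player controller.
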(event `self.ReceiveTick`
  (params (DeltaSeconds :type "Float (single-precision)"))
  (bind _aispawner (`self.AISpawner`))
  (bind _returnvalue (`self.K2_GetActorLocation` (`self.Item2SpawnLocation`)))
  (bind _returnvalue_2 (`self.K2_GetActorLocation` (`self.Item1SpawnLocation`)))
  (`/Engine/EditorBlueprintResources/ActorMacros.Switch Has Authority`
    (:`Authority`
      (if (`/Game/Blueprint/AI/AI_Spawner.HitLimit` _aispawner)
        (if (== (`/Game/Blueprint/AI/AI_Spawner.CurrentSpawn` _aispawner) 0)
          (`/Engine/EditorBlueprintResources/StandardMacros.DoOnce` false
            (:`Completed`
              (`KismetSystemLibrary.Delay` 2.0)
              (bind _outhit (`KismetSystemLibrary.LineTraceSingle` _returnvalue_2 (- _returnvalue_2 (0.0 0.0 500.0)) "TraceTypeQuery3" true))
              (bind _asgame_play__gm (cast `/Game/Blueprint/GamePlay-GM` (`GameplayStatics.GetGameMode`)))
              (for _array_element (`/Game/Blueprint/GamePlay-GM.PlayerControllersRef` _asgame_play__gm)
                (bind _asgame_play__pc (cast `/Game/Blueprint/GamePlay-PC` _array_element))
                (bind (_bblockinghit _binitialoverlap _time _distance _location) (`GameplayStatics.BreakHitResult` _outhit))
                (`/Game/Blueprint/GamePlay-PC.Spawn Particle at Location` _asgame_play__pc _location "/Game/Effects/Skills/Particles/PS_ItemSpawn.PS_ItemSpawn"))
              (`|SpawnActorFromClass` "/Game/Environment/Items/Blueprints/Quest-1_Item-17.Quest-1_Item-17_C" (`KismetMathLibrary.MakeTransform` _location) "AdjustIfPossibleButAlwaysSpawn" "OverrideRootScale" null 1 true null)
              (bind _outhit_2 (`KismetSystemLibrary.LineTraceSingle` _returnvalue (- _returnvalue (0.0 0.0 500.0)) "TraceTypeQuery3" true))
              (bind _asgame_play__gm_2 (cast `/Game/Blueprint/GamePlay-GM` (`GameplayStatics.GetGameMode`)))
              (for _array_element_2 (`/Game/Blueprint/GamePlay-GM.PlayerControllersRef` _asgame_play__gm_2)
                (bind _asgame_play__pc_2 (cast `/Game/Blueprint/GamePlay-PC` _array_element_2))
                (bind (_bblockinghit_2 _binitialoverlap_2 _time_2 _distance_2 _location_2) (`GameplayStatics.BreakHitResult` _outhit_2))
                (`/Game/Blueprint/GamePlay-PC.Spawn Particle at Location` _asgame_play__pc_2 _location_2 "/Game/Effects/Skills/Particles/PS_ItemSpawn.PS_ItemSpawn"))
              (`|SpawnActorFromClass` "/Game/Environment/Items/Blueprints/Quest-2_Item-18.Quest-2_Item-18_C" (`KismetMathLibrary.MakeTransform` _location_2) "AdjustIfPossibleButAlwaysSpawn" "OverrideRootScale" null 1 true null))))))))

(event `self.CollisionComponent.OnComponentBeginOverlap`
  (params (OverlappedComponent :type "PrimitiveComponent Object Reference") (OtherActor :type "Actor Object Reference") (OtherComp :type "PrimitiveComponent Object Reference") (OtherBodyIndex :type Integer) (bFromSweep :type Boolean) (SweepResult :type "HitResult Structure (by ref)"))
  (`/Engine/EditorBlueprintResources/ActorMacros.Switch Has Authority`
    (:`Authority`
      (bind _asbp_character_base (cast `/Game/Characters/Player/TestCharacter2/BP_Character_Base` OtherActor))
      (if (not (`/Game/Characters/Player/TestCharacter2/BP_Character_Base.isAI?` _asbp_character_base))
        (set `/Game/Blueprint/AI/AI_Spawner.Don'tAutoStart` false (`self.AISpawner`))))))

(fn `UserConstructionScript`)