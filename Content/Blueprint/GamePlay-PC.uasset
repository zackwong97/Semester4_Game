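; Gameplay player controller for a top-down, click-to-command game, driving a free camera pawn separately from the player's character.
; Right-click traces pick attack, item pickup or move, forwarded to the character through ROS events, alongside aimed skill shot and dash inputs.
; The camera pans by arrow keys or screen edges at zoom-scaled speed, toggles character follow, and uses a timeline for zoom and pitch.
; It also handles the exit menu and respawn requests to the GameMode.
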(event `Respawn Done`
  (`self.K2_SetActorLocation` (`self.CameraRef`) (`self.K2_GetActorLocation` (`self.CharacterRef`)) false true))

(event `InputAxis|Space Bar Axis`
  (params (AxisValue :type "Float (single-precision)"))
  (bind _characterref (`self.CharacterRef`))
  (bind _cameraref (`self.CameraRef`))
  ;[1 1 1] Reset Camera / Focus On Character
  (if (`self.CameraFollow`)
    (`/Engine/EditorBlueprintResources/StandardMacros.IsValid` _characterref
      (:`Is Valid`
        (`/Engine/EditorBlueprintResources/StandardMacros.IsValid` _cameraref
          (:`Is Valid`
            (`self.K2_SetActorLocation` _cameraref (`self.K2_GetActorLocation` _characterref) false true)))))))

(event `InputAction|Press SpaceBar`
  (params (Key :type "Key Structure"))
  ;[1 1 1] Reset Camera / Focus On Character
  (:`Pressed`
    (`/Engine/EditorBlueprintResources/StandardMacros.FlipFlop`
      (:`A`
        (set `self.CameraFollow` false))
      (:`B`
        (set `self.CameraFollow` true)))))

(event `InputAction|RightClick`
  (params (Key :type "Key Structure"))
  (bind (_hitresult _returnvalue) (`self.GetHitResultUnderCursorByChannel` "TraceTypeQuery4"))
  (bind (_hitresult_2 _returnvalue_2) (`self.GetHitResultUnderCursorByChannel` "TraceTypeQuery5"))
  (bind (_hitresult_3 _returnvalue_3) (`self.GetHitResultUnderCursorByChannel` "TraceTypeQuery3"))
  (bind (_bblockinghit _binitialoverlap _time _distance _location _impactpoint _normal _impactnormal _physmat _hitactor) (`GameplayStatics.BreakHitResult` _hitresult))
  (bind (_bblockinghit_2 _binitialoverlap_2 _time_2 _distance_2 _location_2) (`GameplayStatics.BreakHitResult` _hitresult_3))
  (:`Pressed`
    (if (`/Game/Characters/Player/TestCharacter2/BP_Character_Base.IsCasting?` (`self.CharacterRef`))
      _
      (elif _returnvalue
        (if (not (== _hitactor (`self.CharacterRef`)))
          (`self.ROS_Attack` _hitactor))
        (elif _returnvalue_2
          (`self.ROS_PickupItem` (`.HitActor` (`GameplayStatics.BreakHitResult` _hitresult_2)))
          (elif _returnvalue_3
            (`self.ROS_MoveToLocation` _location_2)
            (`|SpawnActorFromClass` "/Game/Effects/RightClick/BP_RightClick.BP_RightClick_C" (`KismetMathLibrary.Conv_VectorToTransform` _location_2) "Undefined" "OverrideRootScale" null null)))))))

(event `Get CameraRef & Setup UI`
  (bind _loadingscreenref (`/Game/Blueprint/MyGameInstance.LoadingScreenRef` (cast `/Game/Blueprint/MyGameInstance` (`GameplayStatics.GetGameInstance`) :!pure true)))
  ;[1 1 1] Get CameraRef & Setup UI
  (`KismetSystemLibrary.Delay` 0.1)
  (set `self.CameraRef` (cast `/Game/Blueprint/BP_CameraPawn` (`self.K2_GetPawn`) :!pure true))
  (`/Engine/EditorBlueprintResources/StandardMacros.IsValid` _loadingscreenref
    (:`Is Valid`
      (`Widget.RemoveFromParent` _loadingscreenref))
    (:`Is Not Valid`
      _))
  (bind _returnvalue (`|CreateWidget` "/Game/UI/Blueprints/MyHUD.MyHUD_C")))

(event `InputAxis|MoveFoward`
  (params (AxisValue :type "Float (single-precision)"))
  (bind _cameraref (`self.CameraRef`))
  ;[1 1 1] Keyboard Arrow Camera Movement
  (if (not (== AxisValue 0.0))
    (`/Engine/EditorBlueprintResources/StandardMacros.IsValid` _cameraref
      (:`Is Valid`
        (`self.K2_AddActorWorldOffset` _cameraref (`KismetMathLibrary.MakeVector` (* AxisValue (`self.MoveSpeed`) (`self.MoveSpeedMultipier`) (`GameplayStatics.GetWorldDeltaSeconds`))) true false)))))

(event `ROS_Attack`
  (params (Enemy :type "Actor Object Reference"))
  (`/Game/Characters/Player/TestCharacter2/BP_Character_Base.Set Enemy Target` (`self.CharacterRef`) Enemy))

(event `ROS_PickupItem`
  (params (Item :type "Actor Object Reference"))
  (`/Game/Characters/Player/TestCharacter2/BP_Character_Base.Item Pickup` (`self.CharacterRef`) Item))

(event `ROS_MoveToLocation`
  (params (Location :type "Vector Structure"))
  (`/Game/Characters/Player/TestCharacter2/BP_Character_Base.Right Click` (`self.CharacterRef`) Location))

(event `InputAxis|MoveRight`
  (params (AxisValue :type "Float (single-precision)"))
  (bind _cameraref (`self.CameraRef`))
  ;[1 1 1] Keyboard Arrow Camera Movement
  (if (not (== AxisValue 0.0))
    (`/Engine/EditorBlueprintResources/StandardMacros.IsValid` _cameraref
      (:`Is Valid`
        (`self.K2_AddActorWorldOffset` _cameraref (`KismetMathLibrary.MakeVector` 0.0 (* AxisValue (`self.MoveSpeed`) (`self.MoveSpeedMultipier`) (`GameplayStatics.GetWorldDeltaSeconds`))) true false)))))

(event `self.ReceiveBeginPlay`
  (`|ExecutionSequence`
    (:`then_0`
      (`self.Get CameraRef & Setup UI`))
    (:`then_1`
      (`self.Sent Controller Ref to Character`))))

(event `Key|H`
  (params (Key :type "Key Structure"))
  (bind _characterref (`self.CharacterRef`))
  ;[1 1 1] Reset HP
  (:`Pressed`
    (set `/Game/Characters/Player/TestCharacter2/BP_Character_Base.CurrentHealth` (`/Game/Characters/Player/TestCharacter2/BP_Character_Base.MaxHealth` _characterref) _characterref)))

(event `InputAxisKey|MouseX`
  (params (AxisValue :type "Float (single-precision)"))
  (bind _cameraref (`self.CameraRef`))
  ;[1 1 1] Mouse Edge Movement
  (`/Engine/EditorBlueprintResources/StandardMacros.IsValid` _cameraref
    (:`Is Valid`
      (bind (_mousex _mousey) (`self.MouseEdgeMovement` :!label _label)
        (:`Out X`
          (`self.K2_AddActorWorldOffset` _cameraref (`KismetMathLibrary.MakeVector` 0.0 _mousex) true false))
        (:`Out Y`
          (`self.K2_AddActorWorldOffset` _cameraref (`KismetMathLibrary.MakeVector` _mousey) true false))))
    (:`Is Not Valid`
      (`self.Get CameraRef & Setup UI` :!label _label_2))))

(event `InputAxisKey|MouseY`
  (params (AxisValue :type "Float (single-precision)"))
  ;[1 1 1] Mouse Edge Movement
  (`/Engine/EditorBlueprintResources/StandardMacros.IsValid` (`self.CameraRef`)
    (:`Is Valid`
      (goto _label :!via `Mouse Y`))
    (:`Is Not Valid`
      (goto _label_2))))

(event `Sent Controller Ref to Character`
  (`/Game/Characters/Player/TestCharacter2/BP_Character_Base.Get Controller Ref` (`self.CharacterRef`) self))

(event `Key|Escape`
  (params (Key :type "Key Structure"))
  (:`Pressed`
    (if (`self.isExitMenuOpened?`)
      (`Widget.RemoveFromParent` (`self.exitMenu`))
      (set `self.isExitMenuOpened?` false)
      (else
        (`/Engine/EditorBlueprintResources/StandardMacros.IsValid` (`self.exitMenu`)
          (:`Is Valid`
            _)
          (:`Is Not Valid`
            (bind _returnvalue (`|CreateWidget` "/Game/UI/Blueprints/ExitMenu.ExitMenu_C" self))
            (bind _output_get (set `self.exitMenu` _returnvalue))))
        (`UserWidget.AddToViewport` _output_get 0)
        (set `self.isExitMenuOpened?` true)))))

(event `InputAction|MouseScrollUp`
  (params (Key :type "Key Structure"))
  (bind _cameraref (`self.CameraRef`))
  ;[1 1 1] Zoom In / Out
  (:`Pressed`
    (`|MultiGate` false :!label _label_3
      (:`Out 0`
        (`KismetSystemLibrary.RetriggerableDelay` 2.0)
        (goto _label_3 :!via `Reset`))
      (:`Out 1`
        (bind (_direction _0_1) (`Timeline|Zoom Timeline` :!label _label_4)
          (:`Update`
            (set `SpringArmComponent.TargetArmLength` (`|EaseFunction` "EaseInOut" _0_1 (`self.MaxZoomLength`) (`self.MinZoomLength`)) (`/Game/Blueprint/BP_CameraPawn.SpringArm` _cameraref))
            (`self.K2_SetActorRotation` _cameraref (`KismetMathLibrary.MakeRotator` (.roll (`self.K2_GetActorRotation` _cameraref)) (`|EaseFunction` "EaseInOut" _0_1 0.0 (`self.ZoomRotation`)) (.yaw (`self.K2_GetActorRotation` _cameraref))) false)))))))

(event `Respawn Menu`
  (if (not (`self.isExitMenuOpened?`))
    (`/Engine/EditorBlueprintResources/StandardMacros.IsValid` (`self.exitMenu`)
      (:`Is Valid`
        _)
      (:`Is Not Valid`
        (bind _returnvalue (`|CreateWidget` "/Game/UI/Blueprints/ExitMenu.ExitMenu_C" self))
        (bind _output_get (set `self.exitMenu` _returnvalue))))
    (`UserWidget.AddToViewport` _output_get 0)
    (set `self.isExitMenuOpened?` true)))

(event `InputAction|MouseScrollDown`
  (params (Key :type "Key Structure"))
  ;[1 1 1] Zoom In / Out
  (:`Pressed`
    (`|MultiGate` false :!label _label_5
      (:`Out 0`
        (`KismetSystemLibrary.RetriggerableDelay` 2.0)
        (goto _label_5 :!via `Reset`))
      (:`Out 1`
        (goto _label_4 :!via `Reverse`)))))

(event `Respawn PC`
  (bind _asgame_play__gm (cast `/Game/Blueprint/GamePlay-GM` (`GameplayStatics.GetGameMode`)))
  (`/Game/Blueprint/GamePlay-GM.Respawn GM` _asgame_play__gm self (`self.CharacterID`)))

(event `InputAction|Press Q`
  (params (Key :type "Key Structure"))
  (bind (_locationx _locationy) (`self.GetMousePosition`))
  (:`Pressed`
    (if (`/Game/Characters/Player/TestCharacter2/BP_Character_Base.FireSkillReady?` (`self.CharacterRef`))
      (if (`self.currentlyAiming?`)
        (set `self.CurrentMouseCursor` "Default")
        (set `self.currentlyAiming?` false)
        (else
          (set `self.CurrentMouseCursor` "Crosshairs")
          (set `self.currentlyAiming?` true)))
      (`self.SetMouseLocation` (`KismetMathLibrary.FTrunc` _locationx) (`KismetMathLibrary.FTrunc` _locationy)))))

(event `InputAction|Press W`
  (params (Key :type "Key Structure"))
  ;[1 1 1] Dash Skill
  (:`Pressed`
    (`self.Call Dash Skill`)))

(event `Call Dash Skill`
  ;[1 1 1] Dash Skill
  (`/Game/Characters/Player/TestCharacter2/BP_Character_Base.Dash Skill` (`self.CharacterRef`)))

(event `InputAction|LeftClick`
  (params (Key :type "Key Structure"))
  (:`Pressed`
    (if (`/Game/Characters/Player/TestCharacter2/BP_Character_Base.IsCasting?` (`self.CharacterRef`))
      _
      (elif (`self.currentlyAiming?`)
        (set `self.currentlyAiming?` false)
        (set `self.CurrentMouseCursor` "Default")
        (`self.SkillShot_ROS` (`.Location` (`GameplayStatics.BreakHitResult` (`self.GetHitResultUnderCursorByChannel` "TraceTypeQuery6"))))))))

(event `SkillShot_ROS`
  (params (Location :type "Vector Structure (by ref)"))
  (`/Game/Characters/Player/TestCharacter2/BP_Character_Base.SkillShot` (`self.CharacterRef`) Location))

(fn `MoveSpeed`
  (returns (MoveSpeed :type "Float (double-precision)"))
  (return (/ (`SpringArmComponent.TargetArmLength` (`/Game/Blueprint/BP_CameraPawn.SpringArm` (`self.CameraRef`))) 30.0)))

(fn `UserConstructionScript`)