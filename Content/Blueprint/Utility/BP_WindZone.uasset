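; BP_WindZone is a trigger box that changes the global wind intensity when something begins overlapping it.
; It writes the GlobalWindIntensity scalar in the MPC1 material parameter collection, branching on WindSwitch.
; When on, unless already at the high value, it sets a single FInterpTo step between low and high values, with no gradual update over time.
; When off, it sets a hardcoded intensity.
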(event `self.Box.OnComponentBeginOverlap`
  (params (OverlappedComponent :type "PrimitiveComponent Object Reference") (OtherActor :type "Actor Object Reference") (OtherComp :type "PrimitiveComponent Object Reference") (OtherBodyIndex :type Integer) (bFromSweep :type Boolean) (SweepResult :type "HitResult Structure (by ref)"))
  (if (`self.windSwitch`)
    (bind _returnvalue (`KismetMaterialLibrary.GetScalarParameterValue` "/Game/Environment/Props/Materials/Collections/MPC1.MPC1" "GlobalWindIntensity"))
    (if (not (== _returnvalue (`self.highWindValue`)))
      (`KismetMaterialLibrary.SetScalarParameterValue` "/Game/Environment/Props/Materials/Collections/MPC1.MPC1" "GlobalWindIntensity" (`KismetMathLibrary.FInterpTo` (`self.lowWindValue`) (`self.highWindValue`) 1.0 0.5)))
    (else
      (`KismetMaterialLibrary.SetScalarParameterValue` "/Game/Environment/Props/Materials/Collections/MPC1.MPC1" "GlobalWindIntensity" 2.0))))

(fn `UserConstructionScript`)