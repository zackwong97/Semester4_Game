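; BP_PlayCutScene is a trigger actor that plays a referenced level sequence as a cutscene when something overlaps its Box component.
; Each overlap calls Play on the sequence and increments a PlayNumber counter, printed for debugging, until that counter equals the game mode's player count.
; The overlapping actor is not checked, so any overlap uses up one of those plays.
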(event `self.Box.OnComponentBeginOverlap`
  (params (OverlappedComponent :type "PrimitiveComponent Object Reference") (OtherActor :type "Actor Object Reference") (OtherComp :type "PrimitiveComponent Object Reference") (OtherBodyIndex :type Integer) (bFromSweep :type Boolean) (SweepResult :type "HitResult Structure (by ref)"))
  (bind _returnvalue (`GameModeBase.GetNumPlayers` (`GameplayStatics.GetGameMode`)))
  (if (not (== (`self.playNumber`) _returnvalue))
    (`MovieSceneSequencePlayer.Play` (`LevelSequenceActor.SequencePlayer` (`self.Sequence`)))
    (bind _output_get (set `self.playNumber` (+ (`self.playNumber`) 1)))
    (`KismetSystemLibrary.PrintString` (`KismetStringLibrary.Conv_IntToString` _output_get))))

(fn `UserConstructionScript`)