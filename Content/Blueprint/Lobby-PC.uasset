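; Lobby player controller that builds the lobby menu, handles Knight/Girl selection and passes session teardown and loading screen calls to the game instance.
; The player list shows Steam names and avatars, read from GameState's PlayerArray or supplied as player info through a separate widget reference.
; Character picks and releases update availability flags on the Lobby GameMode, which refreshes everyone's menu.
; Delayed retries cover an empty player array or unready widget.
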(event `Get Player List`
  (bind _lobbywidgetreference (`self.LobbyWidgetReference`))
  ;[1 1 1] Update Player List In Lobby
  (bind _aslobby__game_state (cast `/Game/Blueprint/Lobby-GameState` (`GameplayStatics.GetGameState`)))
  (`/Engine/EditorBlueprintResources/StandardMacros.IsValid` _lobbywidgetreference
    (:`Is Valid`
      (`/Game/UI/Blueprints/Lobby/LobbyMenu.Clear Player List` _lobbywidgetreference)
      (bind _playerarray (`GameStateBase.PlayerArray` _aslobby__game_state))
      (if (== (`KismetArrayLibrary.Array_Length` _playerarray) 0)
        (`KismetSystemLibrary.Delay` 0.1)
        (`self.Get Player List`)
        (else
          (for _array_element _playerarray
            (bind _uniquenetid (`AdvancedSessionsLibrary.GetUniqueNetIDFromPlayerState` _array_element))
            (bind _returnvalue (`AdvancedSteamFriendsLibrary.GetSteamPersonaName` _uniquenetid))
            (bind _returnvalue_2 (`AdvancedSteamFriendsLibrary.GetSteamFriendAvatar` _uniquenetid)
              (:`OnSuccess`
                (`/Game/UI/Blueprints/Lobby/LobbyMenu.Add Player` _lobbywidgetreference (make `SlateBrush` (75.0 75.0) (struct) (struct :`SpecifiedColor` (struct :`R` 1.0 :`G` 1.0 :`B` 1.0 :`A` 1.0) :`ColorUseRule` "UseColor_Specified") _returnvalue_2) (`KismetTextLibrary.Conv_StringToText` _returnvalue)))
              (:`OnFailure`
                (`/Game/UI/Blueprints/Lobby/LobbyMenu.Add Default` _lobbywidgetreference)))))))))

(event `Update Player List`
  (params (listOfPlayerInfo :type "Array of /Game/Blueprint/PlayerInfo Structure (by ref)"))
  (bind _lobbywidgetref (`self.LobbyWidgetRef`))
  (bind _lobbywidgetref_2 (`self.LobbyWidgetRef`))
  ;[1 1 1] Update Player List In Lobby
  (set `self.playerInfoList` listOfPlayerInfo)
  (`/Engine/EditorBlueprintResources/StandardMacros.IsValid` _lobbywidgetref_2 :!label _label
    (:`Is Valid`
      (`/Game/UI/Blueprints/Lobby/LobbyMenu.Clear Player List` _lobbywidgetref_2)
      (for _array_element (`self.playerInfoList`)
        (bind (_playeravatar _playername _steamonline_) (break `/Game/Blueprint/PlayerInfo` _array_element))
        (if _steamonline_
          (`/Game/UI/Blueprints/Lobby/LobbyMenu.Add Player` _lobbywidgetref (make `SlateBrush` (75.0 75.0) (struct) (struct :`SpecifiedColor` (struct :`R` 1.0 :`G` 1.0 :`B` 1.0 :`A` 1.0) :`ColorUseRule` "UseColor_Specified") _playeravatar) (`KismetTextLibrary.Conv_StringToText` _playername))
          (else
            (`/Game/UI/Blueprints/Lobby/LobbyMenu.Add Default` _lobbywidgetref)))))
    (:`Is Not Valid`
      (`KismetSystemLibrary.Delay` 0.1)
      (goto _label))))

(event `Get LobbyWidget Ref`
  (params (LobbyMenuRef :type "/Game/UI/Blueprints/Lobby/LobbyMenu Object Reference (by ref)"))
  ;[1 1 1] Update Player List In Lobby
  ;;[1 1 1] Get Lobby Widget BP Ref
  (set `self.LobbyWidgetRef` LobbyMenuRef))

(event `Destroy Session`
  (bind _asmy_game_instance (cast `/Game/Blueprint/MyGameInstance` (`GameplayStatics.GetGameInstance`)))
  (`/Game/Blueprint/MyGameInstance.Destroy Session` _asmy_game_instance self))

(event `Call Loading`
  (`/Game/Blueprint/MyGameInstance.ShowLoadingScreen` (cast `/Game/Blueprint/MyGameInstance` (`GameplayStatics.GetGameInstance`) :!pure true))
  (`Widget.RemoveFromParent` (`self.LobbyWidgetReference`)))

(event `self.ReceiveBeginPlay`
  ;[1 1 1] BeginPlay
  (`self.BeginPlay on Client Only`))

(event `BeginPlay on Client Only`
  ;[1 1 1] BeginPlay
  (`WidgetLayoutLibrary.RemoveAllWidgets`)
  (bind _returnvalue (`|CreateWidget` "/Game/UI/Blueprints/Lobby/LobbyMenu.LobbyMenu_C" (`GameplayStatics.GetPlayerController` 0)))
  (`UserWidget.AddToViewport` _returnvalue 0)
  (set `self.LobbyWidgetReference` _returnvalue)
  (`self.Get Player List`))

(event `Choose Character`
  (params (CharacterID :type "Integer (by ref)"))
  (bind _aslobby__gm (cast `/Game/Blueprint/Lobby-GM` (`GameplayStatics.GetGameMode`) :!pure true))
  (bind _aslobby__gm_2 (cast `/Game/Blueprint/Lobby-GM` (`GameplayStatics.GetGameMode`) :!pure true))
  ;[1 1 1] Choose Character and Update Everyone
  (switch `int` CharacterID
    (:`1`
      (if (`/Game/Blueprint/Lobby-GM.Knight Is Avaible?` _aslobby__gm_2)
        (set `/Game/Blueprint/Lobby-GM.Knight Is Avaible?` false _aslobby__gm_2)
        (`/Game/Blueprint/Lobby-GM.Everyone Update Character Menu` _aslobby__gm_2)
        (set `self.Character ID` 1)))
    (:`2`
      (if (`/Game/Blueprint/Lobby-GM.Girl Is Avaible?` _aslobby__gm)
        (set `/Game/Blueprint/Lobby-GM.Girl Is Avaible?` false _aslobby__gm)
        (`/Game/Blueprint/Lobby-GM.Everyone Update Character Menu` _aslobby__gm)
        (set `self.Character ID` 2)))))

(event `Update Character Availability`
  (params (Knight :type "Boolean (by ref)") (Girl :type "Boolean (by ref)"))
  (bind _lobbywidgetreference (`self.LobbyWidgetReference`))
  ;[1 1 1] Update Character Availability on Lobby Menu
  (`/Engine/EditorBlueprintResources/StandardMacros.IsValid` _lobbywidgetreference :!label _label_2
    (:`Is Valid`
      (`Widget.SetIsEnabled` (`/Game/UI/Blueprints/Lobby/LobbyMenu.Knight` _lobbywidgetreference) Knight)
      (`Widget.SetIsEnabled` (`/Game/UI/Blueprints/Lobby/LobbyMenu.Girl` _lobbywidgetreference) Girl))
    (:`Is Not Valid`
      (`KismetSystemLibrary.Delay` 0.2)
      (goto _label_2))))

(event `Clear Character`
  (bind _aslobby__gm (cast `/Game/Blueprint/Lobby-GM` (`GameplayStatics.GetGameMode`) :!pure true))
  ;[1 1 1] Clear Character
  (switch `int` (`self.Character ID`)
    (:`1`
      (set `/Game/Blueprint/Lobby-GM.Knight Is Avaible?` true _aslobby__gm))
    (:`2`
      (set `/Game/Blueprint/Lobby-GM.Girl Is Avaible?` true _aslobby__gm)))
  (`/Game/Blueprint/Lobby-GM.Everyone Update Character Menu` _aslobby__gm)
  (set `self.Character ID` 0))

(fn `UserConstructionScript`)