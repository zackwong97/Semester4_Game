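; Gameplay manager that directs the scripted story scenes and final Nakary boss encounter for all players.
; Scenes chain AI moves, cameras and NPC dialogue, with ContinueScene triggering one-shot follow-ups, while Tick watches for the fox's death and blends flashback post-process.
; Player counters gate the ending, where Nakary transforms into the beast boss; PlayersDied resets the fight.
; EveryoneDoSomething wraps iteration over player controllers with per-player and done outputs.
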(event `Player Enter Boss Area`
  ;[1 1 1] Ending Trigger
  (if (not (`self.PlayerEnteredBossArea`))
    (`KismetSystemLibrary.PrintString` "Player Enter")
    (bind _result (`/Engine/EditorBlueprintResources/StandardMacros.IncrementInt` (`self.PlayersInBossArea`))
      (:`  `
        (if (== (`KismetArrayLibrary.Array_Length` (`/Game/Blueprint/GamePlay-GM.PlayerControllersRef` (`self.GamemodeRef`))) _result)
          (if (`self.CheckForPotionBossArea?`)
            (for _array_element (`/Game/Blueprint/GamePlay-GM.PlayerControllersRef` (`self.GamemodeRef`))
              (bind _asgame_play__pc (cast `/Game/Blueprint/GamePlay-PC` _array_element))
              (if (>= (`|GetArrayItem` (`/Game/Blueprint/GamePlay-PC.ArrayOfItemsIndex` _asgame_play__pc) 19) 1)
                (`|ExecutionSequence`
                  (:`then_0`
                    (break))
                  (:`then_1`
                    (`self.Start Ending Scene` :!label _label)
                    (set `self.PlayerEnteredBossArea` true)
                    (set `self.PlayersInBossArea` 0)))))
            (else
              (goto _label))))))))

(event `Player Exit Boss Area`
  ;[1 1 1] Ending Trigger
  (if (not (`self.PlayerEnteredBossArea`))
    (`KismetSystemLibrary.PrintString` "Player Exit")
    (`/Engine/EditorBlueprintResources/StandardMacros.DecrementInt` (`self.PlayersInBossArea`))))

(event `self.ReceiveBeginPlay`
  (`self.Begin2`)
  (`/Engine/EditorBlueprintResources/ActorMacros.Switch Has Authority`
    (:`Authority`
      (bind _asmy_game_instance (cast `/Game/Blueprint/MyGameInstance` (`GameplayStatics.GetGameInstance`)))
      (set `self.CurrentGamemode` (`/Game/Blueprint/MyGameInstance.GameModeTypes` _asmy_game_instance))
      (bind _asgame_play__gm (cast `/Game/Blueprint/GamePlay-GM` (`GameplayStatics.GetGameMode`)))
      (set `self.GamemodeRef` _asgame_play__gm)
      (bind _asmonster_ai_controller (cast `/Game/Blueprint/AI/Monster_AI_Controller` (`Pawn.GetController` (`self.FoxMonster`))))
      (set `self.FoxAI-Controller` _asmonster_ai_controller))))

(event `Start Ending Scene`
  (bind _closestdistance (`self.ClosestDistance`))
  (bind _featurepc (`self.FeaturePC`))
  (bind _characterref (`/Game/Blueprint/GamePlay-PC.CharacterRef` _featurepc))
  (`NavModifierVolume.SetAreaClass` (`self.NakaryBeastAreaBlockEnter`) null)
  (bind _each_game_play__pc (`self.EveryoneDoSomething`)
    (:`EachOut`
      (`/Game/Blueprint/GamePlay-PC.Disable Controls` _each_game_play__pc)
      (`/Game/Blueprint/GamePlay-PC.Hide UI` _each_game_play__pc)
      (bind _characterref_2 (`/Game/Blueprint/GamePlay-PC.CharacterRef` _each_game_play__pc))
      (set `/Game/Characters/Player/TestCharacter2/BP_Character_Base.IdleState` 0 _characterref_2)
      (set `/Game/Characters/Player/TestCharacter2/BP_Character_Base.IdleStateTimerCountDown` 120.0 _characterref_2))
    (:`DoneOut`
      (bind _returnvalue (`|SpawnActorFromClass` "/Game/Characters/NPC/BP_Nakary.BP_Nakary_C" (`self.GetTransform` (`self.NakaryBeastSpawnLocation`)) "AdjustIfPossibleButAlwaysSpawn" "OverrideRootScale" null 2.0 225.0 500.0 true null 2.0 0.0 null 100.0 null))
      (bind _output_get (set `self.Nakary2Ref` _returnvalue))
      (`/Game/Characters/Player/TestCharacter2/BP_Character_Base.Play Unlock VFX` _output_get "/Game/Effects/Skills/Particles/PS_Darkness.PS_Darkness")
      (bind _each_game_play__pc_2 (`self.EveryoneDoSomething`)
        (:`EachOut`
          (if (== _closestdistance 0.0)
            (bind _returnvalue_2 (`self.GetDistanceTo` (`/Game/Blueprint/GamePlay-PC.CharacterRef` _each_game_play__pc_2) (`self.EndingP1_Location`)))
            (set `self.ClosestDistance` _returnvalue_2)
            (set `self.FeaturePC` _each_game_play__pc_2)
            (elif (< _returnvalue_2 _closestdistance)
              (set `self.ClosestDistance` _returnvalue_2)
              (set `self.FeaturePC` _each_game_play__pc_2))))
        (:`DoneOut`
          (bind _movementresult (`|AIMoveTo` _characterref _characterref (`self.K2_GetActorLocation` (`self.EndingP1_Location`)) null :!label _label_2)
            (:`then`
              (bind _each_game_play__pc_3 (`self.EveryoneDoSomething`)
                (:`EachOut`
                  (if (!= _each_game_play__pc_3 _featurepc)
                    (bind _characterref_3 (`/Game/Blueprint/GamePlay-PC.CharacterRef` _each_game_play__pc_3))
                    (bind _movementresult_2 (`|AIMoveTo` _characterref_3 _characterref_3 (`self.K2_GetActorLocation` (`self.EndingP2_Location`)) null :!label _label_3)
                      (:`OnSuccess`
                        (`KismetSystemLibrary.PrintString` "Player 2 Reach")
                        (`self.PlayersReach`))
                      (:`OnFail`
                        (`KismetSystemLibrary.PrintString` (`|GetEnumeratorNameAsString` _movementresult_2))
                        (goto _label_3)))))))
            (:`OnSuccess`
              (`KismetSystemLibrary.PrintString` "Player 1 Reach")
              (`self.PlayersReach`))
            (:`OnFail`
              (`KismetSystemLibrary.PrintString` (`|GetEnumeratorNameAsString` _movementresult))
              (goto _label_2))))))))

(event `Boss Died`)

(event `Finish Setup`
  (params (`Gameplay-Pc` :type "/Game/Blueprint/GamePlay-PC Object Reference (by ref)"))
  (switch `int` (`self.CurrentGamemode`)
    (:`1`
      (bind _result (`/Engine/EditorBlueprintResources/StandardMacros.IncrementInt` (`self.FinishedPlayers`))
        (:`  `
          (`KismetSystemLibrary.Delay` 1.0)
          (if (== _result (`KismetArrayLibrary.Array_Length` (`GameStateBase.PlayerArray` (`GameplayStatics.GetGameState`))))
            (if (`self.StartStory?`)
              (`self.Start Scene-1`)
              (else
                (bind _each_game_play__pc (`self.EveryoneDoSomething`)
                  (:`EachOut`
                    (`/Game/Blueprint/GamePlay-PC.Set Skill Availability` _each_game_play__pc true true true true)))))))))
    (:`2`
      (`/Game/Blueprint/GamePlay-PC.Show UI` `Gameplay-Pc` :!label _label_4))
    (:`3`
      (goto _label_4))))

(event `Continue Scene`
  (params (num :type Integer))
  (switch `int` num
    (:`0`
      (`/Engine/EditorBlueprintResources/StandardMacros.DoOnce` false
        (:`Completed`
          (`self.Continue0`))))
    (:`1`
      (`/Engine/EditorBlueprintResources/StandardMacros.DoOnce` false
        (:`Completed`
          (`self.Continue1`))))
    (:`2`
      (`/Engine/EditorBlueprintResources/StandardMacros.DoOnce` false
        (:`Completed`
          (`self.Continue2`))))
    (:`3`
      (`/Engine/EditorBlueprintResources/StandardMacros.DoOnce` false
        (:`Completed`
          (`self.Continue3`))))
    (:`4`
      (`/Engine/EditorBlueprintResources/StandardMacros.DoOnce` false
        (:`Completed`
          (`self.Continue4`))))
    (:`5`
      (`/Engine/EditorBlueprintResources/StandardMacros.DoOnce` false
        (:`Completed`
          (`self.Continue5`))))
    (:`6`
      (`/Engine/EditorBlueprintResources/StandardMacros.DoOnce` false
        (:`Completed`
          (`self.Continue6`))))
    (:`7`
      (`/Engine/EditorBlueprintResources/StandardMacros.DoOnce` false
        (:`Completed`
          (`self.continue7`))))))

(event `PlayersDied`
  (set `self.PlayersInBossArea` 0)
  (set `self.PlayerEnteredBossArea` false)
  (`KismetSystemLibrary.Delay` 2.0)
  (set `self.hasBossFightStarted?` false)
  (bind _each_game_play__pc (`self.EveryoneDoSomething`)
    (:`EachOut`
      (`/Game/Blueprint/GamePlay-PC.Respawn PC` _each_game_play__pc))
    (:`DoneOut`
      (`/Game/Characters/Player/TestCharacter2/BP_Character_Base.Kill` (`self.NakaryBeastRef`)))))

(event `EveryoneContinue`
  (`self.EveryoneContinueDialogue`))

(event `Start Scene-1`
  (bind _each_game_play__pc (`self.EveryoneDoSomething`)
    (:`EachOut`
      (`self.ROC_Scene-1` _each_game_play__pc))))

(event `PlayersReach`
  (bind _nakary2ref (`self.Nakary2Ref`))
  (bind _result (`/Engine/EditorBlueprintResources/StandardMacros.IncrementInt` (`self.PlayersInBossArea`))
    (:`  `
      (if (>= _result (`KismetArrayLibrary.Array_Length` (`/Game/Blueprint/GamePlay-GM.PlayerControllersRef` (`self.GamemodeRef`))))
        (`KismetSystemLibrary.PrintString` "All reach")
        (bind _each_game_play__pc (`self.EveryoneDoSomething`)
          (:`EachOut`
            (`/Game/Blueprint/GamePlay-PC.Set View Camera` _each_game_play__pc (`self.EndingCamera`))
            (`NavModifierVolume.SetAreaClass` (`self.NakaryBeastAreaBlockEnter`) "/Script/NavigationSystem.NavArea_Null"))
          (:`DoneOut`
            (`KismetSystemLibrary.Delay` 2.0)
            (`|AIMoveTo` _nakary2ref _nakary2ref (`self.K2_GetActorLocation` (`self.EndingNakaryMoveToLocation`)) null
              (:`OnSuccess`
                _)
              (:`OnFail`
                _))
            (if (`self.EndingStoryStarted?`)
              (`self.continue7`)
              (else
                (bind _each_game_play__pc_2 (`self.EveryoneDoSomething`)
                  (:`EachOut`
                    (if (== (`/Game/Blueprint/GamePlay-PC.CharacterID` _each_game_play__pc_2) 2)
                      (set `self.otoyoInGame` true)
                      (else
                        (set `self.opiyoInGame` true))))
                  (:`DoneOut`
                    (bind _asbp_ending_npc (cast `/Game/Dialogue/DialogueSystem/Blueprints/AI/BP_EndingNPC` (`self.EndingNPC`)))
                    (`/Game/Dialogue/DialogueSystem/Blueprints/AI/BP_EndingNPC.Set Characters Name` _asbp_ending_npc (`self.opiyoInGame`) (`self.otoyoInGame`))
                    (bind _each_game_play__pc_3 (`self.EveryoneDoSomething`)
                      (:`EachOut`
                        (`/Game/Blueprint/GamePlay-PC.Talk to NPC` _each_game_play__pc_3 _asbp_ending_npc 1)))))))))))))

(event `ROC_Scene-1`
  (params (PC :type "/Game/Blueprint/GamePlay-PC Object Reference") (NarratorNum :type Integer))
  (`/Game/Blueprint/GamePlay-PC.Talk to NPC` PC (`self.narratorNPC`) NarratorNum))

(event `self.ReceiveTick`
  (params (DeltaSeconds :type "Float (single-precision)"))
  (bind _postprocess (`self.PostProcess`))
  (bind _blendweight (`PostProcessVolume.BlendWeight` _postprocess))
  (`|ExecutionSequence`
    (:`then_0`
      (`/Engine/EditorBlueprintResources/ActorMacros.Switch Has Authority`
        (:`Authority`
          (`KismetSystemLibrary.Delay` 0.5)
          (if (`self.CheckFox`)
            (`self.FoxMonster`
              (:`then`)
              (:`else`
                (bind _block1 (`self.Block1`)
                  (:`then`
                    (`self.K2_DestroyActor` _block1))
                  (:`else`
                    (set `self.CheckFox` false)
                    (`/Engine/EditorBlueprintResources/StandardMacros.DoOnce` false
                      (:`Completed`
                        (`self.Start Scene4`)))))))))))
    (:`then_1`
      (if (`self.StartFlashBackPP`)
        (if (not (== _blendweight 1.0))
          (bind _output_get (set `PostProcessVolume.BlendWeight` (+ (/ (`GameplayStatics.GetWorldDeltaSeconds`) (`self.FlashBackPP_BlendTime`)) _blendweight) _postprocess))
          (if (>= _output_get 1.0)
            (set `PostProcessVolume.BlendWeight` 1.0 _postprocess)))
        (elif (not (== _blendweight 0.0))
          (bind _output_get_2 (set `PostProcessVolume.BlendWeight` (- _blendweight (/ (`GameplayStatics.GetWorldDeltaSeconds`) (`self.FlashBackPP_BlendTime`))) _postprocess))
          (if (<= _output_get_2 0.0)
            (set `PostProcessVolume.BlendWeight` 0.0 _postprocess)))))))

(event `Start Scene3`
  (params (PC :type "/Game/Blueprint/GamePlay-PC Object Reference"))
  (bind _foxmonster (`self.FoxMonster`))
  (bind _output_get (set `self.FeaturePC` PC))
  (for _array_element (`/Game/Blueprint/GamePlay-GM.PlayerControllersRef` (`self.GamemodeRef`))
    (bind _asgame_play__pc (cast `/Game/Blueprint/GamePlay-PC` _array_element))
    (if (== (`/Game/Blueprint/GamePlay-PC.SceneState` _asgame_play__pc) 1)
      (`/Game/Blueprint/GamePlay-PC.Hide UI` _asgame_play__pc)
      (`/Game/Blueprint/GamePlay-PC.Disable Controls` _asgame_play__pc)
      (`PlayerController.SetViewTargetWithBlend` _asgame_play__pc (`self.Scene3Cam`) 2.0 "VTBlend_Cubic" 0.0 false)))
  (bind _characterref (`/Game/Blueprint/GamePlay-PC.CharacterRef` _output_get))
  (set `/Game/Characters/Player/TestCharacter2/BP_Character_Base.IdleState` 0 _characterref)
  (set `/Game/Characters/Player/TestCharacter2/BP_Character_Base.IdleStateTimerCountDown` (`/Game/Characters/Player/TestCharacter2/BP_Character_Base.IdleStateTimer` _characterref) _characterref)
  (`|AIMoveTo` _characterref _characterref (`self.K2_GetActorLocation` (`self.FirstP-Scene3-MoveToLocation`)) null 0.0
    (:`OnSuccess`
      _)
    (:`OnFail`
      _))
  (`|AIMoveTo` _foxmonster _foxmonster (`self.K2_GetActorLocation` (`self.Mob-Scene3-MoveToLocation`)) null
    (:`OnSuccess`
      _)
    (:`OnFail`
      _))
  (set `/Game/Characters/Player/TestCharacter2/BP_Character_Base.CurrentEnemyTarget` _characterref _foxmonster)
  (`KismetSystemLibrary.K2_SetTimer` _foxmonster "TurnToTarget" 0.01 true)
  (for _array_element_2 (`/Game/Blueprint/GamePlay-GM.PlayerControllersRef` (`self.GamemodeRef`))
    (bind _asgame_play__pc_2 (cast `/Game/Blueprint/GamePlay-PC` _array_element_2))
    (if (== (`/Game/Blueprint/GamePlay-PC.SceneState` _asgame_play__pc_2) 1)
      (`self.ROC_Scene-1` _asgame_play__pc_2 1))))

(event `Begin2`)

(event `Continue0`
  (bind _foxmonster (`self.FoxMonster`))
  (bind _characterref (`/Game/Blueprint/GamePlay-PC.CharacterRef` (`self.FeaturePC`)))
  (bind _characterref_2 (`/Game/Blueprint/GamePlay-PC.CharacterRef` (stale `Start Scene3` _output_get)))
  (`KismetSystemLibrary.K2_ClearTimer` _characterref_2 "TurnToTarget")
  (`/Game/Characters/Player/TestCharacter2/BP_Character_Base.Set Enemy Target` _foxmonster _characterref_2)
  (if (`/Game/Characters/Player/TestCharacter2/BP_Character_Base.Attacking?` _foxmonster) :!label _label_5
    (`/Game/Characters/Player/TestCharacter2/BP_Character_Base.Stop All Movement and Targets` _foxmonster)
    (set `/Game/Characters/Player/TestCharacter2/BP_Character_Base.IdleState` 0 _characterref)
    (set `/Game/Characters/Player/TestCharacter2/BP_Character_Base.IdleStateTimerCountDown` (`/Game/Characters/Player/TestCharacter2/BP_Character_Base.IdleStateTimer` _characterref) _characterref)
    (`|AIMoveTo` _characterref (`self.K2_GetActorLocation` (`self.Scene3-FirstP_MoveBackLocation`)) null
      (:`OnSuccess`
        _)
      (:`OnFail`
        _))
    (set `/Game/Characters/Player/TestCharacter2/BP_Character_Base.CurrentEnemyTarget` (`self.FoxMonster`) _characterref)
    (`KismetSystemLibrary.K2_SetTimer` _characterref "TurnToTarget" 0.01 true)
    (`KismetSystemLibrary.Delay` 1.0)
    (`KismetSystemLibrary.K2_ClearTimer` _characterref "TurnToTarget")
    (set `/Game/Characters/Player/TestCharacter2/BP_Character_Base.IdleState` 2 _characterref)
    (set `/Game/Characters/Player/TestCharacter2/BP_Character_Base.IdleStateTimerCountDown` (`/Game/Characters/Player/TestCharacter2/BP_Character_Base.IdleStateTimer` _characterref) _characterref)
    (`KismetSystemLibrary.Delay` 1.0)
    (for _array_element (`/Game/Blueprint/GamePlay-GM.PlayerControllersRef` (`self.GamemodeRef`))
      (bind _asgame_play__pc (cast `/Game/Blueprint/GamePlay-PC` _array_element))
      (if (== (`/Game/Blueprint/GamePlay-PC.SceneState` _asgame_play__pc) 1)
        (`/Game/Blueprint/GamePlay-PC.Ping NPC` _asgame_play__pc 0 0)))
    (bind _asmonster_ai_controller (cast `/Game/Blueprint/AI/Monster_AI_Controller` (`Pawn.GetController` (`self.FoxMonster`))))
    (`/Game/Blueprint/AI/Monster_AI_Controller.Set target from NakaryBeast` _asmonster_ai_controller (`/Game/Blueprint/GamePlay-PC.CharacterRef` (`self.FeaturePC`)))
    (set `self.CheckFox` true)
    (else
      (`KismetSystemLibrary.Delay` 2.0)
      (goto _label_5))))

(event `Continue6`
  (bind _featurepc (`self.FeaturePC`))
  (bind _characterref (`/Game/Blueprint/GamePlay-PC.CharacterRef` _featurepc))
  (set `self.PlayersInBossArea` 0)
  (bind _each_game_play__pc (`self.EveryoneDoSomething`)
    (:`EachOut`
      (bind _characterref_2 (`/Game/Blueprint/GamePlay-PC.CharacterRef` _each_game_play__pc))
      (set `/Game/Characters/Player/TestCharacter2/BP_Character_Base.IdleState` 0 _characterref_2)
      (set `/Game/Characters/Player/TestCharacter2/BP_Character_Base.IdleStateTimerCountDown` 120.0 _characterref_2))
    (:`DoneOut`
      (`|AIMoveTo` _characterref _characterref (`self.K2_GetActorLocation` (`self.EndingP1_FrontStep`)) null
        (:`then`
          (bind _each_game_play__pc_2 (`self.EveryoneDoSomething`)
            (:`EachOut`
              (if (!= _each_game_play__pc_2 _featurepc)
                (bind _characterref_3 (`/Game/Blueprint/GamePlay-PC.CharacterRef` _each_game_play__pc_2))
                (`|AIMoveTo` _characterref_3 _characterref_3 (`self.K2_GetActorLocation` (`self.EndingP2_FrontStep`)) null
                  (:`OnSuccess`
                    _)
                  (:`OnFail`
                    _))
                (`self.PlayerStepForward`)))))
        (:`OnSuccess`
          (`self.PlayerStepForward` :!label _label_6))
        (:`OnFail`
          (goto _label_6))))))

(event `Start Scene4`
  (for _array_element (`/Game/Blueprint/GamePlay-GM.PlayerControllersRef` (`self.GamemodeRef`))
    (bind _asgame_play__pc (cast `/Game/Blueprint/GamePlay-PC` _array_element))
    (if (`KismetMathLibrary.InRange_IntInt` (`/Game/Blueprint/GamePlay-PC.SceneState` _asgame_play__pc) 1 2)
      (`self.ROC_Scene-1` _asgame_play__pc 2))))

(event `Continue1`)

(event `PlayerStepForward`
  (bind _result (`/Engine/EditorBlueprintResources/StandardMacros.IncrementInt` (`self.PlayersInBossArea`))
    (:`  `
      (if (>= _result (`KismetArrayLibrary.Array_Length` (`/Game/Blueprint/GamePlay-GM.PlayerControllersRef` (`self.GamemodeRef`))))
        (`/Engine/EditorBlueprintResources/StandardMacros.DoOnce` false
          (:`Completed`
            (bind _each_game_play__pc (`self.EveryoneDoSomething`)
              (:`EachOut`
                (`/Game/Blueprint/GamePlay-PC.Ping NPC` _each_game_play__pc 1 0)))))))))

(event `Start Scene 5`
  (params (TriggerPlayerController :type "/Game/Blueprint/GamePlay-PC Object Reference (by ref)"))
  (bind _nakaryref (`self.NakaryRef`))
  ;[1 1 1] Scene 5
  (set `self.FeaturePC` TriggerPlayerController)
  (for _array_element (`/Game/Blueprint/GamePlay-GM.PlayerControllersRef` (`self.GamemodeRef`))
    (bind _asgame_play__pc (cast `/Game/Blueprint/GamePlay-PC` _array_element))
    (if (`KismetMathLibrary.InRange_IntInt` (`/Game/Blueprint/GamePlay-PC.SceneState` _asgame_play__pc) 1 3)
      (`/Game/Blueprint/GamePlay-PC.Disable Controls` _asgame_play__pc)
      (`/Game/Blueprint/GamePlay-PC.Hide UI` _asgame_play__pc)
      (`PlayerController.SetViewTargetWithBlend` _asgame_play__pc (`self.Scene5-Cam`) 2.0 "VTBlend_Cubic" 0.0 false)))
  (set `self.StartFlashBackPP` true)
  (`|AIMoveTo` _nakaryref _nakaryref (`self.K2_GetActorLocation` (`self.Scene5-NakaryMove`)) null
    (:`OnSuccess`
      _)
    (:`OnFail`
      _))
  (set `/Game/Characters/Player/TestCharacter2/BP_Character_Base.CurrentEnemyTarget` (`/Game/Blueprint/GamePlay-PC.CharacterRef` (`self.FeaturePC`)) _nakaryref)
  (`KismetSystemLibrary.K2_SetTimer` _nakaryref "TurnToTarget" 0.02 true)
  (for _array_element_2 (`/Game/Blueprint/GamePlay-GM.PlayerControllersRef` (`self.GamemodeRef`))
    (bind _asgame_play__pc_2 (cast `/Game/Blueprint/GamePlay-PC` _array_element_2))
    (if (`KismetMathLibrary.InRange_IntInt` (`/Game/Blueprint/GamePlay-PC.SceneState` _asgame_play__pc_2) 1 3)
      (`self.ROC_Scene-1` _asgame_play__pc_2 3))))

(event `Continue3`
  ;[1 1 1] Scene 5
  (`KismetSystemLibrary.Delay` 0.2)
  (bind _each_game_play__pc (`self.EveryoneDoSomething`)
    (:`EachOut`
      (`/Game/Blueprint/GamePlay-PC.Ping NPC` _each_game_play__pc 3 (`/Game/Blueprint/GamePlay-PC.CharacterID` (`self.FeaturePC`))))))

(event `continue7`
  (bind _nakarybeastref (`self.NakaryBeastRef`))
  (`self.SpawnTransformVFX`)
  (set `self.Nakary2Location` (`self.GetTransform` (`self.Nakary2Ref`)))
  (`KismetSystemLibrary.Delay` 1.5)
  (`self.K2_DestroyActor` (`self.Nakary2Ref`))
  (bind _returnvalue (`|SpawnActorFromClass` "/Game/Blueprint/AI/BP_NakaryBeast.BP_NakaryBeast_C" (`KismetMathLibrary.MakeTransform` (.location (`self.Nakary2Location`)) (.rotation (`self.Nakary2Location`))) "AdjustIfPossibleButAlwaysSpawn" "OverrideRootScale" null self 2.0 350.0 1000.0 true null 2.0 0.0 null 100.0 null))
  (`SceneComponent.SetVisibility` (`/Game/Characters/Player/TestCharacter2/BP_Character_Base.HealthBar` _returnvalue) false false)
  (set `self.NakaryBeastRef` _returnvalue)
  (`KismetSystemLibrary.Delay` 2.5)
  (bind _each_game_play__pc (`self.EveryoneDoSomething`)
    (:`EachOut`
      (if (`self.EndingStoryStarted?`)
        (`/Game/Blueprint/GamePlay-PC.Enable Controls` _each_game_play__pc)
        (`/Game/Blueprint/GamePlay-PC.Show UI` _each_game_play__pc)
        (`/Game/Blueprint/GamePlay-PC.Set View Camera` _each_game_play__pc null)
        (else
          (`/Game/Blueprint/GamePlay-PC.Ping NPC` _each_game_play__pc 2 0))))
    (:`DoneOut`
      (`KismetSystemLibrary.Delay` 1.0)
      (`SceneComponent.SetVisibility` (`/Game/Characters/Player/TestCharacter2/BP_Character_Base.HealthBar` _nakarybeastref) false false)
      (bind _asnakary_beast_ai_controller (cast `/Game/Blueprint/AI/NakaryBeast_AI_Controller` (`Pawn.GetController` _nakarybeastref)))
      (`/Game/Blueprint/AI/NakaryBeast_AI_Controller.StartAI` _asnakary_beast_ai_controller)
      (set `self.hasBossFightStarted?` true)
      (set `self.EndingStoryStarted?` true))))

(event `Continue4`
  ;[1 1 1] Scene 5
  (`KismetSystemLibrary.Delay` 0.2)
  (bind _each_game_play__pc (`self.EveryoneDoSomething`)
    (:`EachOut`
      (`/Game/Blueprint/GamePlay-PC.Ping NPC` _each_game_play__pc 4 0))))

(event `SpawnTransformVFX`
  (`GameplayStatics.SpawnEmitterAtLocation` "/Game/Effects/Skills/Particles/PS_FlashTransform.PS_FlashTransform" (+ (`self.K2_GetActorLocation` (`self.Nakary2Ref`)) (0.0 0.0 75.0))))

(event `Continue5`
  (bind _nakaryref (`self.NakaryRef`))
  ;[1 1 1] Scene 5
  (`|AIMoveTo` _nakaryref _nakaryref (`self.K2_GetActorLocation` (`self.NakaryDissapearLocation`)) null
    (:`OnSuccess`
      _)
    (:`OnFail`
      _))
  (bind _nakaryref_2 (`self.NakaryRef`)
    (:`then`
      (`self.K2_DestroyActor` _nakaryref_2)
      (set `self.StartFlashBackPP` false)
      (bind _each_game_play__pc (`self.EveryoneDoSomething`)
        (:`EachOut`
          (`/Game/Blueprint/GamePlay-PC.Ping NPC` _each_game_play__pc 5 0))))
    (:`else`)))

(event `Continue2`
  (bind _nakaryref (`self.NakaryRef`))
  (bind _characterref (`/Game/Blueprint/GamePlay-PC.CharacterRef` (`self.FeaturePC`)))
  ;[1 1 1] Scene 5
  (set `/Game/Characters/Player/TestCharacter2/BP_Character_Base.IdleState` 0 _characterref)
  (set `/Game/Characters/Player/TestCharacter2/BP_Character_Base.IdleStateTimerCountDown` (`/Game/Characters/Player/TestCharacter2/BP_Character_Base.IdleStateTimer` _characterref) _characterref)
  (`|AIMoveTo` _characterref (`self.K2_GetActorLocation` (`self.Scene4-NakaryMove`)) null
    (:`OnSuccess`
      _)
    (:`OnFail`
      _))
  (set `/Game/Characters/Player/TestCharacter2/BP_Character_Base.CurrentEnemyTarget` _nakaryref _characterref)
  (`KismetSystemLibrary.K2_SetTimer` _characterref "TurnToTarget" 0.01 true)
  (`KismetSystemLibrary.K2_ClearTimer` _nakaryref "TurnToTarget")
  (for _array_element (`/Game/Blueprint/GamePlay-GM.PlayerControllersRef` (`self.GamemodeRef`))
    (bind _asgame_play__pc (cast `/Game/Blueprint/GamePlay-PC` _array_element))
    (`/Game/Blueprint/GamePlay-PC.Ping NPC` _asgame_play__pc 2 0))
  (`KismetSystemLibrary.K2_ClearTimer` _characterref "TurnToTarget"))

(fn `UserConstructionScript`)