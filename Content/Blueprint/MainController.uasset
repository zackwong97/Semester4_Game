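; MainController is a player controller for a detached, top-down-style camera that spawns a BP_Character_Base and forwards right-clicks to it.
; It moves the BP_CameraPawn by axis input or screen-edge mouse checks in a MouseEdgeMovement macro, scaling speed with spring arm length.
; Space snaps the camera to the character.
; A second scroll within a MultiGate's delay window plays or reverses a timeline easing zoom and pitch.
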(event `self.ReceiveBeginPlay`
  (`WidgetBlueprintLibrary.SetInputMode_GameAndUIEx` self null "LockAlways" false)
  (set `self.bShowMouseCursor` true)
  (bind _returnvalue (`|SpawnActorFromClass` "/Game/Characters/Player/TestCharacter2/BP_Character_Base.BP_Character_Base_C" (`KismetMathLibrary.Conv_VectorToTransform` (`self.K2_GetActorLocation` (`self.K2_GetPawn`))) "Undefined" "OverrideRootScale" null null))
  (set `self.CharacterRef` _returnvalue)
  (set `self.CameraRef` (cast `/Game/Blueprint/BP_CameraPawn` (`self.K2_GetPawn`) :!pure true)))

(event `InputAction|Press SpaceBar`
  (params (Key :type "Key Structure"))
  ;[1 1 1] Reset Camera / Focus on Character
  (:`Pressed`
    (`self.K2_SetActorLocation` (`self.CameraRef`) (`self.K2_GetActorLocation` (`self.CharacterRef`)) false true)))

(event `InputAction|Press Q`
  (params (Key :type "Key Structure")))

(event `InputAxis|MoveFoward`
  (params (AxisValue :type "Float (single-precision)"))
  ;[1 1 1] Keyboard Camera Movement
  (`self.K2_AddActorWorldOffset` (`self.CameraRef`) (`KismetMathLibrary.MakeVector` (* AxisValue (`self.MoveSpeed`) (`self.MoveSpeedMultipier`) 1.5)) true false))

(event `InputAction|RightClick`
  (params (Key :type "Key Structure"))
  (:`Pressed`
    (`/Game/Characters/Player/TestCharacter2/BP_Character_Base.Right Click` (`self.CharacterRef`))))

(event `InputAxis|MoveRight`
  (params (AxisValue :type "Float (single-precision)"))
  ;[1 1 1] Keyboard Camera Movement
  (`self.K2_AddActorWorldOffset` (`self.CameraRef`) (`KismetMathLibrary.MakeVector` 0.0 (* AxisValue (`self.MoveSpeed`) (`self.MoveSpeedMultipier`) 1.5)) true false))

(event `InputAxisKey|MouseX`
  (params (AxisValue :type "Float (single-precision)"))
  ;[1 1 1] Mouse Edge Movement
  (bind (_mousex _mousey) (`self.MouseEdgeMovement` :!label _label)
    (:`Out`
      (`self.K2_AddActorWorldOffset` (`self.CameraRef`) (`KismetMathLibrary.MakeVector` _mousey _mousex) true false))))

(event `InputAxisKey|MouseY`
  (params (AxisValue :type "Float (single-precision)"))
  ;[1 1 1] Mouse Edge Movement
  (goto _label :!via `Mouse Y`))

(event `InputAction|MouseScrollUp`
  (params (Key :type "Key Structure"))
  (bind _cameraref (`self.CameraRef`))
  ;[1 1 1] Zoom In / Out
  (:`Pressed`
    (`|MultiGate` false :!label _label_2
      (:`Out 0`
        (`KismetSystemLibrary.RetriggerableDelay` 2.0)
        (goto _label_2 :!via `Reset`))
      (:`Out 1`
        (bind (_direction _0_1) (`Timeline|Arm Length` :!label _label_3)
          (:`Update`
            (set `SpringArmComponent.TargetArmLength` (`|EaseFunction` "EaseInOut" _0_1 (`self.MaxZoomLength`) (`self.MinZoomLength`)) (`/Game/Blueprint/BP_CameraPawn.SpringArm` _cameraref))
            (`self.K2_SetActorRotation` _cameraref (`KismetMathLibrary.MakeRotator` (.roll (`self.K2_GetActorRotation` _cameraref)) (`|EaseFunction` "SinusoidalInOut" _0_1 0.0 (`self.ZoomRotation`)) (.yaw (`self.K2_GetActorRotation` _cameraref))) false)))))))

(event `InputAction|MouseScrollDown`
  (params (Key :type "Key Structure"))
  ;[1 1 1] Zoom In / Out
  (:`Pressed`
    (`|MultiGate` false :!label _label_4
      (:`Out 0`
        (`KismetSystemLibrary.RetriggerableDelay` 2.0)
        (goto _label_4 :!via `Reset`))
      (:`Out 1`
        (goto _label_3 :!via `Reverse`)))))

(fn `MoveSpeed`
  (returns (MoveSpeed :type "Float (double-precision)"))
  (return (/ (`SpringArmComponent.TargetArmLength` (`/Game/Blueprint/BP_CameraPawn.SpringArm` (`self.CameraRef`))) 100.0)))

(fn `OnRep_CameraRef`)

(fn `OnRep_CharacterRef`)

(fn `UserConstructionScript`)