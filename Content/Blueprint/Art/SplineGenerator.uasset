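; Spline-driven mesh generator that builds cable or track-like geometry in the construction script, with optional end caps and debug point labels and arrows.
; It syncs per-point roll, scale and detail data to the spline, then BuildTrackElement creates a spline mesh per segment, with detail meshes replacing or overlaying the body.
; DynamicMaterialBuild feeds segment distances to each material to fix texture distortion.
; Looping splines get roll correction on the closing segment.
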(fn `BuildTrackElement`
  (params (LoopIndex :type Integer) (TrackElementMesh :type "StaticMesh Object Reference") (IsDetail :type Boolean))
  (returns (SplineMesh :type "SplineMeshComponent Object Reference"))
  (locals (Local_CurrentLoopIndex :type Integer) (Local_NextLoopIndex :type Integer :default 0) (Local_TrackElementMesh :type "StaticMesh Object Reference") (Local_StartLocation :type "Vector Structure" :default (0.0 0.0 0.0)) (Local_StartTangent :type "Vector Structure" :default (0.0 0.0 0.0)) (Local_EndLocation :type "Vector Structure") (Local_EndTangent :type "Vector Structure") (Local_CurrentSplineMesh :type "SplineMeshComponent Object Reference") (Local_StartRoll :type "Float (double-precision)") (Local_StartScale :type "Vector2D Structure") (Local_EndScale :type "Vector2D Structure") (Local_EndRoll :type "Float (double-precision)") (Local_Start :type "Float (double-precision)") (Local_LastLoop :type Boolean) (Local_IncrementalRoll :type "Float (double-precision)") (Local_LastLoopRoll :type "Float (double-precision)") (Local_Isdetail :type Boolean))
  (bind _local_currentloopindex (`local.Local_CurrentLoopIndex`))
  (bind _spline (`self.Spline`))
  (bind _returnvalue (`SplineComponent.GetUpVectorAtSplinePoint` _spline _local_currentloopindex "Local"))
  (bind (_location _tangent) (`SplineComponent.GetLocationAndTangentAtSplinePoint` (`self.Spline`) (`local.Local_NextLoopIndex`) "Local"))
  (bind (_location_2 _tangent_2) (`SplineComponent.GetLocationAndTangentAtSplinePoint` (`self.Spline`) (`local.Local_CurrentLoopIndex`) "Local"))
  (bind _returnvalue_2 (* (`local.Local_EndScale`) (`self.MainScale`)))
  (bind _returnvalue_3 (* (`local.Local_StartScale`) (`self.MainScale`)))
  (bind (_output_detail _output_roll _output_scale) (break `/Game/Blueprint/Art/SplineData` (`|GetArrayItem` (`self.SplineDataArray`) (`local.Local_CurrentLoopIndex`))))
  (bind (_output_detail_2 _output_roll_2 _output_scale_2) (break `/Game/Blueprint/Art/SplineData` (`|GetArrayItem` (`self.SplineDataArray`) (`local.Local_NextLoopIndex`))))
  (bind _returnvalue_4 (+ (`local.Local_EndRoll`) (* (`local.Local_NextLoopIndex`) (`self.IncrementalRoll`))))
  (bind _returnvalue_5 (mod (+ (`local.Local_StartRoll`) (* (`local.Local_CurrentLoopIndex`) (`self.IncrementalRoll`))) (* (`KismetMathLibrary.GetPI`) 2.0)))
  (bind _returnvalue_6 (select `bool` (`local.Local_LastLoop`) :`false` (+ (`local.Local_StartRoll`) (* (`local.Local_CurrentLoopIndex`) (`self.IncrementalRoll`))) :`true` (`local.Local_LastLoopRoll`)))
  (set `local.Local_Isdetail` IsDetail)
  (set `local.Local_CurrentLoopIndex` LoopIndex)
  (set `local.Local_NextLoopIndex` (mod (+ LoopIndex 1) (`self.NumberOfSplinePoints`)))
  (set `local.Local_TrackElementMesh` TrackElementMesh)
  (`|ExecutionSequence`
    (:`then_0`
      (set `local.Local_StartLocation` _location_2)
      (set `local.Local_StartTangent` _tangent_2)
      (set `local.Local_EndLocation` _location)
      (set `local.Local_EndTangent` _tangent)
      (set `local.Local_StartRoll` _output_roll)
      (set `local.Local_StartScale` _output_scale)
      (set `local.Local_Start` 0.0)
      (set `local.Local_EndRoll` _output_roll_2)
      (set `local.Local_EndScale` _output_scale_2)
      (if (`self.Enable Loop`)
        (`/Engine/EditorBlueprintResources/StandardMacros.CompareInt` (- (`self.NumberOfSplinePoints`) 1) (`local.Local_CurrentLoopIndex`)
          (:`>`
            (set `local.Local_LastLoop` false :!label _label))
          (:`==`
            (set `local.Local_LastLoop` true)
            (set `local.Local_LastLoopRoll` _returnvalue_5)
            (`/Engine/EditorBlueprintResources/StandardMacros.CompareFloat` _returnvalue_5 (+ (`KismetMathLibrary.GetPI`) (/ (`KismetMathLibrary.GetPI`) 2.0))
              (:`>`
                (set `local.Local_LastLoopRoll` (- (`local.Local_LastLoopRoll`) (* (`KismetMathLibrary.GetPI`) 2.0))))))
          (:`<`
            (goto _label)))
        (else
          (goto _label))))
    (:`then_1`
      (bind _returnvalue_7 (`AddComponent|NODE_AddSplineMeshComponent-0`))
      (bind _output_get (set `local.Local_CurrentSplineMesh` _returnvalue_7))
      (`StaticMeshComponent.SetStaticMesh` _output_get (`local.Local_TrackElementMesh`))
      (`SplineMeshComponent.SetForwardAxis` (`local.Local_CurrentSplineMesh`) (`self.Body Forward Axis`) true)
      (if (`self.Simple Twist Fix (can break tiling)`)
        ;[1 1 1] simple twist fix
        (`SplineMeshComponent.SetSplineUpDir` (`local.Local_CurrentSplineMesh`) (select `ESplineMeshAxis` (`self.TwistFixMode (X=Z)`) :`X` _returnvalue :`Y` (`SplineComponent.GetRightVectorAtSplinePoint` _spline _local_currentloopindex "Local") :`Z` _returnvalue) true))
      (`self.DynamicMaterialBuild` (`local.Local_CurrentSplineMesh`) (`local.Local_CurrentLoopIndex`) (`local.Local_NextLoopIndex`) (`local.Local_Isdetail`))
      (`SplineMeshComponent.SetStartAndEnd` (`local.Local_CurrentSplineMesh`) (`local.Local_StartLocation`) (`local.Local_StartTangent`) (`local.Local_EndLocation`) (`local.Local_EndTangent`) true)
      (`SplineMeshComponent.SetStartRoll` (`local.Local_CurrentSplineMesh`) (select `bool` (`local.Local_Isdetail`) :`false` _returnvalue_6 :`true` (+ _returnvalue_6 (`self.Detail Mesh StartRoll`))) true)
      (`SplineMeshComponent.SetEndRoll` (`local.Local_CurrentSplineMesh`) (select `bool` (`local.Local_Isdetail`) :`false` _returnvalue_4 :`true` (+ _returnvalue_4 (`self.Detail Mesh EndRoll`))) true)
      (`SplineMeshComponent.SetStartScale` (`local.Local_CurrentSplineMesh`) (select `bool` (`local.Local_Isdetail`) :`false` _returnvalue_3 :`true` (* _returnvalue_3 (`self.Detail Mesh StartScale`))) true)
      (`SplineMeshComponent.SetEndScale` (`local.Local_CurrentSplineMesh`) (select `bool` (`local.Local_Isdetail`) :`false` _returnvalue_2 :`true` (* _returnvalue_2 (`self.Detail Mesh EndScale`))) true)
      (`PrimitiveComponent.SetCollisionEnabled` (`local.Local_CurrentSplineMesh`) (select `bool` (`self.Collision Enable`) :`false` "NoCollision" :`true` "QueryAndPhysics" :!type "ECollisionEnabled Enum")))
    (:`then_2`
      (return (`local.Local_CurrentSplineMesh`)))))

(fn `DynamicMaterialBuild`
  (params (`Spline mesh` :type "SplineMeshComponent Object Reference") (CurrentLoopIndex :type Integer) (NextLoopIndex :type Integer) (IsDetail :type Boolean))
  (locals (LocalDynamicMat :type "MaterialInstanceDynamic Object Reference") (local_isDetail :type Boolean) (local_isLoop :type Boolean))
  (bind _spline (`self.Spline`))
  (bind _returnvalue (`SplineComponent.GetSplineLength` _spline))
  (bind _returnvalue_2 (- _returnvalue (`SplineComponent.GetDistanceAlongSplineAtSplinePoint` _spline NextLoopIndex)))
  (set `local.local_isLoop` false)
  (set `local.local_isDetail` IsDetail)
  (if (== NextLoopIndex 0)
    (set `local.local_isLoop` true))
  (`|ExecutionSequence`
    (:`then_0`
      ;[1 1 1] Dynamic Material Creation / Feed values start and end  to Fix distorsion
      (bind _returnvalue_3 (`PrimitiveComponent.CreateDynamicMaterialInstance` `Spline mesh` 0 (`self.Spline Material`) "None"))
      (set `local.LocalDynamicMat` _returnvalue_3)
      (`MaterialInstanceDynamic.SetScalarParameterValue` (`local.LocalDynamicMat`) "start" (select `bool` (`local.local_isDetail`) :`false` _returnvalue_2 :`true` (+ _returnvalue_2 (`self.Detail Length factor`))))
      (`MaterialInstanceDynamic.SetScalarParameterValue` (`local.LocalDynamicMat`) "end" (- _returnvalue (`SplineComponent.GetDistanceAlongSplineAtSplinePoint` _spline CurrentLoopIndex)))
      (if (`local.local_isDetail`)
        (`MaterialInstanceDynamic.SetScalarParameterValue` (`local.LocalDynamicMat`) "Flip U" (select `bool` (`self.Detail Flip U`) :`false` 1.0 :`true` -1.0 :!type "Float (single-precision)"))
        (`MaterialInstanceDynamic.SetScalarParameterValue` (`local.LocalDynamicMat`) "Flip V" (select `bool` (`self.Detail Flip V`) :`false` 1.0 :`true` -1.0 :!type "Float (single-precision)"))
        (else
          (`MaterialInstanceDynamic.SetScalarParameterValue` (`local.LocalDynamicMat`) "Flip U" (select `bool` (`self.Main Flip U`) :`false` 1.0 :`true` -1.0 :!type "Float (single-precision)"))
          (`MaterialInstanceDynamic.SetScalarParameterValue` (`local.LocalDynamicMat`) "Flip V" (select `bool` (`self.Main Flip V`) :`false` 1.0 :`true` -1.0 :!type "Float (single-precision)")))))
    (:`then_1`
      ;[1 1 1] Add values to expose through blueprint
      (`MaterialInstanceDynamic.SetScalarParameterValue` (`local.LocalDynamicMat`) "Make V Forward Axis" (select `bool` (`local.local_isDetail`) :`false` (select `bool` (`self.V Forward Axis`) :`true` 1.0 :!type "Float (single-precision)") :`true` (select `bool` (`self.Detail V Forward Axis`) :`true` 1.0 :!type "Float (single-precision)")))
      (if (`local.local_isLoop`)
        (`MaterialInstanceDynamic.SetScalarParameterValue` (`local.LocalDynamicMat`) "Stretch Factor" (`self.Loop_Stretch Factor`))
        (else
          (`MaterialInstanceDynamic.SetScalarParameterValue` (`local.LocalDynamicMat`) "Stretch Factor" (`self.Stretch Factor`))))
      (`MaterialInstanceDynamic.SetScalarParameterValue` (`local.LocalDynamicMat`) "Main Tiling" (`self.Main Tiling`)))
    (:`then_2`
      ;[1 1 1] Enable Debug
      (`MaterialInstanceDynamic.SetScalarParameterValue` (`local.LocalDynamicMat`) "Show Debug Color" (`self.Debug Overlay`)))))

(fn `UserConstructionScript`
  (locals (Local_StartDynamicMaterial :type "MaterialInstanceDynamic Object Reference") (Local_EndDynamicMaterial :type "MaterialInstanceDynamic Object Reference") (NewLocalVar_0 :type Integer :default 1))
  (bind _spline (`self.Spline`))
  (bind _splinedataarray (`self.SplineDataArray`))
  (bind (_location _tangent) (`SplineComponent.GetLocationAndTangentAtSplinePoint` (`self.Spline`) (`self.NumberOfSplinePoints`) "Local"))
  (bind (_location_2 _tangent_2) (`SplineComponent.GetLocationAndTangentAtSplinePoint` (`self.Spline`) (`self.NumberOfSplinePoints`) "Local"))
  (bind (_location_3 _tangent_3) (`SplineComponent.GetLocationAndTangentAtSplinePoint` (`self.Spline`) 0 "Local"))
  (bind (_location_4 _tangent_4) (`SplineComponent.GetLocationAndTangentAtSplinePoint` (`self.Spline`) 0 "Local"))
  (bind _returnvalue (`KismetMathLibrary.Conv_VectorToRotator` _tangent))
  (bind _returnvalue_2 (`KismetMathLibrary.Conv_VectorToRotator` _tangent_2))
  (bind _returnvalue_3 (`KismetMathLibrary.Conv_VectorToRotator` _tangent_3))
  (bind _returnvalue_4 (`KismetMathLibrary.Conv_VectorToRotator` _tangent_4))
  (`|ExecutionSequence`
    (:`then_0`
      (set `self.NumberOfSplinePoints` (`SplineComponent.GetNumberOfSplinePoints` (`self.Spline`))))
    (:`then_1`
      (`/Engine/EditorBlueprintResources/StandardMacros.CompareInt` (`KismetArrayLibrary.Array_Length` (`self.SplineDataArray`)) (`self.NumberOfSplinePoints`) :!label _label
        (:`>`
          (`KismetArrayLibrary.Array_Remove` _splinedataarray (`KismetArrayLibrary.Array_LastIndex` _splinedataarray)))
        (:`<`
          (`KismetArrayLibrary.Array_Add` (`self.SplineDataArray`) (`self.CableMeshDefaults`))
          (goto _label))))
    (:`then_2`
      (for _index (range (+ (- (`self.NumberOfSplinePoints`) (`KismetMathLibrary.SelectInt` 1 2 (`self.Enable Loop`))) 1))
        (set `self.Current_loopIndex` _index)
        (bind _output_detail (break `/Game/Blueprint/Art/SplineData` (`|GetArrayItem` (`self.SplineDataArray`) _index)))
        (set `self.draw detail` _output_detail)
        (if (`self.draw detail`)
          (if (`self.DetailReplaceMode`)
            ;[1 0.9225 0.3229] Detail Draw
            (`self.BuildTrackElement` (`self.Current_loopIndex`) (`self.Detail Mesh`) true :!label _label_2)
            (else
              (`|ExecutionSequence`
                (:`then_0`
                  (`self.BuildTrackElement` (`self.Current_loopIndex`) (`self.BodyMesh`) :!label _label_3))
                (:`then_1`
                  (goto _label_2)))))
          (else
            (goto _label_3))))
      (`|ExecutionSequence`
        (:`then_0`
          (if (`self.Draw_Start`)
            ;[1 1 1] Create Static Mesh 1 on Beginning
            (bind _returnvalue_5 (`AddComponent|NODE_AddStaticMeshComponent-3`))
            (`StaticMeshComponent.SetStaticMesh` _returnvalue_5 (`self.Start Mesh 1`))
            (`SceneComponent.K2_SetRelativeLocationAndRotation` _returnvalue_5 _location_4 (select `ESplineMeshAxis` (`self.Terminations Forward Axis`) :`X` _returnvalue_4 :`Y` (`KismetMathLibrary.MakeRotator` (+ (.roll _returnvalue_4) 90.0) (.pitch _returnvalue_4) (.yaw _returnvalue_4)) :`Z` (`KismetMathLibrary.MakeRotator` (.roll _returnvalue_4) (+ (.pitch _returnvalue_4) 90.0) (.yaw _returnvalue_4))) false false)
            (`SceneComponent.SetRelativeScale3D` _returnvalue_5 (`self.Start Mesh Scale`))
            (`SceneComponent.K2_AddLocalOffset` _returnvalue_5 (`self.Start Mesh Offset`) false false)
            (`SceneComponent.K2_AddLocalRotation` _returnvalue_5 (`KismetMathLibrary.MakeRotator` (.x (`self.Start Mesh Roll`)) (.y (`self.Start Mesh Roll`)) (.z (`self.Start Mesh Roll`))) false false)
            (`PrimitiveComponent.SetCollisionEnabled` _returnvalue_5 (select `bool` (`self.Collision Enable`) :`false` "NoCollision" :`true` "QueryAndPhysics" :!type "ECollisionEnabled Enum"))
            (bind _returnvalue_6 (`PrimitiveComponent.CreateDynamicMaterialInstance` _returnvalue_5 0 (`self.Start Material Override`) "None"))
            (set `local.Local_StartDynamicMaterial` _returnvalue_6)
            (if (`self.Start Mesh2 Enable`)
              ;[1 1 1] Create Static Mesh 2 on Beginning
              (bind _returnvalue_7 (`AddComponent|NODE_AddStaticMeshComponent-5`))
              (`StaticMeshComponent.SetStaticMesh` _returnvalue_7 (`self.Start Mesh 2`))
              (`SceneComponent.K2_SetRelativeLocationAndRotation` _returnvalue_7 _location_3 (select `ESplineMeshAxis` (`self.Terminations Forward Axis`) :`X` _returnvalue_3 :`Y` (`KismetMathLibrary.MakeRotator` (+ (.roll _returnvalue_3) 90.0) (.pitch _returnvalue_3) (.yaw _returnvalue_3)) :`Z` (`KismetMathLibrary.MakeRotator` (.roll _returnvalue_3) (+ (.pitch _returnvalue_3) 90.0) (.yaw _returnvalue_3))) false false)
              (`SceneComponent.SetRelativeScale3D` _returnvalue_7 (`self.Start Mesh Scale`))
              (`SceneComponent.K2_AddLocalOffset` _returnvalue_7 (`KismetMathLibrary.MakeVector` (+ (.x (`self.Start Mesh Offset`)) (`self.Start Mesh2 Offset`)) (.y (`self.Start Mesh Offset`)) (.z (`self.Start Mesh Offset`))) false false)
              (`SceneComponent.K2_AddLocalRotation` _returnvalue_7 (`KismetMathLibrary.MakeRotator` (.x (`self.Start Mesh Roll`)) (.y (`self.Start Mesh Roll`)) (.z (`self.Start Mesh Roll`))) false false)
              (`PrimitiveComponent.SetCollisionEnabled` _returnvalue_7 (select `bool` (`self.Collision Enable`) :`false` "NoCollision" :`true` "QueryAndPhysics" :!type "ECollisionEnabled Enum"))
              (`PrimitiveComponent.SetMaterial` _returnvalue_7 0 (`local.Local_StartDynamicMaterial`)))))
        (:`then_1`
          (if (`self.Draw_End`)
            ;[1 1 1] Create Static Mesh 2  on End
            (bind _returnvalue_8 (`AddComponent|NODE_AddStaticMeshComponent-4`))
            (`StaticMeshComponent.SetStaticMesh` _returnvalue_8 (`self.End Mesh 1`))
            (`SceneComponent.K2_SetRelativeLocationAndRotation` _returnvalue_8 _location (select `ESplineMeshAxis` (`self.Terminations Forward Axis`) :`X` _returnvalue :`Y` (`KismetMathLibrary.MakeRotator` (+ (.roll _returnvalue) -90.0) (.pitch _returnvalue) (.yaw _returnvalue)) :`Z` (`KismetMathLibrary.MakeRotator` (.roll _returnvalue) (+ (.pitch _returnvalue) -90.0) (.yaw _returnvalue))) false false)
            (`SceneComponent.SetRelativeScale3D` _returnvalue_8 (`self.End Mesh Scale`))
            (`SceneComponent.K2_AddLocalOffset` _returnvalue_8 (`self.End Mesh Offset`) false false)
            (`SceneComponent.K2_AddLocalRotation` _returnvalue_8 (`KismetMathLibrary.MakeRotator` (.x (`self.End Mesh Roll`)) (.y (`self.End Mesh Roll`)) (.z (`self.End Mesh Roll`))) false false)
            (`PrimitiveComponent.SetCollisionEnabled` _returnvalue_8 (select `bool` (`self.Collision Enable`) :`false` "NoCollision" :`true` "QueryAndPhysics" :!type "ECollisionEnabled Enum"))
            (bind _returnvalue_9 (`PrimitiveComponent.CreateDynamicMaterialInstance` _returnvalue_8 0 (`self.End Material Override`) "None"))
            (set `local.Local_EndDynamicMaterial` _returnvalue_9)
            (if (`self.End Mesh2 Enable`)
              ;[1 1 1] Create Static Mesh 2 on End
              (bind _returnvalue_10 (`AddComponent|NODE_AddStaticMeshComponent-6`))
              (`StaticMeshComponent.SetStaticMesh` _returnvalue_10 (`self.End Mesh 2`))
              (`SceneComponent.K2_SetRelativeLocationAndRotation` _returnvalue_10 _location_2 (select `ESplineMeshAxis` (`self.Terminations Forward Axis`) :`X` _returnvalue_2 :`Y` (`KismetMathLibrary.MakeRotator` (+ (.roll _returnvalue_2) -90.0) (.pitch _returnvalue_2) (.yaw _returnvalue_2)) :`Z` (`KismetMathLibrary.MakeRotator` (.roll _returnvalue_2) (+ (.pitch _returnvalue_2) -90.0) (.yaw _returnvalue_2))) false false)
              (`SceneComponent.SetRelativeScale3D` _returnvalue_10 (`self.End Mesh Scale`))
              (`SceneComponent.K2_AddLocalOffset` _returnvalue_10 (`KismetMathLibrary.MakeVector` (+ (.x (`self.End Mesh Offset`)) (`self.End Mesh2 Offset`)) (.y (`self.End Mesh Offset`)) (.z (`self.End Mesh Offset`))) false false)
              (`SceneComponent.K2_AddLocalRotation` _returnvalue_10 (`KismetMathLibrary.MakeRotator` (.x (`self.End Mesh Roll`)) (.y (`self.End Mesh Roll`)) (.z (`self.End Mesh Roll`))) false false)
              (`PrimitiveComponent.SetCollisionEnabled` _returnvalue_10 (select `bool` (`self.Collision Enable`) :`false` "NoCollision" :`true` "QueryAndPhysics" :!type "ECollisionEnabled Enum"))
              (`PrimitiveComponent.SetMaterial` _returnvalue_10 0 (`local.Local_EndDynamicMaterial`)))))))
    (:`then_3`
      (if (`self.Draw Track Point Numbers`)
        ;[1 1 1] Show Spline Point numbers
        (for _index_2 (range (`self.NumberOfSplinePoints`))
          (set `self.Current track point` (`KismetStringLibrary.Conv_IntToString` _index_2))
          (bind _returnvalue_11 (`AddComponent|NODE_AddTextRenderComponent-0` :`RelativeTransform` (`KismetMathLibrary.MakeTransform` (+ (* (`SplineComponent.GetUpVectorAtSplinePoint` _spline _index_2 "Local") (`self.Debug Z position`)) (.location (`SplineComponent.GetTransformAtSplinePoint` _spline _index_2 "Local" false))) (.rotation (`SplineComponent.GetTransformAtSplinePoint` _spline _index_2 "Local" false)) (.scale (`SplineComponent.GetTransformAtSplinePoint` _spline _index_2 "Local" false)))))
          (`TextRenderComponent.K2_SetText` _returnvalue_11 (`KismetTextLibrary.Conv_StringToText` (`self.Current track point`)))
          (`TextRenderComponent.SetWorldSize` _returnvalue_11 (`self.Debug Text Size`)))))
    (:`then_4`
      (if (`self.draw point arrows`)
        ;[1 1 1] draw SP local transform arrows
        (for _index_3 (range (`self.NumberOfSplinePoints`))
          (bind _returnvalue_12 (`SplineComponent.GetTransformAtSplinePoint` (`self.Spline`) _index_3 "Local" false))
          (bind (_x _y _z) (`KismetMathLibrary.BreakRotIntoAxes` (.rotation _returnvalue_12)))
          (`AddComponent|NODE_AddArrowComponent-1` :`RelativeTransform` (`KismetMathLibrary.MakeTransform` (.location _returnvalue_12) (`KismetMathLibrary.MakeRotationFromAxes` _z _y _x) (* (.scale _returnvalue_12) 0.1)))
          (bind (_x_2 _y_2 _z_2) (`KismetMathLibrary.BreakRotIntoAxes` (.rotation _returnvalue_12)))
          (`AddComponent|NODE_AddArrowComponent-2` :`RelativeTransform` (`KismetMathLibrary.MakeTransform` (.location _returnvalue_12) (`KismetMathLibrary.MakeRotationFromAxes` _x_2 _y_2 _z_2) (* (.scale _returnvalue_12) 0.1)))
          (bind (_x_3 _y_3 _z_3) (`KismetMathLibrary.BreakRotIntoAxes` (.rotation _returnvalue_12)))
          (`AddComponent|NODE_AddArrowComponent-3` :`RelativeTransform` (`KismetMathLibrary.MakeTransform` (.location _returnvalue_12) (`KismetMathLibrary.MakeRotationFromAxes` _y_3 _x_3 _z_3) (* (.scale _returnvalue_12) 0.1))))))))