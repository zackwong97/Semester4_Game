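; Game instance Blueprint that drives front-end menus and hosting of multiplayer sessions.
; Events create main, host, server list and options widgets; main and host reuse stored references as guards, while the options check is inverted, creating only if one already exists.
; LauchLobby calls a stub loading screen, creates an Advanced Session with optional LAN, then opens the Main level as a listen server or prints a failure.
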(event `ShowLoadingScreen`)

(event `Spawn Main Menu Widget`
  (bind _returnvalue (`GameplayStatics.GetPlayerController` 0))
  ;[1 1 1] Create Main Menu / Trigger on level blueprint event begin
  (`/Engine/EditorBlueprintResources/StandardMacros.IsValid` (`self.mainMenuRef`)
    (:`Is Not Valid`
      (bind _returnvalue_2 (`|CreateWidget` "/Game/UI/Blueprints/MainMenu.MainMenu_C" _returnvalue))
      (bind _output_get (set `self.mainMenuRef` _returnvalue_2))
      (`UserWidget.AddToViewport` _output_get 0)
      (set `PlayerController.bShowMouseCursor` true _returnvalue)
      (`WidgetBlueprintLibrary.SetInputMode_GameAndUIEx` _returnvalue _output_get "DoNotLock" false))))

(event `Show Host Menu`
  ;[1 1 1] Shows Host Menu
  (`/Engine/EditorBlueprintResources/StandardMacros.IsValid` (`self.HostMenuRef`)
    (:`Is Not Valid`
      (bind _returnvalue (`|CreateWidget` "/Game/UI/Blueprints/HostMenu.HostMenu_C" (`GameplayStatics.GetPlayerController` 0)))
      (bind _output_get (set `self.HostMenuRef` _returnvalue))
      (`UserWidget.AddToViewport` _output_get 0))))

(event `Lauch Lobby`
  (params (ServerName :type Text) (Lan :type Boolean))
  (set `self.ServerName` ServerName)
  (`self.ShowLoadingScreen`)
  (`CreateSessionCallbackProxyAdvanced.CreateAdvancedSession` :`PlayerController` (`GameplayStatics.GetPlayerController` 0) :`PublicConnections` 10 :`PrivateConnections` 10 :`bUseLAN` Lan
    (:`OnSuccess`
      (`GameplayStatics.OpenLevel` "Main" true "listen"))
    (:`OnFailure`
      (`KismetSystemLibrary.PrintString` "Fail to Host Game" true true (struct :`G` 0.66 :`B` 1.0 :`A` 1.0) 10.0))))

(event `Show Servers Menu`
  ;[1 1 1] Create Server List Menu
  (bind _returnvalue (`|CreateWidget` "/Game/UI/Blueprints/ServerMenu.ServerMenu_C" (`GameplayStatics.GetPlayerController` 0)))
  (`UserWidget.AddToViewport` _returnvalue 0))

(event `Show Options Menu`
  ;[1 1 1] Shows Options Menu
  (`/Engine/EditorBlueprintResources/StandardMacros.IsValid` (`self.OptionsMenuRef`)
    (:`Is Valid`
      (bind _returnvalue (`|CreateWidget` "/Game/UI/Blueprints/OptionsMenu.OptionsMenu_C" (`GameplayStatics.GetPlayerController` 0)))
      (bind _output_get (set `self.OptionsMenuRef` _returnvalue))
      (`UserWidget.AddToViewport` _output_get 0))))