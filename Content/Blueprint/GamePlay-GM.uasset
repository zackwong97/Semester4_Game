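; Gameplay game mode that spawns each player's character at a player start and stores it in that player's GamePlay-PC CharacterRef.
; On a controller swap from the lobby, the CharacterID on Lobby-PC picks the class: 0 and 1 give BP_Character_Base, 2 gives BP_Girl.
; Players arriving through PostLogin always receive BP_Character_Base.
; Possession is not handled in this graph.
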(event `self.K2_OnSwapPlayerControllers`
  (params (OldPC :type "PlayerController Object Reference") (NewPC :type "PlayerController Object Reference"))
  (bind _asgame_play__pc (cast `/Game/Blueprint/GamePlay-PC` NewPC :!pure true))
  (bind _asgame_play__pc_2 (cast `/Game/Blueprint/GamePlay-PC` NewPC :!pure true))
  (switch `int` (`/Game/Blueprint/Lobby-PC.Character ID` (cast `/Game/Blueprint/Lobby-PC` OldPC :!pure true))
    (:`0`
      (bind _returnvalue (`|SpawnActorFromClass` "/Game/Characters/Player/TestCharacter2/BP_Character_Base.BP_Character_Base_C" (`self.GetTransform` (`self.K2_FindPlayerStart` _asgame_play__pc_2)) "Undefined" "OverrideRootScale" null null :!label _label))
      (set `/Game/Blueprint/GamePlay-PC.CharacterRef` _returnvalue _asgame_play__pc_2))
    (:`1`
      (goto _label))
    (:`2`
      (bind _returnvalue_2 (`|SpawnActorFromClass` "/Game/Characters/Player/TestCharacter2/BP_Girl.BP_Girl_C" (`self.GetTransform` (`self.K2_FindPlayerStart` _asgame_play__pc)) "Undefined" "OverrideRootScale" null null))
      (set `/Game/Blueprint/GamePlay-PC.CharacterRef` _returnvalue_2 _asgame_play__pc))))

(event `self.K2_PostLogin`
  (params (NewPlayer :type "PlayerController Object Reference"))
  (bind _asgame_play__pc (cast `/Game/Blueprint/GamePlay-PC` NewPlayer))
  (bind _returnvalue (`|SpawnActorFromClass` "/Game/Characters/Player/TestCharacter2/BP_Character_Base.BP_Character_Base_C" (`self.GetTransform` (`self.K2_FindPlayerStart` _asgame_play__pc)) "Undefined" "OverrideRootScale" null null))
  (set `/Game/Blueprint/GamePlay-PC.CharacterRef` _returnvalue _asgame_play__pc))

(fn `UserConstructionScript`)