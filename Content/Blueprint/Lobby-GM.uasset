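; Lobby game mode that tracks joined players, shares Knight and Girl character availability, and launches the DemoB level.
; Logins and logouts update the player list, with logouts freeing the leaver's character and pushing availability to every Lobby-PC.
; EnterGame triggers loading on each controller, then server-travels.
; A helper returns a player's Steam avatar and name, retrying on fetch failure and still returning when Steam is absent.
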(event `self.K2_PostLogin`
  (params (NewPlayer :type "PlayerController Object Reference"))
  (`KismetArrayLibrary.Array_Add` (`self.List of Players`) NewPlayer)
  (`KismetSystemLibrary.PrintString` (`KismetStringLibrary.Concat_StrStr` (`AdvancedSessionsLibrary.GetPlayerName` NewPlayer) " has entered the lobby") true true (struct :`R` 0.001567 :`G` 1.0 :`A` 1.0) 3.0)
  (for _array_element (`self.List of Players`)
    (bind _aslobby__pc (cast `/Game/Blueprint/Lobby-PC` _array_element))
    (`/Game/Blueprint/Lobby-PC.Get Player List` _aslobby__pc)
    (`self.Everyone Update Character Menu`)))

(event `self.K2_OnLogout`
  (params (ExitingController :type "Controller Object Reference"))
  (bind _aslobby__pc (cast `/Game/Blueprint/Lobby-PC` ExitingController))
  (`KismetArrayLibrary.Array_RemoveItem` (`self.List of Players`) _aslobby__pc)
  (switch `int` (`/Game/Blueprint/Lobby-PC.Character ID` _aslobby__pc)
    (:`1`
      (set `self.Knight Is Avaible?` true))
    (:`2`
      (set `self.Girl Is Avaible?` true)))
  (`self.Everyone Update Character Menu`))

(event `Enter Game`
  (for _array_element (`self.List of Players`)
    (`/Game/Blueprint/Lobby-PC.Call Loading` (cast `/Game/Blueprint/Lobby-PC` _array_element :!pure true)))
  (`KismetSystemLibrary.ExecuteConsoleCommand` "servertravel /Game/Maps/DemoB/DemoB_Persistent" null))

(event `Everyone Update Character Menu`
  (for _array_element (`self.List of Players`)
    (bind _aslobby__pc (cast `/Game/Blueprint/Lobby-PC` _array_element))
    (`/Game/Blueprint/Lobby-PC.Update Character Availability` _aslobby__pc (`self.Knight Is Avaible?`) (`self.Girl Is Avaible?`))))

(fn `getAvatar_and_Name`
  (params (PlayerController :type "/Game/Blueprint/Lobby-PC Object Reference (by ref)"))
  (returns (AvatarImage :type "Texture2D Object Reference") (Name :type String) (`steamOnline?` :type Boolean))
  (bind _returnvalue (`AdvancedSessionsLibrary.HasOnlineSubsystem` "STEAM"))
  (if _returnvalue :!label _label
    (bind _returnvalue_2 (`AdvancedSteamFriendsLibrary.GetSteamFriendAvatar` (`AdvancedSessionsLibrary.GetUniqueNetID` PlayerController))
      (:`OnSuccess`
        _)
      (:`OnFailure`
        (goto _label)))
    (else
      (`KismetSystemLibrary.PrintString` "Can't connect to Steam" true true (struct :`G` 0.66 :`B` 1.0 :`A` 1.0) 5.0)))
  (return _returnvalue_2 (`AdvancedSessionsLibrary.GetPlayerName` PlayerController) _returnvalue))

(fn `UserConstructionScript`)