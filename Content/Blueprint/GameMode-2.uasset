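; Game mode that gives each joining MainController a separate camera pawn and character.
; On PostLogin it spawns a BP_CameraPawn at a player start and has the controller possess it, then spawns an unpossessed BP_Character_Base at the same transform, storing both references on the controller.
; A ListPlayers debug event prints all characters and camera pawns, repeating the controller list for each camera pawn.
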(event `self.K2_PostLogin`
  (params (NewPlayer :type "PlayerController Object Reference"))
  (bind _asmain_controller (cast `/Game/Blueprint/MainController` NewPlayer))
  (bind _returnvalue (`|SpawnActorFromClass` "/Game/Blueprint/BP_CameraPawn.BP_CameraPawn_C" (`self.GetTransform` (`self.K2_FindPlayerStart` null)) "Undefined" "OverrideRootScale" null null))
  (bind _output_get (set `/Game/Blueprint/MainController.ServerCameraRef` _returnvalue _asmain_controller))
  (`Controller.Possess` _asmain_controller _output_get)
  (bind _returnvalue_2 (`|SpawnActorFromClass` "/Game/Characters/Player/TestCharacter2/BP_Character_Base.BP_Character_Base_C" (`self.GetTransform` _output_get) "Undefined" "OverrideRootScale" null null))
  (set `/Game/Blueprint/MainController.CharacterRef` _returnvalue_2 _asmain_controller))

(event `List Players`
  (bind _outactors (`GameplayStatics.GetAllActorsOfClass` "/Game/Characters/Player/TestCharacter2/BP_Character_Base.BP_Character_Base_C"))
  (for _array_element _outactors
    (`KismetSystemLibrary.PrintString` (`KismetSystemLibrary.GetDisplayName` _array_element) true true (struct :`R` 0.100626 :`G` 1.0 :`A` 1.0) 5.0))
  (bind _outactors_2 (`GameplayStatics.GetAllActorsOfClass` "/Game/Blueprint/BP_CameraPawn.BP_CameraPawn_C"))
  (for _array_element_2 _outactors_2
    (`KismetSystemLibrary.PrintString` (`KismetSystemLibrary.GetDisplayName` _array_element_2) true true (struct :`G` 0.66 :`B` 1.0 :`A` 1.0) 5.0)
    (bind _outactors_3 (`GameplayStatics.GetAllActorsOfClass` "/Game/Blueprint/MainController.MainController_C"))
    (for _array_element_3 _outactors_3
      (`KismetSystemLibrary.PrintString` (`KismetSystemLibrary.GetDisplayName` _array_element_3) true true (struct :`R` 1.0 :`G` 0.01492 :`A` 1.0) 5.0))))

(fn `UserConstructionScript`)