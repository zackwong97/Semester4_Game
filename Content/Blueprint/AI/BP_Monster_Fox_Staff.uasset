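; Fox staff monster Blueprint, a child AI pawn that layers a few variant-specific settings over its parent's behavior.
; On BeginPlay it sets a particle color, runs the parent logic, and randomly sets the Mask material's X Pan to one of two values for visual variation.
; If its Start flag is set, it tells its Monster_AI_Controller to begin play from the pawn.
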(event `self.ReceiveBeginPlay`
  (set `self.ParticleColor` "NewEnumerator2")
  (`parent.ReceiveBeginPlay`)
  (`MeshComponent.SetScalarParameterValueOnMaterials` (`self.Mask`) "X Pan" (`KismetMathLibrary.Conv_IntToDouble` (`KismetMathLibrary.RandomIntegerInRange` 0 1)))
  (if (`self.Start?`)
    (bind _asmonster_ai_controller (cast `/Game/Blueprint/AI/Monster_AI_Controller` (`self.GetController`)))
    (`/Game/Blueprint/AI/Monster_AI_Controller.BeginPlayFromAIPawn` _asmonster_ai_controller)))

(fn `UserConstructionScript`
  (`parent.UserConstructionScript`))