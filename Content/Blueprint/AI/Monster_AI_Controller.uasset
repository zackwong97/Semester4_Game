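; AI controller for monsters that wander, detect players and react to attackers.
; Wandering sends the pawn to random points from its spawner through RightClick, pausing randomly after each arrival.
; AI Perception sets non-AI characters as the pawn's enemy target, with a brief grace period before sight can be lost.
; Attackers trigger a short timed chase, while losing sight or a dead or invalid target resumes wandering.
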(event `BeginPlayFromAIPawn`
  ;[1 1 1] Get Ref and Start Walking around
  (bind _output_get (set `self.PawnRef` (cast `/Game/Characters/Player/TestCharacter2/BP_Character_Base` (`self.K2_GetPawn`) :!pure true)))
  (if (`/Game/Characters/Player/TestCharacter2/BP_Character_Base.isAI?` _output_get)
    (`self.MoveToRandomLocation`)))

(event `self.ReceiveTick`
  (params (DeltaSeconds :type "Float (single-precision)"))
  (bind _target (`self.Target`))
  (`KismetSystemLibrary.Delay` 0.02)
  (if (`self.HasTargetCurrently?`)
    (if (not (`/Game/Characters/Player/TestCharacter2/BP_Character_Base.isDead?` _target))
      (`/Engine/EditorBlueprintResources/StandardMacros.IsValid` _target
        (:`Is Not Valid`
          _)))
    (set `self.HasTargetCurrently?` false)
    (set `self.Target` null)
    (`self.MoveToRandomLocation`)))

(event `MoveToRandomLocation`
  (bind _pawnref (`self.PawnRef`))
  ;[1 1 1] Move to random Location
  (bind _randomlocation (`/Game/Blueprint/AI/AI_Spawner.GetRandomLocation` (`/Game/Characters/Player/TestCharacter2/BP_Character_Base.AISpawnerRef` _pawnref)))
  (`/Game/Characters/Player/TestCharacter2/BP_Character_Base.Right Click` _pawnref _randomlocation false))

(event `ReachLocationAI`
  ;[1 1 1] Move to random Location
  (`KismetSystemLibrary.Delay` (`KismetMathLibrary.RandomFloatInRange` 2.0 6.0))
  (if (`self.HasTargetCurrently?`)
    _
    (elif (not (`self.IsChasing?`))
      (`self.MoveToRandomLocation`))))

(event `ChaseAttacker`
  (params (Attacker :type "Actor Object Reference (by ref)"))
  (if (`self.HasTargetCurrently?`)
    _
    (elif (not (`self.IsChasing?`))
      (`self.StopMovement`)
      (`|AIMoveTo` (`self.PawnRef`) (0.0 0.0 0.0) Attacker 0.0 true
        (:`then`
          (set `self.IsChasing?` true)
          (`KismetSystemLibrary.Delay` 4.0)
          (if (not (`self.HasTargetCurrently?`))
            (set `self.IsChasing?` false)
            (`self.MoveToRandomLocation`)))))))

(event `self.AIPerception.OnTargetPerceptionUpdated`
  (params (Actor :type "Actor Object Reference") (Stimulus :type "AIStimulus Structure"))
  ;[1 1 1] Player Detection
  (bind _asbp_character_base (cast `/Game/Characters/Player/TestCharacter2/BP_Character_Base` Actor))
  (if (`/Game/Characters/Player/TestCharacter2/BP_Character_Base.isAI?` _asbp_character_base)
    _
    (elif (`.bSuccessfullySensed` (break `AIStimulus` Stimulus))
      (if (not (`self.HasTargetCurrently?`))
        (`KismetSystemLibrary.PrintString` "sense player")
        (set `self.canLoseSight?` false)
        (`self.StopMovement`)
        (bind _output_get (set `self.Target` _asbp_character_base))
        (set `self.HasTargetCurrently?` true)
        (set `self.IsChasing?` false)
        (`/Game/Characters/Player/TestCharacter2/BP_Character_Base.Set Enemy Target` (`self.PawnRef`) _output_get)
        (`KismetSystemLibrary.Delay` 1.0)
        (set `self.canLoseSight?` true))
      (elif (== _asbp_character_base (`self.Target`))
        (if (`self.canLoseSight?`)
          (`KismetSystemLibrary.PrintString` "lose player")
          (set `self.HasTargetCurrently?` false)
          (set `self.Target` null)
          (`self.MoveToRandomLocation`))))))

(fn `UserConstructionScript`)