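; AI controller for the Nakary Beast that picks an enemy target for its pawn on the server.
; After a short delay on BeginPlay, it gathers non-AI BP_Character_Base actors and sets the first as CurrentEnemyTarget.
; GetNearestEnemy retargets by distance but is not called here.
; Tick only validates the target into an empty sequence; delayed Reposition and WindBlast calls are disconnected, so never run.
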(event `self.ReceiveBeginPlay`
  (`KismetSystemLibrary.Delay` 1.0)
  (`/Engine/EditorBlueprintResources/ActorMacros.Switch Has Authority`
    (:`Authority`
      (bind _asbp_nakary_beast (cast `/Game/Blueprint/AI/BP_NakaryBeast` (`self.K2_GetPawn`)))
      (set `self.CharacterRef` _asbp_nakary_beast)
      (bind _outactors (`GameplayStatics.GetAllActorsOfClass` "/Game/Characters/Player/TestCharacter2/BP_Character_Base.BP_Character_Base_C"))
      (for _array_element _outactors
        (if (not (`/Game/Characters/Player/TestCharacter2/BP_Character_Base.isAI?` _array_element))
          (`KismetArrayLibrary.Array_AddUnique` (`self.EnemyArray`) _array_element)))
      (bind _output_get (set `self.CurrentTarget` (`|GetArrayItem` (`self.EnemyArray`))))
      (set `/Game/Characters/Player/TestCharacter2/BP_Character_Base.CurrentEnemyTarget` _output_get (`self.CharacterRef`)))))

(event `Get Nearest Enemy`
  (bind _characterref (`self.CharacterRef`))
  (set `self.EnemyDistance` 0.0)
  (for _array_element (`self.EnemyArray`)
    (if (== (`self.EnemyDistance`) 0.0)
      (bind _returnvalue (`self.GetDistanceTo` _array_element (`self.CharacterRef`)))
      (set `self.EnemyDistance` _returnvalue)
      (bind _output_get (set `self.CurrentTarget` _array_element))
      (set `/Game/Characters/Player/TestCharacter2/BP_Character_Base.CurrentEnemyTarget` _output_get _characterref)
      (else
        (`/Engine/EditorBlueprintResources/StandardMacros.CompareFloat` _returnvalue (`self.EnemyDistance`)
          (:`<`
            (set `self.EnemyDistance` _returnvalue)
            (bind _output_get_2 (set `self.CurrentTarget` _array_element))
            (set `/Game/Characters/Player/TestCharacter2/BP_Character_Base.CurrentEnemyTarget` _output_get_2 _characterref)))))))

(event `self.ReceiveTick`
  (params (DeltaSeconds :type "Float (single-precision)"))
  (`/Engine/EditorBlueprintResources/ActorMacros.Switch Has Authority`
    (:`Authority`
      (`/Game/Characters/Player/TestCharacter2/BP_Character_Base.CurrentEnemyTarget` (`self.CharacterRef`)
        (:`then`
          (`|ExecutionSequence`))
        (:`else`)))))

(fn `UserConstructionScript`)