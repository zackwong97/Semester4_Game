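; Squirrel monster AI pawn (SnS variant) that extends a parent monster Blueprint.
; On BeginPlay it sets its particle color, runs the parent logic and, if its Start flag is set, calls the startup function on its Monster_AI_Controller.
; A StartAI event sets that flag and runs the same controller startup, so the AI can be activated after spawn.
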(event `self.ReceiveBeginPlay`
  (set `self.ParticleColor` "NewEnumerator3")
  (`parent.ReceiveBeginPlay`)
  (if (`self.Start?`)
    (bind _asmonster_ai_controller (cast `/Game/Blueprint/AI/Monster_AI_Controller` (`self.GetController`) :!label _label))
    (`/Game/Blueprint/AI/Monster_AI_Controller.BeginPlayFromAIPawn` _asmonster_ai_controller)))

(event `StartAI`
  (set `self.Start?` true)
  (goto _label))

(fn `UserConstructionScript`
  (`parent.UserConstructionScript`))