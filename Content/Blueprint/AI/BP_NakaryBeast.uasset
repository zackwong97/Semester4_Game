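; Nakary Beast AI boss character with tornado, roar, minion summon, wind blast and dash reposition abilities.
; Animation-finish events clear casting flags and resume attacking; repositioning dashes to a random reachable point behind or beside it, then chains two wind blasts.
; Roar briefly enables a sphere for server-side knockback and once-per-player damage; minions inherit the controller's target.
; Delay-loop macros handle turning, and death destroys spawned tornadoes.
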(event `Tornado`
  (bind _spawn (`self.spawn`))
  (bind _returnvalue (+ (`SceneComponent.K2_GetComponentLocation` _spawn) (* (`SceneComponent.GetRightVector` _spawn) 125.0)))
  (bind _outhit (`KismetSystemLibrary.LineTraceSingle` _returnvalue (+ _returnvalue (0.0 0.0 -300.0)) "TraceTypeQuery3" true))
  (bind _returnvalue_2 (`|SpawnActorFromClass` "/Game/Effects/Skills/Blueprint/BP_Tornado.BP_Tornado_C" (`KismetMathLibrary.Conv_VectorToTransform` (+ (`.Location` (`GameplayStatics.BreakHitResult` _outhit)) (0.0 0.0 250.0))) "AlwaysSpawn" "OverrideRootScale" null self 700.0 true null true 0.0 null null))
  (`KismetArrayLibrary.Array_Add` (`self.TornadoRef`) _returnvalue_2)
  (`/Engine/EditorBlueprintResources/StandardMacros.IncrementInt` (`/Game/Blueprint/AI/NakaryBeast_AI_Controller.TornadoInField` (cast `/Game/Blueprint/AI/NakaryBeast_AI_Controller` (`self.GetController`) :!pure true))))

(event `self.Sphere.OnComponentBeginOverlap`
  (params (OverlappedComponent :type "PrimitiveComponent Object Reference") (OtherActor :type "Actor Object Reference") (OtherComp :type "PrimitiveComponent Object Reference") (OtherBodyIndex :type Integer) (bFromSweep :type Boolean) (SweepResult :type "HitResult Structure (by ref)"))
  ;[1 1 1] Roar
  (`/Engine/EditorBlueprintResources/ActorMacros.Switch Has Authority`
    (:`Authority`
      (cast `/Game/Effects/Skills/Blueprint/BP_Tornado` OtherActor
        (:`CastFailed`
          (if (not (== OtherActor self))
            (for _array_element (`self.hasReceivedRoarDamage`)
              (if (== _array_element OtherActor)
                (goto _label :!via `Close`)
                (else
                  (goto _label :!via `Open`))))
            (`/Engine/EditorBlueprintResources/StandardMacros.Gate` false :!label _label
              (:`Exit`
                (bind _asbp_character_base (cast `/Game/Characters/Player/TestCharacter2/BP_Character_Base` OtherActor))
                (bind _knockbackspeed (`/Game/Characters/Player/TestCharacter2/BP_Character_Base.KnockBackSpeed` _asbp_character_base))
                (if (== _knockbackspeed (`self.KnockBackSpeed`))
                  (set `/Game/Characters/Player/TestCharacter2/BP_Character_Base.KnockBackSpeed` (* _knockbackspeed (`self.KnockBackMultiplier`)) _asbp_character_base))
                (`self.Knock Back` _asbp_character_base (`self.K2_GetActorLocation`))
                (if (not (`/Game/Characters/Player/TestCharacter2/BP_Character_Base.isAI?` _asbp_character_base))
                  (`KismetArrayLibrary.Array_Add` (`self.hasReceivedRoarDamage`) _asbp_character_base)
                  (`self.Receive Damage` _asbp_character_base false null (0.0 0.0 0.0) self (`self.RoarDamage`) "NewEnumerator0"))))))))))

(event `self.Sphere.OnComponentEndOverlap`
  (params (OverlappedComponent :type "PrimitiveComponent Object Reference") (OtherActor :type "Actor Object Reference") (OtherComp :type "PrimitiveComponent Object Reference") (OtherBodyIndex :type Integer))
  ;[1 1 1] Roar
  (`/Engine/EditorBlueprintResources/ActorMacros.Switch Has Authority`
    (:`Authority`
      (if (not (== self OtherActor))
        (bind _asbp_character_base (cast `/Game/Characters/Player/TestCharacter2/BP_Character_Base` OtherActor))
        (`self.Stop Knock Back` _asbp_character_base)
        (bind _knockbackspeed (`/Game/Characters/Player/TestCharacter2/BP_Character_Base.KnockBackSpeed` _asbp_character_base))
        (if (not (== _knockbackspeed (`self.KnockBackSpeed`)))
          (set `/Game/Characters/Player/TestCharacter2/BP_Character_Base.KnockBackSpeed` (/ _knockbackspeed (`self.KnockBackMultiplier`)) _asbp_character_base))))))

(event `self.PS_Roar.OnSystemFinished`
  (params (PSystem :type "ParticleSystemComponent Object Reference"))
  ;[1 1 1] Roar
  (`ActorComponent.Deactivate` PSystem))

(event `Tornado Anim Finish`
  (set `self.TornadoAnim` false)
  (set `self.IsCasting?` false)
  (`self.Attack`))

(event `RoarFinish`
  ;[1 1 1] Roar
  (set `self.Roar` false)
  (set `self.IsCasting?` false)
  (`self.Attack`))

(event `EmitRoar`
  ;[1 1 1] Roar
  (`ActorComponent.Activate` (`self.PS_Roar`) false)
  (`PrimitiveComponent.SetCollisionEnabled` (`self.Sphere`) "QueryOnly")
  (`KismetSystemLibrary.Delay` 0.35)
  (`PrimitiveComponent.SetCollisionEnabled` (`self.Sphere`) "NoCollision")
  (`KismetArrayLibrary.Array_Clear` (`self.hasReceivedRoarDamage`))
  (`|ExecutionSequence`
    (:`then_0`
      (goto _label :!via `Open`))))

(event `Spawn Minions`
  (bind _sphere (`self.Sphere`))
  (bind (_randomlocation _returnvalue) (`NavigationSystemV1.K2_GetRandomReachablePointInRadius` (+ (`SceneComponent.K2_GetComponentLocation` _sphere) (* (`SceneComponent.GetForwardVector` _sphere) 100)) (`SphereComponent.SphereRadius` _sphere) null null))
  ;[1 1 1] Roar
  (if (>= (`self.CurrentMonsters`) (`self.MonsterLimit`)) :!label _label_2
    _
    (elif _returnvalue
      (bind _returnvalue_2 (`|SpawnActorFromClass` (`self.MonsterToSpawn`) (`KismetMathLibrary.Conv_VectorToTransform` _randomlocation) "AdjustIfPossibleButDontSpawnIfColliding" "OverrideRootScale" null 100.0 true null true 0.0 self null))
      (`/Engine/EditorBlueprintResources/StandardMacros.IsValid` _returnvalue_2
        (:`Is Valid`
          (`/Engine/EditorBlueprintResources/StandardMacros.IncrementInt` (`self.CurrentMonsters`)
            (:`  `
              (bind _asmonster_ai_controller (cast `/Game/Blueprint/AI/Monster_AI_Controller` (`AIBlueprintHelperLibrary.GetAIController` _returnvalue_2)))
              (bind _currentnearesttarget (`/Game/Blueprint/AI/NakaryBeast_AI_Controller.CurrentNearestTarget` (cast `/Game/Blueprint/AI/NakaryBeast_AI_Controller` (`self.GetController`) :!pure true))
                (:`then`
                  (`/Game/Blueprint/AI/Monster_AI_Controller.Set target from NakaryBeast` _asmonster_ai_controller _currentnearesttarget))
                (:`else`))))))
      (else
        (goto _label_2)))))

(event `self.ReceiveBeginPlay`
  (`parent.ReceiveBeginPlay`)
  (`/Engine/EditorBlueprintResources/ActorMacros.Switch Has Authority`))

(event `self.ReceiveTick`
  (params (DeltaSeconds :type "Float (single-precision)"))
  (`parent.ReceiveTick` DeltaSeconds)
  (`/Engine/EditorBlueprintResources/ActorMacros.Switch Has Authority`
    (:`Authority`
      (if (`self.isDead?`)
        (`/Engine/EditorBlueprintResources/StandardMacros.DoOnce` false
          (:`Completed`
            (for _array_element (`self.TornadoRef`)
              (`/Engine/EditorBlueprintResources/StandardMacros.IsValid` _array_element
                (:`Is Valid`
                  (`self.K2_DestroyActor` _array_element))))))))))

(event `Stop Everything`
  ;[1 1 1] Reposition
  (`MovementComponent.StopMovementImmediately` (`self.CharacterMovement`))
  (set `self.Attacking?` false)
  (`KismetSystemLibrary.K2_ClearTimer` null "TurnToTarget"))

(event `WindBlastAnim_1_Finish`
  ;[1 1 1] Wind Blast
  (set `self.WindBlastAnim_1` false)
  (if (not (`self.isDead?`)) :!label _label_3
    (set `self.IsCasting?` true)
    (`self.Stop Everything`)
    (`self.TurnToEnemy`
      (:`CompleteTurn`
        (switch `int` (`self.WindBlastCount`)
          (:`0`
            (set `self.WindBlastAnim_1` true)
            (set `self.WindBlastCount` 1))
          (:`1`
            (set `self.WindBlastAnim_2` true)
            (set `self.WindBlastCount` 0)))))))

(event `WindBlast`
  ;[1 1 1] Wind Blast
  (if (not (`self.IsCasting?`))
    (goto _label_3)))

(event `self.Dash Done`
  ;[1 1 1] Reposition
  (if (`self.repositioning`)
    (`self.Stop Everything`)
    (`self.WindBlast`)
    (set `self.repositioning` false)
    (else
      (`self.Attack`))))

(event `Reposition`
  (bind (_randomlocation _returnvalue) (`NavigationSystemV1.K2_GetRandomReachablePointInRadius` (- (`self.K2_GetActorLocation`) (* (`self.GetActorForwardVector`) (`self.DistanceCheck`))) (`self.RadiusCheck`) null null))
  (bind (_randomlocation_2 _returnvalue_2) (`NavigationSystemV1.K2_GetRandomReachablePointInRadius` (+ (`self.K2_GetActorLocation`) (* (`self.GetActorRightVector`) (`self.DistanceCheck`))) (`self.RadiusCheck`) null null))
  (bind (_randomlocation_3 _returnvalue_3) (`NavigationSystemV1.K2_GetRandomReachablePointInRadius` (- (`self.K2_GetActorLocation`) (* (`self.GetActorRightVector`) (`self.DistanceCheck`))) (`self.RadiusCheck`) null null))
  ;[1 1 1] Reposition
  (set `self.IsCasting?` true)
  (set `self.repositioning` true)
  (switch `int` (`KismetMathLibrary.RandomIntegerInRange` 0 2) :!label _label_4
    (:`0`
      (if _returnvalue
        (set `self.TargetLocation` _randomlocation)
        (else
          (goto _label_4))))
    (:`1`
      (if _returnvalue_3
        (set `self.TargetLocation` _randomlocation_3)
        (else
          (goto _label_4))))
    (:`2`
      (if _returnvalue_2
        (set `self.TargetLocation` _randomlocation_2)
        (else
          (goto _label_4)))))
  (`self.TurnToAim` (`self.TargetLocation`)
    (:`complete`
      (`self.Stop Everything`)
      (`self.Dash Skill`))))

(event `SpawnWindBlast`
  ;[1 1 1] Wind Blast
  (`|SpawnActorFromClass` "/Game/Effects/Skills/Blueprint/BP_WindBlast.BP_WindBlast_C" (`KismetMathLibrary.Conv_VectorToTransform` (`SceneComponent.K2_GetComponentLocation` (`self.spawn`))) "AlwaysSpawn" "OverrideRootScale" null self (`self.K2_GetActorLocation` (`self.CurrentEnemyTarget`)) (`self.WindBlast_Damage`) null))

(event `WindBlastAnim_2_Finish`
  ;[1 1 1] Wind Blast
  (set `self.WindBlastAnim_2` false)
  (set `self.IsCasting?` false)
  (`self.Attack`))

(fn `UserConstructionScript`
  (`parent.UserConstructionScript`))