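; Server-authoritative AI spawner that places monsters of a configurable class at random reachable navmesh points within its radius.
; Tick passes through a gate and a Delay to pace spawns up to a limit, optionally closing the gate once reached.
; Each monster receives stat overrides, an optional material and a spawner reference, and successful spawns increment the count.
; The construction script sizes the collision sphere to the spawn radius.
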(event `self.ReceiveTick`
  (params (DeltaSeconds :type "Float (single-precision)"))
  (bind _materialoverride (`self.MaterialOverride`))
  (bind (_randomlocation _returnvalue) (`NavigationSystemV1.K2_GetRandomReachablePointInRadius` (`self.K2_GetActorLocation`) (`self.SpawnRadius`) null null))
  (`/Engine/EditorBlueprintResources/ActorMacros.Switch Has Authority`
    (:`Authority`
      (`/Engine/EditorBlueprintResources/StandardMacros.Gate` false :!label _label
        (:`Exit`
          (if (== (`self.CurrentSpawn`) (`self.SpawnLimit`))
            (if (`self.DisableOnceHitLimit?`)
              (goto _label :!via `Close`))
            (else
              (`KismetSystemLibrary.Delay` (`self.SpawnDelayInSec`))
              (if _returnvalue
                (bind _returnvalue_2 (`|SpawnActorFromClass` (`self.MonsterClass`) (`KismetMathLibrary.Conv_VectorToTransform` _randomlocation) "AdjustIfPossibleButDontSpawnIfColliding" "OverrideRootScale" null (`self.AttackRangedOverride`) (`self.AttackSpeed(AnimPlayRate)`) (`self.Movementspeed`) (`self.Max Health`) true self (`self.IsRange?`) (`self.HP_Regen`) (`self.AI_Damage_Override`) null null))
                (`/Engine/EditorBlueprintResources/StandardMacros.IsValid` _returnvalue_2
                  (:`Is Valid`
                    (`/Engine/EditorBlueprintResources/StandardMacros.IsValid` _materialoverride
                      (:`Is Valid`
                        (`PrimitiveComponent.SetMaterial` (`Character.Mesh` _returnvalue_2) 0 _materialoverride))
                      (:`Is Not Valid`
                        _))
                    (set `self.CurrentSpawn` (+ (`self.CurrentSpawn`) 1))))))))))))

(fn `GetRandomLocation`
  (returns (RandomLocation :type "Vector Structure"))
  (return (`NavigationSystemV1.K2_GetRandomReachablePointInRadius` (`self.K2_GetActorLocation`) (`self.SpawnRadius`) null null)))

(fn `UserConstructionScript`
  (`SphereComponent.SetSphereRadius` (`self.sphereCollision`) (`self.SpawnRadius`) false))