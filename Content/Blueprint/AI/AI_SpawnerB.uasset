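; AI spawner actor that spawns BP_MonsterBoss enemies at random reachable navmesh points within SpawnRadius.
; Tick runs through a Gate and Delay, counting successful spawns up to SpawnLimit, then optionally closing the gate.
; Each boss receives damage, range and spawner-reference values, plus an optional material override.
; The construction script sizes the collision sphere to the spawn radius.
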(event `self.ReceiveTick`
  (params (DeltaSeconds :type "Float (single-precision)"))
  (bind _materialoverride (`self.MaterialOverride`))
  (bind (_randomlocation _returnvalue) (`NavigationSystemV1.K2_GetRandomReachablePointInRadius` (`self.K2_GetActorLocation`) (`self.SpawnRadius`) null null))
  (`/Engine/EditorBlueprintResources/StandardMacros.Gate` false :!label _label
    (:`Exit`
      (if (== (`self.CurrentSpawn`) (`self.SpawnLimit`))
        (if (`self.DisableOnceHitLimit?`)
          (goto _label :!via `Close`))
        (else
          (`KismetSystemLibrary.Delay` (`self.SpawnDelayInSec`))
          (if _returnvalue
            (bind _returnvalue_2 (`|SpawnActorFromClass` "/Game/Blueprint/AI/BP_MonsterBoss.BP_MonsterBoss_C" (`KismetMathLibrary.Conv_VectorToTransform` _randomlocation) "AdjustIfPossibleButDontSpawnIfColliding" "OverrideRootScale" null (`self.AI_Damage`) (`self.AttackRangedOverride`) true self (`self.IsRange?`) null))
            (`/Engine/EditorBlueprintResources/StandardMacros.IsValid` _returnvalue_2
              (:`Is Valid`
                (`/Engine/EditorBlueprintResources/StandardMacros.IsValid` _materialoverride
                  (:`Is Valid`
                    (`PrimitiveComponent.SetMaterial` (`Character.Mesh` _returnvalue_2) 0 _materialoverride))
                  (:`Is Not Valid`
                    _))
                (set `self.CurrentSpawn` (+ (`self.CurrentSpawn`) 1))))))))))

(fn `GetRandomLocation`
  (returns (RandomLocation :type "Vector Structure"))
  (return (`NavigationSystemV1.K2_GetRandomReachablePointInRadius` (`self.K2_GetActorLocation`) (`self.SpawnRadius`) null null)))

(fn `UserConstructionScript`
  (`SphereComponent.SetSphereRadius` (`self.sphereCollision`) (`self.SpawnRadius`) false))