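; Behavior Tree task that, despite its MoveToActor name, issues no move and hands the blackboard's target to a dagger fox monster.
; On execute it halts the TargetActor character's movement, not the controlled pawn's, then passes that character to the monster's SetEnemyTarget.
; It finishes with success only if the target is Attacking at that moment; otherwise it never calls FinishExecute.
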(event `self.ReceiveExecuteAI`
  (params (OwnerController :type "AIController Object Reference") (ControlledPawn :type "Pawn Object Reference"))
  (bind _asbp_character_base (cast `/Game/Characters/Player/TestCharacter2/BP_Character_Base` (`BlackboardComponent.GetValueAsObject` (`AIBlueprintHelperLibrary.GetBlackboard` OwnerController) "TargetActor") :!pure true))
  (bind _attacking_ (`/Game/Characters/Player/TestCharacter2/BP_Character_Base.Attacking?` _asbp_character_base))
  (`MovementComponent.StopMovementImmediately` (`Character.CharacterMovement` _asbp_character_base))
  (`/Game/Characters/Player/TestCharacter2/BP_Character_Base.Set Enemy Target` (cast `/Game/Blueprint/AI/BP_Monster_Fox_Dagger` ControlledPawn :!pure true) _asbp_character_base)
  (if _attacking_
    (`self.FinishExecute` _attacking_)))