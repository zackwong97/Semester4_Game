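; BP_Flame is a skill projectile that flies toward a target location and damages the first character it hits other than its attacker.
; On spawn it turns to face the target in yaw only, then Tick moves it forward along local X, scaled by Speed.
; A sphere overlap with a BP_Character_Base spawns an explosion, applies damage once and destroys the flame.
; Without a hit, it destroys itself after a short delay.
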(event `self.ReceiveTick`
  (params (DeltaSeconds :type "Float (single-precision)"))
  (`self.K2_AddActorLocalOffset` (`KismetMathLibrary.MakeVector` (* DeltaSeconds (* (`self.Speed`) 2.0)))))

(event `self.ReceiveBeginPlay`
  (`self.K2_SetActorRotation` (`KismetMathLibrary.MakeRotator` 0.0 0.0 (.yaw (`KismetMathLibrary.FindLookAtRotation` (`self.K2_GetActorLocation`) (`self.targetLocation`)))))
  (`KismetSystemLibrary.Delay` 2.0)
  (`self.K2_DestroyActor`))

(event `self.Sphere.OnComponentBeginOverlap`
  (params (OverlappedComponent :type "PrimitiveComponent Object Reference") (OtherActor :type "Actor Object Reference") (OtherComp :type "PrimitiveComponent Object Reference") (OtherBodyIndex :type Integer) (bFromSweep :type Boolean) (SweepResult :type "HitResult Structure (by ref)"))
  (if (not (== OtherActor (`self.Attacker`)))
    (bind _asbp_character_base (cast `/Game/Characters/Player/TestCharacter2/BP_Character_Base` OtherActor))
    (`/Engine/EditorBlueprintResources/StandardMacros.DoOnce` false
      (:`Completed`
        (`GameplayStatics.SpawnEmitterAtLocation` "/Game/StarterContent/Particles/P_Explosion.P_Explosion" (`self.K2_GetActorLocation`) (struct) (1.5 1.5 1.5))
        (`/Game/Characters/Player/TestCharacter2/BP_Character_Base.Receive Damage` _asbp_character_base (`self.Damage`) (`self.Attacker`))
        (`self.K2_DestroyActor`)))))

(fn `UserConstructionScript`)