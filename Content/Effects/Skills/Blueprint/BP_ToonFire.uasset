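; BP_ToonFire is a homing fire projectile skill effect that damages a specific target.
; BeginPlay homes the projectile movement on the target's capsule, and the construction script picks a red or blue particle template from ParticleColor.
; Overlapping the target or its shield calls ReceiveDamage once, flagged reflectable, then destroys the actor after a brief delay.
; The IsShieldUp check leads to the same hit logic either way.
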(event `self.Sphere.OnComponentBeginOverlap`
  (params (OverlappedComponent :type "PrimitiveComponent Object Reference") (OtherActor :type "Actor Object Reference") (OtherComp :type "PrimitiveComponent Object Reference") (OtherBodyIndex :type Integer) (bFromSweep :type Boolean) (SweepResult :type "HitResult Structure (by ref)"))
  (bind _targetactor (`self.TargetActor`))
  (bind _asbp_shield (cast `/Game/Effects/Skills/Blueprint/BP_Shield` OtherActor)
    (:`then`
      (if (== (`/Game/Effects/Skills/Blueprint/BP_Shield.ShieldOwner` _asbp_shield) (`self.TargetActor`))
        (`/Engine/EditorBlueprintResources/StandardMacros.DoOnce` false :!label _label
          (:`Completed`
            (`/Game/Characters/Player/TestCharacter2/BP_Character_Base.Receive Damage` (`self.TargetActor`) true (`GameplayStatics.GetObjectClass` self) (`self.K2_GetActorLocation`) (`self.Attacker`) (`self.Damage`) (`self.ParticleColor`))
            (`KismetSystemLibrary.Delay` 0.1)
            (`self.K2_DestroyActor`)))))
    (:`CastFailed`
      (if (== OtherActor _targetactor)
        (if (`/Game/Characters/Player/TestCharacter2/BP_Character_Base.isShieldUp?` _targetactor)
          (goto _label)
          (else
            (goto _label)))))))

(event `self.ReceiveBeginPlay`
  (bind _targetactor (`self.TargetActor`))
  (`/Engine/EditorBlueprintResources/StandardMacros.IsValid` _targetactor
    (:`Is Valid`
      (set `ProjectileMovementComponent.HomingTargetComponent` (`Character.CapsuleComponent` _targetactor) (`self.ProjectileMovement`)))))

(fn `UserConstructionScript`
  (bind _particlesystem (`self.ParticleSystem`))
  (switch `/Game/Blueprint/ENormalAttackParticle` (`self.ParticleColor`)
    (:`NewEnumerator0`
      (`ParticleSystemComponent.SetTemplate` _particlesystem "/Game/Effects/Skills/Particles/PS_ToonFire_Red.PS_ToonFire_Red"))
    (:`NewEnumerator1`
      (`ParticleSystemComponent.SetTemplate` _particlesystem "/Game/Effects/Skills/Particles/PS_ToonFire_Blue.PS_ToonFire_Blue"))))