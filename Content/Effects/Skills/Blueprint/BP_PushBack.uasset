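; BP_PushBack is a skill effect actor that knocks back characters caught in its sphere, excluding its owner.
; On overlap it stops the character's movement and targets, then calls KnockBack with the effect's location.
; The first hit starts a brief one-time delay that destroys the sphere, keeping the push window short.
; The construction script picks a red or blue particle template from EffectColor, and the actor destroys itself when the particles finish.
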(event `self.Sphere.OnComponentBeginOverlap`
  (params (OverlappedComponent :type "PrimitiveComponent Object Reference") (OtherActor :type "Actor Object Reference") (OtherComp :type "PrimitiveComponent Object Reference") (OtherBodyIndex :type Integer) (bFromSweep :type Boolean) (SweepResult :type "HitResult Structure (by ref)"))
  (if (not (== OtherActor (`self.GetOwner`)))
    (bind _asbp_character_base (cast `/Game/Characters/Player/TestCharacter2/BP_Character_Base` OtherActor))
    (`/Game/Characters/Player/TestCharacter2/BP_Character_Base.Stop All Movement and Targets` _asbp_character_base)
    (`/Game/Characters/Player/TestCharacter2/BP_Character_Base.Knock Back` _asbp_character_base (`self.K2_GetActorLocation`))
    (`/Engine/EditorBlueprintResources/StandardMacros.DoOnce` false
      (:`Completed`
        (`KismetSystemLibrary.Delay` 0.05)
        (`ActorComponent.K2_DestroyComponent` (`self.Sphere`))))))

(event `self.ParticleSystem.OnSystemFinished`
  (params (PSystem :type "ParticleSystemComponent Object Reference"))
  (`self.K2_DestroyActor`))

(fn `UserConstructionScript`
  (bind _particlesystem (`self.ParticleSystem`))
  (switch `/Game/Blueprint/ENormalAttackParticle` (`self.EffectColor`)
    (:`NewEnumerator0`
      (`ParticleSystemComponent.SetTemplate` _particlesystem "/Game/Effects/Skills/Particles/PS_FleetingPowerRed.PS_FleetingPowerRed"))
    (:`NewEnumerator1`
      (`ParticleSystemComponent.SetTemplate` _particlesystem "/Game/Effects/Skills/Particles/PS_FleetingPowerBlue.PS_FleetingPowerBlue"))))