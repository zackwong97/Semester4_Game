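; BP_Shield is a skill effect actor that shows a red or blue shield sphere, with its material picked by EffectColor at construction.
; Tick ramps a timer from 0 to 1 over TimeToCompleteShield, driving the material's Amount parameter.
; ShieldEnd sets FringeSpace negative and restarts the ramp.
; A DoOnce and Gate pair lets the first completion arm destruction, so the completed end ramp destroys the actor.
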(event `ShieldEnd`
  (bind _sphere (`self.Sphere`))
  (`MeshComponent.SetScalarParameterValueOnMaterials` _sphere "Amount" 0.0)
  (`MeshComponent.SetScalarParameterValueOnMaterials` _sphere "FringeSpace" -1.0)
  (set `self.timer` 0.0))

(event `self.ReceiveBeginPlay`
  (set `self.timer` 0.0))

(event `self.ReceiveTick`
  (params (DeltaSeconds :type "Float (single-precision)"))
  (if (== (`self.timer`) 1.0)
    (`/Engine/EditorBlueprintResources/StandardMacros.DoOnce` false :!label _label
      (:`Completed`
        (`|ExecutionSequence`
          (:`then_0`
            (`/Engine/EditorBlueprintResources/StandardMacros.Gate` true :!label _label_2
              (:`Exit`
                (`self.K2_DestroyActor`))))
          (:`then_1`
            (goto _label_2 :!via `Open`)))))
    (else
      (`MeshComponent.SetScalarParameterValueOnMaterials` (`self.Sphere`) "Amount" (`self.timer`))
      (set `self.timer` (`KismetMathLibrary.FClamp` (+ (/ DeltaSeconds (`self.TimeToCompleteShield`)) (`self.timer`))))
      (goto _label :!via `Reset`))))

(fn `UserConstructionScript`
  (bind _sphere (`self.Sphere`))
  (switch `/Game/Blueprint/ENormalAttackParticle` (`self.EffectColor`)
    (:`NewEnumerator0`
      (`PrimitiveComponent.SetMaterial` _sphere 0 "/Game/Effects/Skills/Materials/M_Shield2Red_Inst.M_Shield2Red_Inst"))
    (:`NewEnumerator1`
      (`PrimitiveComponent.SetMaterial` _sphere 0 "/Game/Effects/Skills/Materials/M_Shield2Blue_Inst.M_Shield2Blue_Inst"))))