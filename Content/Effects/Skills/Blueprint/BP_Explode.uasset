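; Explosion skill effect actor: an expanding, dissolving sphere that damages opposing characters before destroying itself.
; EffectColor picks a red or blue material, while Tick drives one clamped alpha over DissolveTime to scale the sphere and animate the material's "Amount" parameter.
; Overlap damages characters whose IsAI differs from the Attacker's, skipping HitActor, the Attacker and tornadoes, and always passes Red as the damage color.
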(event `self.ReceiveBeginPlay`
  (bind _sphere1 (`self.Sphere1`))
  (switch `/Game/Blueprint/ENormalAttackParticle` (`self.EffectColor`)
    (:`NewEnumerator0`
      (`PrimitiveComponent.SetMaterial` _sphere1 0 "/Game/TopDownBP/Exp_Particle/Exp_M_Inst.Exp_M_Inst"))
    (:`NewEnumerator1`
      (`PrimitiveComponent.SetMaterial` _sphere1 0 "/Game/TopDownBP/Exp_Particle/Exp_M_Inst_Blue.Exp_M_Inst_Blue"))))

(event `self.ReceiveTick`
  (params (DeltaSeconds :type "Float (single-precision)"))
  (bind _output_get (set `self.dissolveLerpAlpha` (`KismetMathLibrary.FClamp` (+ (/ DeltaSeconds (`self.DissolveTime`)) (`self.dissolveLerpAlpha`)))))
  (`MeshComponent.SetScalarParameterValueOnMaterials` (`self.Sphere1`) "Amount" (`KismetMathLibrary.Lerp` 0.1 1.0 _output_get))
  (bind _returnvalue (`KismetMathLibrary.Lerp` 1.0 3.5 _output_get))
  (`SceneComponent.SetWorldScale3D` (`self.Sphere1`) (`KismetMathLibrary.MakeVector` _returnvalue _returnvalue _returnvalue))
  (if (== (`self.dissolveLerpAlpha`) 1.0)
    (`self.K2_DestroyActor`)))

(event `self.Sphere1.OnComponentBeginOverlap`
  (params (OverlappedComponent :type "PrimitiveComponent Object Reference") (OtherActor :type "Actor Object Reference") (OtherComp :type "PrimitiveComponent Object Reference") (OtherBodyIndex :type Integer) (bFromSweep :type Boolean) (SweepResult :type "HitResult Structure (by ref)"))
  (bind _attacker (`self.Attacker`))
  (if (== OtherActor (`self.HitActor`))
    _
    (elif (== OtherActor _attacker)
      _
      (elif (not (== (`/Game/Characters/Player/TestCharacter2/BP_Character_Base.isAI?` _attacker) (`/Game/Characters/Player/TestCharacter2/BP_Character_Base.isAI?` (cast `/Game/Characters/Player/TestCharacter2/BP_Character_Base` OtherActor :!pure true))))
        (bind _asbp_character_base (cast `/Game/Characters/Player/TestCharacter2/BP_Character_Base` OtherActor))
        (cast `/Game/Effects/Skills/Blueprint/BP_Tornado` _asbp_character_base
          (:`CastFailed`
            (`/Game/Characters/Player/TestCharacter2/BP_Character_Base.Receive Damage` _asbp_character_base false null (0.0 0.0 0.0) (`self.Attacker`) (`self.damage`) "NewEnumerator0")))))))

(fn `UserConstructionScript`
  (bind _sphere1 (`self.Sphere1`))
  (switch `/Game/Blueprint/ENormalAttackParticle` (`self.EffectColor`)
    (:`NewEnumerator0`
      (`PrimitiveComponent.SetMaterial` _sphere1 0 "/Game/TopDownBP/Exp_Particle/Exp_M_Inst.Exp_M_Inst"))
    (:`NewEnumerator1`
      (`PrimitiveComponent.SetMaterial` _sphere1 0 "/Game/TopDownBP/Exp_Particle/Exp_M_Inst_Blue.Exp_M_Inst_Blue"))))