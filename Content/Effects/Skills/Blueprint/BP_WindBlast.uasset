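; BP_WindBlast is a server-driven wind skill projectile that turns toward a target location, travels forward, and expires after a short delay.
; Each tick a downward line trace snaps it to a fixed height above the surface below.
; Sphere overlaps deal reflectable damage to characters other than the attacker, passing through them.
; Hitting another player's shield damages that shield's owner and destroys the blast.
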(event `self.ReceiveTick`
  (params (DeltaSeconds :type "Float (single-precision)"))
  (bind _returnvalue (`self.K2_GetActorLocation`))
  (`/Engine/EditorBlueprintResources/ActorMacros.Switch Has Authority`
    (:`Authority`
      (`self.K2_AddActorLocalOffset` (`KismetMathLibrary.MakeVector` (* DeltaSeconds (* (`self.Speed`) 2.0))))
      (bind _outhit (`KismetSystemLibrary.LineTraceSingle` :`Start` _returnvalue :`End` (`KismetMathLibrary.MakeVector` (.x _returnvalue) (.y _returnvalue) (- (.z _returnvalue) (`self.Raycast Distance`))) :`TraceChannel` "TraceTypeQuery3" :`TraceColor` (struct :`G` 1.0 :`B` 0.980435 :`A` 1.0)))
      (`self.K2_SetActorLocation` (`KismetMathLibrary.MakeVector` (.x (`.Location` (`GameplayStatics.BreakHitResult` _outhit))) (.y (`.Location` (`GameplayStatics.BreakHitResult` _outhit))) (+ (.z (`.Location` (`GameplayStatics.BreakHitResult` _outhit))) 125.0))))))

(event `self.ReceiveBeginPlay`
  (`/Engine/EditorBlueprintResources/ActorMacros.Switch Has Authority`
    (:`Authority`
      (`self.K2_SetActorRotation` (`KismetMathLibrary.MakeRotator` 0.0 0.0 (.yaw (`KismetMathLibrary.FindLookAtRotation` (`self.K2_GetActorLocation`) (`self.targetLocation`)))))
      (`KismetSystemLibrary.Delay` 2.0)
      (`self.K2_DestroyActor`))))

(event `self.Sphere.OnComponentBeginOverlap`
  (params (OverlappedComponent :type "PrimitiveComponent Object Reference") (OtherActor :type "Actor Object Reference") (OtherComp :type "PrimitiveComponent Object Reference") (OtherBodyIndex :type Integer) (bFromSweep :type Boolean) (SweepResult :type "HitResult Structure (by ref)"))
  (`/Engine/EditorBlueprintResources/ActorMacros.Switch Has Authority`
    (:`Authority`
      (if (not (== OtherActor (`self.Attacker`)))
        (bind _asbp_shield (cast `/Game/Effects/Skills/Blueprint/BP_Shield` OtherActor)
          (:`then`
            (bind _shieldowner (`/Game/Effects/Skills/Blueprint/BP_Shield.ShieldOwner` _asbp_shield))
            (if (== _shieldowner (`self.Attacker`))
              (bind _asbp_character_base (cast `/Game/Characters/Player/TestCharacter2/BP_Character_Base` OtherActor :!label _label))
              (set `self.HitEnemy` _asbp_character_base)
              (else
                (set `self.HitShield` true)
                (set `self.HitEnemy` _shieldowner))))
          (:`CastFailed`
            (goto _label)))
        (`/Game/Characters/Player/TestCharacter2/BP_Character_Base.Receive Damage` (`self.HitEnemy`) true (`GameplayStatics.GetObjectClass` self) (`self.K2_GetActorLocation`) (`self.Attacker`) (`self.Damage`) "NewEnumerator0")
        (if (`self.HitShield`)
          (`self.K2_DestroyActor`))))))

(fn `UserConstructionScript`)