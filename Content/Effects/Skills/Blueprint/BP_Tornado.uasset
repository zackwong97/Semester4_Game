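; BP_Tornado is a server-driven, killable tornado pawn belonging to a Nakary Beast that damages players caught inside it.
; It wanders via AI MoveTo to random reachable points around its owner, retrying when a point is too close.
; Box overlaps track non-AI characters for delayed, repeating damage from Tick.
; At zero health it deregisters from the beast and its controller, then destroys itself; cursor hover toggles custom-depth highlighting.
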(event `self.ReceiveBeginPlay`
  (bind (_randomlocation _returnvalue) (`NavigationSystemV1.K2_GetRandomReachablePointInRadius` (`self.K2_GetActorLocation` (`self.OwnerRef`)) (`self.Radius`) null null))
  (`parent.ReceiveBeginPlay`)
  (`/Engine/EditorBlueprintResources/ActorMacros.Switch Has Authority`
    (:`Authority`
      (`self.OwnerRef`
        (:`then`
          (if _returnvalue :!label _label
            (if (>= (`KismetMathLibrary.Vector_Distance` _randomlocation (`self.K2_GetActorLocation`)) (`self.Minimun Distance`))
              (`|AIMoveTo` self _randomlocation null 0.0
                (:`OnSuccess`
                  (`self.move around`)))
              (else
                (`self.move around` :!label _label_2)))
            (else
              (`KismetSystemLibrary.PrintString` "fail to get random")
              (goto _label_2))))
        (:`else`)))))

(event `move around`
  (`KismetSystemLibrary.Delay` 0.2)
  (goto _label))

(event `self.ReceiveTick`
  (params (DeltaSeconds :type "Float (single-precision)"))
  (`/Engine/EditorBlueprintResources/ActorMacros.Switch Has Authority`
    (:`Authority`
      (if (<= (`self.CurrentHealth`) 0.0)
        (bind _asnakary_beast_ai_controller (cast `/Game/Blueprint/AI/NakaryBeast_AI_Controller` (`self.GetController` (`self.OwnerRef`))))
        (`/Engine/EditorBlueprintResources/StandardMacros.DecrementInt` (`/Game/Blueprint/AI/NakaryBeast_AI_Controller.TornadoInField` _asnakary_beast_ai_controller)
          (:`  `
            (`KismetArrayLibrary.Array_RemoveItem` (`/Game/Blueprint/AI/BP_NakaryBeast.TornadoRef` (`/Game/Blueprint/AI/NakaryBeast_AI_Controller.CharacterRef` _asnakary_beast_ai_controller)) self)
            (`self.K2_DestroyActor`)))
        (else
          (`|ExecutionSequence`
            (:`then_0`
              (`KismetSystemLibrary.Delay` 1.0)
              (for _array_element (`self.CharacterList`)
                (`/Engine/EditorBlueprintResources/StandardMacros.IsValid` _array_element
                  (:`Is Valid`
                    (`self.Receive Damage` _array_element false null (0.0 0.0 0.0) (`self.OwnerRef`) (`self.Damage`) "NewEnumerator0")))))
            (:`then_1`
              (`KismetSystemLibrary.Delay` 4.0)
              (`self.move around`))))))))

(event `self.CapsuleComponent.OnComponentBeginOverlap`
  (params (OverlappedComponent :type "PrimitiveComponent Object Reference") (OtherActor :type "Actor Object Reference") (OtherComp :type "PrimitiveComponent Object Reference") (OtherBodyIndex :type Integer) (bFromSweep :type Boolean) (SweepResult :type "HitResult Structure (by ref)")))

(event `self.Box.OnComponentBeginOverlap`
  (params (OverlappedComponent :type "PrimitiveComponent Object Reference") (OtherActor :type "Actor Object Reference") (OtherComp :type "PrimitiveComponent Object Reference") (OtherBodyIndex :type Integer) (bFromSweep :type Boolean) (SweepResult :type "HitResult Structure (by ref)"))
  (`/Engine/EditorBlueprintResources/ActorMacros.Switch Has Authority`
    (:`Authority`
      (bind _asbp_character_base (cast `/Game/Characters/Player/TestCharacter2/BP_Character_Base` OtherActor))
      (if (not (`/Game/Characters/Player/TestCharacter2/BP_Character_Base.isAI?` _asbp_character_base))
        (`KismetArrayLibrary.Array_Add` (`self.CharacterList`) _asbp_character_base)))))

(event `self.CapsuleComponent.OnComponentEndOverlap`
  (params (OverlappedComponent :type "PrimitiveComponent Object Reference") (OtherActor :type "Actor Object Reference") (OtherComp :type "PrimitiveComponent Object Reference") (OtherBodyIndex :type Integer)))

(event `self.Box.OnComponentEndOverlap`
  (params (OverlappedComponent :type "PrimitiveComponent Object Reference") (OtherActor :type "Actor Object Reference") (OtherComp :type "PrimitiveComponent Object Reference") (OtherBodyIndex :type Integer))
  (`/Engine/EditorBlueprintResources/ActorMacros.Switch Has Authority`
    (:`Authority`
      (bind _asbp_character_base (cast `/Game/Characters/Player/TestCharacter2/BP_Character_Base` OtherActor))
      (`KismetArrayLibrary.Array_RemoveItem` (`self.CharacterList`) _asbp_character_base))))

(event `self.Box.OnBeginCursorOver`
  (params (TouchedComponent :type "PrimitiveComponent Object Reference")))

(event `self.CapsuleComponent.OnBeginCursorOver`
  (params (TouchedComponent :type "PrimitiveComponent Object Reference"))
  (`PrimitiveComponent.SetRenderCustomDepth` (`self.ParticleSystem_0`) true))

(event `self.CapsuleComponent.OnEndCursorOver`
  (params (TouchedComponent :type "PrimitiveComponent Object Reference"))
  (`PrimitiveComponent.SetRenderCustomDepth` (`self.ParticleSystem_0`) false))

(event `self.Box.OnEndCursorOver`
  (params (TouchedComponent :type "PrimitiveComponent Object Reference")))

(fn `UserConstructionScript`)