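; Villager ally NPC that paces back and forth and responds to cursor hover.
; On BeginPlay, it loops AI moves along world X by Movedistance, forward then back from its current location, pausing briefly after each.
; Cursor hover offsets the mesh's custom depth stencil value and restores it on exit, a technique typically paired with post-process highlighting.
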(event `self.ReceiveBeginPlay`
  (bind _movedistance (`self.movedistance`))
  (`parent.ReceiveBeginPlay`)
  (`AITask_MoveTo.AIMoveTo` (`AIBlueprintHelperLibrary.GetAIController` self) (`KismetMathLibrary.MakeVector` (+ (.x (`self.GetNavAgentLocation`)) _movedistance) (.y (`self.GetNavAgentLocation`)) (.z (`self.GetNavAgentLocation`))) null :!label _label
    (:`OnMoveFinished`
      (`KismetSystemLibrary.Delay` 2.0)
      (`AITask_MoveTo.AIMoveTo` (`AIBlueprintHelperLibrary.GetAIController` self) (`KismetMathLibrary.MakeVector` (- (.x (`self.GetNavAgentLocation`)) _movedistance) (.y (`self.GetNavAgentLocation`)) (.z (`self.GetNavAgentLocation`))) null -1.0 "Enable"
        (:`OnMoveFinished`
          (`KismetSystemLibrary.Delay` 2.0)
          (goto _label))))))

(event `self.ReceiveActorBeginCursorOver`
  (bind _mesh (`self.Mesh`))
  (`PrimitiveComponent.SetCustomDepthStencilValue` _mesh (+ (`PrimitiveComponent.CustomDepthStencilValue` _mesh) 10)))

(event `self.ReceiveActorEndCursorOver`
  (bind _mesh (`self.Mesh`))
  (`PrimitiveComponent.SetCustomDepthStencilValue` _mesh (- (`PrimitiveComponent.CustomDepthStencilValue` _mesh) 10)))

(fn `UserConstructionScript`
  (`parent.UserConstructionScript`))