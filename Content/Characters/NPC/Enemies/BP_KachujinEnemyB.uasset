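; Kachujin enemy NPC that roams, chases seen pawns and dies when bullet hits deplete its HP.
; PawnSensing sightings start a repeating AIMoveTo chase at a faster speed, if chasing is allowed.
; Tick ends the chase through a delayed distance check, otherwise roaming to random navmesh points or looping through path points with random pauses.
; Optional custom-depth presets enable outlines, and cursor hover shifts the mesh's stencil value.
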(event `self.ReceiveBeginPlay`
  (bind _mesh (`self.Mesh`))
  (set `CharacterMovementComponent.MaxWalkSpeed` (`self.roamSpeed`) (`self.CharacterMovement`))
  (if (`self.bUsePresetsForOutline`)
    (`PrimitiveComponent.SetRenderCustomDepth` _mesh true)
    (`PrimitiveComponent.SetCustomDepthStencilValue` _mesh 3)
    (`PrimitiveComponent.SetCollisionResponseToChannel` _mesh "ECC_Visibility" "ECR_Block")
    (`PrimitiveComponent.SetCollisionResponseToChannel` _mesh "ECC_GameTraceChannel3" "ECR_Block")
    (`PrimitiveComponent.SetCollisionResponseToChannel` _mesh "ECC_Camera" "ECR_Block")))

(event `self.PawnSensing.OnSeePawn`
  (params (Pawn :type "Pawn Object Reference"))
  ;[1 1 1] Chase player when seen
  (if (`self.bAllowChase`)
    (if (not (`self.bCanSeePlayer`))
      (set `self.bCanSeePlayer` true)
      (if (`self.bEnableDebug`)
        ;[1 0 0] Debug
        (`KismetSystemLibrary.PrintString` (`KismetStringLibrary.Concat_StrStr` (`KismetSystemLibrary.GetDisplayName` self) " is now in chase mode!") true true (struct :`R` 1.0 :`G` 0.1 :`A` 1.0))))
    (bind _ascharacter (cast `Character` Pawn))
    (`|AIMoveTo` self (0.0 0.0 0.0) _ascharacter :!label _label
      (:`then`
        (set `CharacterMovementComponent.MaxWalkSpeed` (`self.ChaseSpeed`) (`self.CharacterMovement`)))
      (:`OnSuccess`
        (`KismetSystemLibrary.Delay` 1.0)
        (goto _label)))))

(event `self.ReceiveActorBeginCursorOver`
  (bind _mesh (`self.Mesh`))
  (`PrimitiveComponent.SetCustomDepthStencilValue` _mesh (+ (`PrimitiveComponent.CustomDepthStencilValue` _mesh) 10)))

(event `self.ReceiveTick`
  (params (DeltaSeconds :type "Float (single-precision)"))
  (bind _pathpoints (`self.PathPoints`))
  (bind _pathpointindex (`self.pathPointIndex`))
  (bind _returnvalue (`KismetSystemLibrary.GetDisplayName` self))
  (bind _returnvalue_2 (`KismetStringLibrary.Conv_IntToString` (+ _pathpointindex 1)))
  (if (<= (`self.HP`) 0)
    (`self.K2_DestroyActor`)
    (else
      ;[1 1 1] Determines speed based on whether or not AI is chasing player
      (if (`self.bCanSeePlayer`)
        ;[1 1 1] Stop chasing the player once the player is over a distance, checked every few seconds
        (set `self.bIsRoaming` false)
        (`KismetSystemLibrary.Delay` 5.0)
        (if (> (`self.GetDistanceTo` (stale `self.PawnSensing.OnSeePawn` Pawn) self) (`self.stopChaseDistance`))
          (set `self.bCanSeePlayer` false)
          (if (`self.bEnableDebug`)
            ;[1 0 0] Debug
            (`KismetSystemLibrary.PrintString` (`KismetStringLibrary.Concat_StrStr` (`KismetSystemLibrary.GetDisplayName` self) " has stopped chasing...") true true (struct :`R` 1.0 :`G` 0.1 :`A` 1.0))))
        (else
          ;[1 1 1] Switch between random roam (0) or
          ; point path roam (1)
          (switch `int` (`self.roamType`)
            (:`0`
              ;[1 1 1] Roams randomly when not chasing
              (if (not (`self.bIsRoaming`))
                (`|AIMoveTo` self (`NavigationSystemV1.K2_GetRandomLocationInNavigableRadius` (`self.K2_GetActorLocation` self) (`self.randomRoamRadius`) (`self.navData`) null) null
                  (:`then`
                    (set `self.bIsRoaming` true)
                    (set `CharacterMovementComponent.MaxWalkSpeed` (`self.roamSpeed`) (`self.CharacterMovement`)))
                  (:`OnSuccess`
                    (`KismetSystemLibrary.Delay` (`KismetMathLibrary.RandomFloatInRange` (`self.minRoamDelay`) (`self.maxRoamDelay`)) :!label _label_2)
                    (set `self.bIsRoaming` false))
                  (:`OnFail`
                    (goto _label_2)))))
            (:`1`
              ;[1 1 1] Roams through a list of points when not chasing
              (if (not (`self.bIsRoaming`))
                (if (`self.bEnableDebug`)
                  ;[1 0 0] Debug
                  (`KismetSystemLibrary.PrintString` (`KismetStringLibrary.Concat_StrStr` _returnvalue " going to point " _returnvalue_2)))
                (`|AIMoveTo` self (0.0 0.0 0.0) (`|GetArrayItem` _pathpoints _pathpointindex)
                  (:`then`
                    (set `self.bIsRoaming` true)
                    (set `CharacterMovementComponent.MaxWalkSpeed` (`self.roamSpeed`) (`self.CharacterMovement`)))
                  (:`OnSuccess`
                    (if (`self.bEnableDebug`)
                      (`KismetSystemLibrary.PrintString` (`KismetStringLibrary.Concat_StrStr` _returnvalue " reached point " _returnvalue_2)))
                    (`KismetSystemLibrary.Delay` (`KismetMathLibrary.RandomFloatInRange` (`self.minRoamDelay`) (`self.maxRoamDelay`)) :!label _label_3)
                    (if (< _pathpointindex (- (`KismetArrayLibrary.Array_Length` _pathpoints) 1))
                      (set `self.pathPointIndex` (+ _pathpointindex 1))
                      (else
                        (set `self.pathPointIndex` 0)))
                    (set `self.bIsRoaming` false))
                  (:`OnFail`
                    (goto _label_3)))))))))))

(event `self.ReceiveActorEndCursorOver`
  (bind _mesh (`self.Mesh`))
  (`PrimitiveComponent.SetCustomDepthStencilValue` _mesh (- (`PrimitiveComponent.CustomDepthStencilValue` _mesh) 10)))

(event `self.CapsuleComponent.OnComponentBeginOverlap`
  (params (OverlappedComponent :type "PrimitiveComponent Object Reference") (OtherActor :type "Actor Object Reference") (OtherComp :type "PrimitiveComponent Object Reference") (OtherBodyIndex :type Integer) (bFromSweep :type Boolean) (SweepResult :type "HitResult Structure (by ref)"))
  (cast `/Game/Effects/Skills/Blueprint/BP_Bullet` OtherActor)
  (set `self.HP` (- (`self.HP`) 1)))

(fn `UserConstructionScript`
  (`parent.UserConstructionScript`))