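; Kachujin enemy NPC that patrols back and forth, takes damage from bullets and is destroyed when its HP runs out.
; Patrol starts on BeginPlay, looping AI MoveTo between positive and negative X/Y offsets from its current location, with random waits between moves.
; Capsule overlaps with BP_Bullet decrement HP, which Tick polls for death.
; Cursor hover shifts the mesh's custom depth stencil value.
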(event `self.ReceiveBeginPlay`
  (`parent.ReceiveBeginPlay`)
  (`self.Patrol`))

(event `self.ReceiveActorBeginCursorOver`
  (bind _mesh (`self.Mesh`))
  (`PrimitiveComponent.SetCustomDepthStencilValue` _mesh (+ (`PrimitiveComponent.CustomDepthStencilValue` _mesh) 10)))

(event `self.ReceiveTick`
  (params (DeltaSeconds :type "Float (single-precision)"))
  (if (<= (`self.HP`) 0)
    (`self.K2_DestroyActor`)))

(event `self.ReceiveActorEndCursorOver`
  (bind _mesh (`self.Mesh`))
  (`PrimitiveComponent.SetCustomDepthStencilValue` _mesh (- (`PrimitiveComponent.CustomDepthStencilValue` _mesh) 10)))

(event `self.CapsuleComponent.OnComponentBeginOverlap`
  (params (OverlappedComponent :type "PrimitiveComponent Object Reference") (OtherActor :type "Actor Object Reference") (OtherComp :type "PrimitiveComponent Object Reference") (OtherBodyIndex :type Integer) (bFromSweep :type Boolean) (SweepResult :type "HitResult Structure (by ref)"))
  (cast `/Game/Effects/Skills/Blueprint/BP_Bullet` OtherActor)
  (set `self.HP` (- (`self.HP`) 1)))

(fn `UserConstructionScript`
  (`parent.UserConstructionScript`))