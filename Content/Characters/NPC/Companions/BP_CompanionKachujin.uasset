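; Companion NPC (Kachujin) that follows its FollowTarget and roams nearby, with optional custom-depth outlining whose stencil value shifts on cursor hover.
; A Tick throttled by a Delay checks distance, teleporting with a cooldown when too far, or using AIMoveTo at catch-up speed when moderately far.
; The IsNotIdle flag switches between these checks and roaming to random navigable points around the target, with randomized idle pauses.
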(event `self.ReceiveBeginPlay`
  (bind _mesh (`self.Mesh`))
  (set `CharacterMovementComponent.MaxWalkSpeed` (`self.roamSpeed`) (`self.CharacterMovement`))
  (if (`self.bUsePresetsForOutline`)
    (`PrimitiveComponent.SetRenderCustomDepth` _mesh true)
    (`PrimitiveComponent.SetCustomDepthStencilValue` _mesh 1)
    (`PrimitiveComponent.SetCollisionResponseToChannel` _mesh "ECC_Visibility" "ECR_Block")
    (`PrimitiveComponent.SetCollisionResponseToChannel` _mesh "ECC_GameTraceChannel3" "ECR_Block")
    (`PrimitiveComponent.SetCollisionResponseToChannel` _mesh "ECC_Camera" "ECR_Block")))

(event `self.ReceiveActorBeginCursorOver`
  (bind _mesh (`self.Mesh`))
  (`PrimitiveComponent.SetCustomDepthStencilValue` _mesh (+ (`PrimitiveComponent.CustomDepthStencilValue` _mesh) 10)))

(event `self.ReceiveActorEndCursorOver`
  (bind _mesh (`self.Mesh`))
  (`PrimitiveComponent.SetCustomDepthStencilValue` _mesh (- (`PrimitiveComponent.CustomDepthStencilValue` _mesh) 10)))

(event `self.ReceiveTick`
  (params (DeltaSeconds :type "Float (single-precision)"))
  (bind _roamspeed (`self.roamSpeed`))
  (bind _charactermovement (`self.CharacterMovement`))
  (bind _followtarget (`self.followTarget`))
  (bind _returnvalue (`self.GetDistanceTo` _followtarget))
  (bind _randomlocation (`NavigationSystemV1.K2_GetRandomLocationInNavigableRadius` (`self.K2_GetActorLocation` _followtarget) (`self.roamRadius`) (`self.navData`) null))
  (`KismetSystemLibrary.Delay` 0.5) ; Causes rest of code to execute every delay seconds \ninstead of every frame.
  (if (`self.bIsNotIdle`)
    (if (> _returnvalue (`self.teleportDistance`))
      ;[1 1 1] Teleports to target.
      (if (> (- (`KismetSystemLibrary.GetGameTimeInSeconds`) (`self.teleportStartTime`)) (`self.teleportCooldown`))
        (`self.K2_TeleportTo` _randomlocation)
        (set `self.teleportStartTime` (`KismetSystemLibrary.GetGameTimeInSeconds`))
        ;[1 1 1] Alters movement speed based on whether companion is catching up or roaming.
        (set `CharacterMovementComponent.MaxWalkSpeed` _roamspeed _charactermovement) ; Teleport
        (set `self.bIsNotIdle` false) ; Sets up a roam destination for the \ncompanion after teleportation
      )
      (elif (> _returnvalue (`self.catchUpDistance`))
        ;[1 1 1] Follows the target.
        (`|AIMoveTo` self (0.0 0.0 0.0) _followtarget 150.0
          (:`then`
            (`KismetSystemLibrary.PrintString` "Catching up to master")
            (set `CharacterMovementComponent.MaxWalkSpeed` (`self.catchUpSpeed`) _charactermovement) ; Catch up
          )
          (:`OnSuccess`
            (set `self.bIsNotIdle` false :!label _label) ; Sets up a roam destination for the \ncompanion after catching up
          )
          (:`OnFail`
            (goto _label)))
        (else
          (set `CharacterMovementComponent.MaxWalkSpeed` _roamspeed _charactermovement) ; Roam
        )))
    (else
      ;[1 1 1] Roams around the target.
      (`|AIMoveTo` self _randomlocation null 25.0 :!label _label_2
        (:`then`
          (set `self.bIsNotIdle` true)
          (`KismetSystemLibrary.PrintString` "Roaming around master."))
        (:`OnSuccess`
          (if (> (`self.idleChance`) (`KismetMathLibrary.RandomIntegerInRange` 0 99)) :!label _label_3
            (`KismetSystemLibrary.Delay` 1.0)
            (goto _label_2)
            (else
              (`KismetSystemLibrary.PrintString` "Idling near master.")
              (`KismetSystemLibrary.Delay` (`self.roamDelay`))
              (set `self.bIsNotIdle` false))))
        (:`OnFail`
          (goto _label_3))))))

(fn `UserConstructionScript`
  (`parent.UserConstructionScript`))