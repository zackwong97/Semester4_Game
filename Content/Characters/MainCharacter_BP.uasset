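; Player character with MOBA-style mouse controls: right-click to move or target an enemy, left-click to cast a skill.
; Right-clicks issue AI moves, while Tick chases the targeted enemy and toggles Attacking by range and animation state.
; An animation-triggered event fires homing projectiles from the right hand, and left-click spawns ExplodeSkill_BP above the cursor when casting is active.
; Cursor hover offsets custom depth stencil values for highlighting.
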(event `self.ReceiveBeginPlay`
  (bind _returnvalue (`GameplayStatics.GetPlayerController` 0))
  (bind _returnvalue_2 (`|CreateWidget` "/Game/Blueprint/MyHUD.MyHUD_C"))
  (`UserWidget.AddToViewport` _returnvalue_2 0)
  (bind _ascharacter_animation_bp (cast `/Game/Characters/Character_Animation_BP` (`SkeletalMeshComponent.GetAnimInstance` (`self.Mesh`))))
  (set `self.Anim_BP` _ascharacter_animation_bp)
  (set `PlayerController.bShowMouseCursor` true _returnvalue)
  (set `PlayerController.bEnableMouseOverEvents` true _returnvalue))

(event `On Left Click From Controller`
  (bind _asmy_controller (cast `/Game/Blueprint/MyController` (`GameplayStatics.GetPlayerController` 0)))
  (if (`/Game/Blueprint/MyController.CastingActive` _asmy_controller)
    (`|SpawnActorFromClass` "/Game/Skill/Skill1/BP/ExplodeSkill_BP.ExplodeSkill_BP_C" (`KismetMathLibrary.Conv_VectorToTransform` (`KismetMathLibrary.MakeVector` (.x (`.Location` (`GameplayStatics.BreakHitResult` (`PlayerController.GetHitResultUnderCursorByChannel` (`GameplayStatics.GetPlayerController` 0) "TraceTypeQuery3" true)))) (.y (`.Location` (`GameplayStatics.BreakHitResult` (`PlayerController.GetHitResultUnderCursorByChannel` (`GameplayStatics.GetPlayerController` 0) "TraceTypeQuery3" true)))) (+ (.z (`.Location` (`GameplayStatics.BreakHitResult` (`PlayerController.GetHitResultUnderCursorByChannel` (`GameplayStatics.GetPlayerController` 0) "TraceTypeQuery3" true)))) 200.0))) "Undefined" "OverrideRootScale" null null)
    (set `/Game/Blueprint/MyController.CastingActive` false _asmy_controller)))

(event `self.ReceiveActorBeginCursorOver`
  (bind (_bblockinghit _binitialoverlap _time _distance _location _impactpoint _normal _impactnormal _physmat _hitactor _hitcomponent) (`GameplayStatics.BreakHitResult` (`PlayerController.GetHitResultUnderCursorByChannel` (`GameplayStatics.GetPlayerController` 0) "TraceTypeQuery4" true)))
  (`PrimitiveComponent.SetCustomDepthStencilValue` _hitcomponent (+ (`PrimitiveComponent.CustomDepthStencilValue` _hitcomponent) 10))
  (bind _output_get (set `self.mousedOverComponent` _hitcomponent)))

(event `self.ReceiveActorEndCursorOver`
  (`PrimitiveComponent.SetCustomDepthStencilValue` (stale `self.ReceiveActorBeginCursorOver` _output_get) (- (`PrimitiveComponent.CustomDepthStencilValue` (stale `self.ReceiveActorBeginCursorOver` _output_get)) 10)))

(event `Press Q Character`)

(event `self.ReceiveTick`
  (params (DeltaSeconds :type "Float (single-precision)"))
  (bind _currentenemy (`self.currentEnemy`))
  (bind _currentenemy_2 (`self.currentEnemy`))
  (bind _returnvalue (`self.K2_GetActorLocation` _currentenemy_2))
  (bind _output_get (set `self.mouseOverObj` (`.ReturnValue` (`PlayerController.GetHitResultUnderCursorByChannel` (`GameplayStatics.GetPlayerController` 0) "TraceTypeQuery4" true))))
  (`/Engine/EditorBlueprintResources/StandardMacros.IsValid` _currentenemy
    (:`Is Valid`
      (cast `/Game/Characters/MainCharacter_BP_Enemy` _currentenemy)
      (if (`self.Attacking`)
        (if (> (`self.GetDistanceTo` _currentenemy_2) (+ (`self.AttackRange`) (`CapsuleComponent.CapsuleRadius` (`self.CapsuleComponent`)) 5.0))
          (if (`/Game/Characters/Character_Animation_BP.attackEnd` (`self.Anim_BP`))
            (set `self.Attacking` false)))
        (else
          (`|AIMoveTo` self _returnvalue null (`self.AttackRange`) true
            (:`OnSuccess`
              (`self.K2_SetActorRotation` (`KismetMathLibrary.FindLookAtRotation` (`self.K2_GetActorLocation`) _returnvalue))
              (set `self.Attacking` true)
              (`Controller.StopMovement` (`AIBlueprintHelperLibrary.GetAIController` self)))))))))

(event `On Right Click From Controller`
  (bind (_hitresult _returnvalue) (`PlayerController.GetHitResultUnderCursorByChannel` (`GameplayStatics.GetPlayerController` 0) "TraceTypeQuery3" true))
  (bind (_bblockinghit _binitialoverlap _time _distance _location) (`GameplayStatics.BreakHitResult` _hitresult))
  (bind (_bblockinghit_2 _binitialoverlap_2 _time_2 _distance_2 _location_2 _impactpoint _normal _impactnormal _physmat _hitactor _hitcomponent) (`GameplayStatics.BreakHitResult` (`PlayerController.GetHitResultUnderCursorByChannel` (`GameplayStatics.GetPlayerController` 0) "TraceTypeQuery4" true)))
  (if (stale `self.ReceiveTick` _output_get)
    (if (not (== _hitactor self))
      (bind _output_get (set `self.currentEnemy` _hitactor))
      (cast `/Game/Characters/MainCharacter_BP_Enemy` _output_get
        (:`then`
          (set `self.Attacking` false :!label _label))
        (:`CastFailed`
          (set `self.Attacking` false)
          (`|AIMoveTo` self (`self.K2_GetActorLocation` (`self.currentEnemy`)) null (`self.AttackRange`) true))))
    (elif _returnvalue
      (set `self.currentEnemy` null)
      (`|SpawnActorFromClass` "/Game/Effects/rightClickEffect.rightClickEffect_C" (`KismetMathLibrary.MakeTransform` _location) "Undefined" "OverrideRootScale" null null)
      (`AIController.MoveToLocation` (`AIBlueprintHelperLibrary.GetAIController` (`self.GetController`)) _location -1.0 true true false true "/Script/AIModule.NavFilter_AIControllerDefault" true)
      (goto _label))))

(event `Attacked From Anim`
  (`self.Normal_Attack`))

(fn `Normal_Attack`
  (bind _returnvalue (`|SpawnActorFromClass` "/Game/Skill/Skill1/BP/BulletParcitalBP.BulletParcitalBP_C" (`KismetMathLibrary.Conv_VectorToTransform` (`SceneComponent.GetSocketLocation` (`self.Mesh`) "RightHand")) "Undefined" "OverrideRootScale" null null))
  (bind _asmain_character_bp_enemy (cast `/Game/Characters/MainCharacter_BP_Enemy` (`self.currentEnemy`))
    (:`then`
      (set `ProjectileMovementComponent.HomingTargetComponent` (`Character.CapsuleComponent` _asmain_character_bp_enemy) (`/Game/Skill/Skill1/BP/BulletParcitalBP.ProjectileMovement` _returnvalue)))
    (:`CastFailed`
      (`KismetSystemLibrary.PrintString` "cast failed"))))

(fn `UserConstructionScript`)