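; Kachujin player character with top-down-style click controls for moving, attacking enemies and collecting items.
; Right-click cursor traces on separate channels pick the target for AI navigation; Tick chases the current enemy until in range, and animation-driven attacks fire homing bullets from the right hand.
; Left click spawns a firework explosion above the cursor while casting.
; Hover outlines use custom depth stencil, and position optionally feeds a material parameter collection.
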(event `On Left Click From Controller`
  ;[1 1 1] Firework skill
  (bind _asmy_controller (cast `/Game/Blueprint/MyController` (`GameplayStatics.GetPlayerController` 0)))
  (if (`/Game/Blueprint/MyController.CastingActive` _asmy_controller)
    (`|SpawnActorFromClass` "/Game/Effects/Skills/Blueprint/BP_Explode.BP_Explode_C" (`KismetMathLibrary.Conv_VectorToTransform` (`KismetMathLibrary.MakeVector` (.x (`.Location` (`GameplayStatics.BreakHitResult` (`PlayerController.GetHitResultUnderCursorByChannel` (`GameplayStatics.GetPlayerController` 0) "TraceTypeQuery3" true)))) (.y (`.Location` (`GameplayStatics.BreakHitResult` (`PlayerController.GetHitResultUnderCursorByChannel` (`GameplayStatics.GetPlayerController` 0) "TraceTypeQuery3" true)))) (+ (.z (`.Location` (`GameplayStatics.BreakHitResult` (`PlayerController.GetHitResultUnderCursorByChannel` (`GameplayStatics.GetPlayerController` 0) "TraceTypeQuery3" true)))) 200.0))) "Undefined" "OverrideRootScale" null null)
    (set `/Game/Blueprint/MyController.CastingActive` false _asmy_controller)))

(event `self.ReceiveBeginPlay`
  (bind _returnvalue (`GameplayStatics.GetPlayerController` 0))
  ;[1 1 1] Begin Play
  (if (`self.bEnableScreenUI`)
    (bind _returnvalue_2 (`|CreateWidget` "/Game/UI/Blueprints/MyHUD.MyHUD_C"))
    (else
      (bind _ascharacter_anim_bp (cast `/Game/Characters/Player/TestMainCharacter/Animations/Character_AnimBP` (`SkeletalMeshComponent.GetAnimInstance` (`self.Mesh`))))
      (set `self.Anim_BP` _ascharacter_anim_bp)
      (set `PlayerController.bShowMouseCursor` true _returnvalue)
      (set `PlayerController.bEnableMouseOverEvents` true _returnvalue))))

(event `self.ReceiveActorBeginCursorOver`
  (bind (_bblockinghit _binitialoverlap _time _distance _location _impactpoint _normal _impactnormal _physmat _hitactor _hitcomponent) (`GameplayStatics.BreakHitResult` (`PlayerController.GetHitResultUnderCursorByChannel` (`GameplayStatics.GetPlayerController` 0) "TraceTypeQuery4" true)))
  ;[1 1 1] Activate outline pp mat
  (`PrimitiveComponent.SetCustomDepthStencilValue` _hitcomponent (+ (`PrimitiveComponent.CustomDepthStencilValue` _hitcomponent) 10))
  (bind _output_get (set `self.mousedOverComponent` _hitcomponent)))

(event `self.ReceiveActorEndCursorOver`
  ;[1 1 1] Activate outline pp mat
  (`PrimitiveComponent.SetCustomDepthStencilValue` (stale `self.ReceiveActorBeginCursorOver` _output_get) (- (`PrimitiveComponent.CustomDepthStencilValue` (stale `self.ReceiveActorBeginCursorOver` _output_get)) 10)))

(event `Press Q Character`)

(event `self.ReceiveTick`
  (params (DeltaSeconds :type "Float (single-precision)"))
  (bind _currentenemy (`self.currentEnemy`))
  (bind _returnvalue (`self.K2_GetActorLocation` _currentenemy))
  (`|ExecutionSequence`
    (:`then_0`
      (bind _output_get (set `self.mouseOverObj` (`.ReturnValue` (`PlayerController.GetHitResultUnderCursorByChannel` (`GameplayStatics.GetPlayerController` 0) "TraceTypeQuery4" true))))
      (`/Engine/EditorBlueprintResources/StandardMacros.IsValid` _currentenemy
        (:`Is Valid`
          (cast `/Game/Characters/NPC/Enemies/BP_KachujinEnemyA` _currentenemy)
          (if (`self.Attacking`)
            ;[1 1 1] Stops attack when enemy moves away from attack range
            (if (> (`self.GetDistanceTo` _currentenemy) (+ (`self.AttackRange`) (`CapsuleComponent.CapsuleRadius` (`self.CapsuleComponent`)) 5.0))
              (if (`/Game/Characters/Player/TestMainCharacter/Animations/Character_AnimBP.attackEnd` (`self.Anim_BP`))
                (set `self.Attacking` false)))
            (else
              ;[1 1 1] Moves to enemy and attacks when within attack range
              (`|AIMoveTo` self _returnvalue null (`self.AttackRange`) true
                (:`OnSuccess`
                  (`self.K2_SetActorRotation` (`KismetMathLibrary.FindLookAtRotation` (`self.K2_GetActorLocation`) _returnvalue))
                  (set `self.Attacking` true)
                  (`Controller.StopMovement` (`AIBlueprintHelperLibrary.GetAIController` self)))))))))
    (:`then_1`
      ;[1 1 1] Updates character position into material parameter collection for materials to use
      (if (`self.bRecordPosition`)
        (`KismetMaterialLibrary.SetVectorParameterValue` "/Game/Environment/Props/Materials/Collections/MPC1.MPC1" "Character Position" (`KismetMathLibrary.Conv_VectorToLinearColor` (`self.K2_GetActorLocation`)))))))

(event `Attacked From Anim`
  ;[1 1 1] Moves to enemy and attacks when within attack range
  (`self.Normal_Attack`))

(event `On Right Click From Controller`
  (bind _returnvalue (`GameplayStatics.GetPlayerController` 0))
  (bind (_hitresult _returnvalue_2) (`PlayerController.GetHitResultUnderCursorByChannel` _returnvalue "TraceTypeQuery5" true))
  (bind (_hitresult_2 _returnvalue_3) (`PlayerController.GetHitResultUnderCursorByChannel` _returnvalue "TraceTypeQuery3" true))
  (bind (_bblockinghit _binitialoverlap _time _distance _location) (`GameplayStatics.BreakHitResult` _hitresult_2))
  (bind (_bblockinghit_2 _binitialoverlap_2 _time_2 _distance_2 _location_2 _impactpoint _normal _impactnormal _physmat _hitactor _hitcomponent) (`GameplayStatics.BreakHitResult` (`PlayerController.GetHitResultUnderCursorByChannel` _returnvalue "TraceTypeQuery4" true)))
  ;[1 1 1] Condition setup for right click behavior
  (if (stale `self.ReceiveTick` _output_get)
    ;;[1 1 1] Enemy
    (if (not (== _hitactor self))
      (bind _output_get (set `self.currentEnemy` _hitactor))
      (cast `/Game/Characters/NPC/Enemies/BP_KachujinEnemyA` _output_get
        (:`then`
          (set `self.Attacking` false))
        (:`CastFailed`
          (set `self.Attacking` false)
          (`|AIMoveTo` self (`self.K2_GetActorLocation` (`self.currentEnemy`)) null (`self.AttackRange`) true))))
    (elif _returnvalue_2
      ;;[1 1 1] Item collect
      (bind _output_get_2 (set `self.currentItem` (`.HitActor` (`GameplayStatics.BreakHitResult` _hitresult))))
      (`|AIMoveTo` self (`self.K2_GetActorLocation` _output_get_2) null 5.0 true
        (:`OnSuccess`
          (`self.K2_DestroyActor` (`self.currentItem`))
          (bind _output_get_3 (set `self.item_inhand` (+ (`self.item_inhand`) 1)))
          (`KismetSystemLibrary.PrintString` (`KismetStringLibrary.Concat_StrStr` (`self.getItemMessage`) (`KismetStringLibrary.Conv_IntToString` _output_get_3) (`self.itemName`)) true true (struct :`G` 0.66 :`B` 1.0 :`A` 1.0) 3.0)))
      (elif _returnvalue_3
        ;;[1 1 1] Move to location
        (set `self.currentEnemy` null)
        (`|SpawnActorFromClass` "/Game/Effects/RightClick/BP_RightClick.BP_RightClick_C" (`KismetMathLibrary.MakeTransform` _location) "Undefined" "OverrideRootScale" null null)
        (`AIController.MoveToLocation` (`AIBlueprintHelperLibrary.GetAIController` (`self.GetController`)) _location -1.0 true true false true "/Script/AIModule.NavFilter_AIControllerDefault" true)
        (set `self.Attacking` false)))))

(fn `Normal_Attack`
  (bind _returnvalue (`|SpawnActorFromClass` "/Game/Effects/Skills/Blueprint/BP_Bullet.BP_Bullet_C" (`KismetMathLibrary.Conv_VectorToTransform` (`SceneComponent.GetSocketLocation` (`self.Mesh`) "RightHand")) "Undefined" "OverrideRootScale" null null))
  (bind _asbp_kachujin_enemy_a (cast `/Game/Characters/NPC/Enemies/BP_KachujinEnemyA` (`self.currentEnemy`))
    (:`then`
      (set `ProjectileMovementComponent.HomingTargetComponent` (`Character.CapsuleComponent` _asbp_kachujin_enemy_a) (`/Game/Effects/Skills/Blueprint/BP_Bullet.ProjectileMovement` _returnvalue)))
    (:`CastFailed`
      (`KismetSystemLibrary.PrintString` "cast failed"))))

(fn `UserConstructionScript`)