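; Base player character Blueprint for click-driven movement, item pickup and attacking.
; Right-click moves, item pickups and attacks all use AIMoveTo; moving or picking up clears attack state, and reached items are destroyed.
; Within attack range, a looping timer turns the character's yaw toward the enemy, then sets Attacking to trigger the attack animation.
; Construction applies MovementSpeed to max walk speed, and BeginPlay caches the knight AnimBP.
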(event `self.ReceiveBeginPlay`
  (set `self.Anim_BP_Ref` (cast `/Game/Characters/Player/TestCharacter2/KnightAnim_BP` (`SkeletalMeshComponent.GetAnimInstance` (`self.Mesh`)) :!pure true)))

(event `Item Pickup`
  (params (Item :type "Actor Object Reference"))
  ;[1 1 1] Pick Up Item
  (set `self.Attacking?` false)
  (set `self.CurrentEnemyTarget` null)
  (bind _asitem_base_class (cast `/Game/Environment/Items/ItemBaseClass` Item))
  (bind _output_get (set `self.CurrentItemTarget` _asitem_base_class))
  (`|AIMoveTo` self (0.0 0.0 0.0) _output_get -1.0 true
    (:`OnSuccess`
      (`/Game/Environment/Items/ItemBaseClass.Destroy when pickup` (`self.CurrentItemTarget`))
      (set `self.CurrentItemTarget` null))))

(event `Set Enemy Target`
  (params (Enemy :type "Actor Object Reference"))
  ;[1 1 1] Attack System
  ;;[1 1 1] Set Enemy Target
  (set `self.CurrentEnemyTarget` Enemy)
  (`self.Attack`))

(event `Attack`
  (bind _currentenemytarget (`self.CurrentEnemyTarget`))
  ;[1 1 1] Attack System
  ;;[1 1 1] If Enemy Target is Valid > Go to Enemy > Rotation to Towards Enemy > Start Attacking
  (`/Engine/EditorBlueprintResources/StandardMacros.IsValid` _currentenemytarget
    (:`Is Valid`
      (`|AIMoveTo` self (0.0 0.0 0.0) _currentenemytarget (`self.AttackRange`) true
        (:`OnSuccess`
          (`KismetSystemLibrary.K2_SetTimer` null "TurnToTarget" 0.01 true))))))

(event `Right Click`
  (params (Location :type "Vector Structure"))
  ;[1 1 1] Clear Attacking Status & Target then > Move to Location
  (set `self.Attacking?` false)
  (set `self.CurrentEnemyTarget` null)
  (`|AIMoveTo` self Location null -1.0))

(event `Finish Turning`
  ;[1 1 1] Attack System
  ;;[1 1 1] Called when TurnToTarget finish > Set Status to Attacking which triggers the attack animation
  (set `self.Attacking?` true))

(fn `TurnToTarget`
  (bind _yaw (.yaw (`KismetMathLibrary.RInterpTo_Constant` (`self.K2_GetActorRotation`) (`KismetMathLibrary.FindLookAtRotation` (`self.K2_GetActorLocation`) (`self.TargetLocation`)) (`self.TurnRate`) 0.01)))
  (`/Engine/EditorBlueprintResources/StandardMacros.IsValid` (`self.CurrentEnemyTarget`)
    (:`Is Valid`
      (set `self.TargetLocation` (`self.K2_GetActorLocation` (`self.CurrentEnemyTarget`)))
      (`self.K2_SetActorRotation` (`KismetMathLibrary.MakeRotator` 0.0 0.0 _yaw))
      (if (`KismetMathLibrary.NearlyEqual_FloatFloat` (.yaw (`self.K2_GetActorRotation`)) _yaw 0.0001)
        (`KismetSystemLibrary.K2_ClearTimer` null "TurnToTarget")
        (`self.Finish Turning`)))))

(fn `UserConstructionScript`
  (set `CharacterMovementComponent.MaxWalkSpeed` (`self.MovementSpeed`) (`self.CharacterMovement`)))